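; Self-destroying effect actor that teleports its Target to Destination with dissolve and reappear VFX, starting on BeginPlay.
; A timeline drives height-based dissolve parameters on Target's mesh materials, then triggers the teleport and a reverse Spawn timeline before cleanup.
; Each phase spawns a ground-traced Niagara effect plus attached per-mesh systems, chosen by skeletal or static type.
; Tick optionally keeps the ground effect under Target.
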(event Custom|Teleportation
  (bind _target (Variables|Parameters|GetTarget))
  (bind _spawneffect_choice (Variables|Parameters|GetSpawnEffect_Choice))
  (bind _effectrotation (Variables|Parameters|GetEffectRotation))
  (bind _target_2 (Variables|Parameters|GetTarget))
  (bind _returnvalue (Transformation|GetActorLocation _target))
  (bind _returnvalue_2 (Transformation|GetActorLocation _target_2))
  (if (Variables|Parameters|GetbKeepRotation?)
    (Transformation|Teleport (Variables|Parameters|GetTarget) (Variables|Parameters|GetDestination) (Transformation|GetActorRotation (Variables|Parameters|GetTarget)))
    (else
      (Transformation|Teleport (Variables|Parameters|GetTarget) (Variables|Parameters|GetDestination) (Variables|Parameters|GetNewRotation))))
  ;[1 1 1] Spawn teleportation effect
  (bind (_outhit _returnvalue_3) (Collision|LineTraceByChannel (+ _returnvalue "0, 0,10.000000") (- _returnvalue "0, 0,1000.000000") "TraceTypeQuery1" false (Utilities|Array|MakeArray _target) "None"))
  (if _returnvalue_3
    (bind _returnvalue_4 (Niagara|SpawnSystematLocation _spawneffect_choice (.ImpactPoint (Collision|BreakHitResult _outhit)) _effectrotation))
    (Variables|Default|SetEffect _returnvalue_4)
    (else
      (bind _returnvalue_5 (Niagara|SpawnSystematLocation _spawneffect_choice (Transformation|GetActorLocation) _effectrotation))
      (Variables|Default|SetEffect _returnvalue_5)))
  (Effects|Components|ParticleSystem|SetColorParameter (Variables|Default|GetEffect) "User.color" (Variables|Parameters|GetColor))
  (Effects|Components|ParticleSystem|SetFloatParameter (Variables|Default|GetEffect) "User.ColorBoost" (Variables|Parameters|GetColorBoost))
  (Effects|Components|ParticleSystem|SetFloatParameter (Variables|Default|GetEffect) "User.Height" (Variables|Parameters|GetHeight))
  (Effects|Components|ParticleSystem|SetFloatParameter (Variables|Default|GetEffect) "User.Speed" (/ 1.0 (Variables|Parameters|GetSpeed)))
  (Effects|Components|ParticleSystem|SetFloatParameter (Variables|Default|GetEffect) "User.Size" (Variables|Parameters|GetEffect_Size))
  (Effects|Components|ParticleSystem|SetFloatParameter (Variables|Default|GetEffect) "User.Thickness" (Variables|Parameters|GetCircle_Thickness))
  ;[1 1 1] Dissolve components
  (CallFunction|Spawn)
  (for _array_element (Variables|Default|GetMeshesReferences)
    (bind _asskeletal_mesh_component (Utilities|Casting|CastToSkeletalMeshComponent (.component _array_element))
      (:then
        (Rendering|Material|SetScalarParameterValueonMaterials _asskeletal_mesh_component "Z_Location" (.z _returnvalue_2))
        (bind _returnvalue_6 (Niagara|SpawnSystemAttached "/Game/Teleportation_VFX/Particles/P_Spawn_SkMesh.P_Spawn_SkMesh" _asskeletal_mesh_component "None" "0, 0, 0" "0, 0, 0" "KeepRelativeOffset" true))
        (Effects|Components|ParticleSystem|SetColorParameter _returnvalue_6 "User.color" (Variables|Parameters|GetColor))
        (Effects|Components|ParticleSystem|SetFloatParameter _returnvalue_6 "User.ColorBoost" (Variables|Parameters|GetColorBoost))
        (Effects|Components|ParticleSystem|SetFloatParameter _returnvalue_6 "User.Height" (Variables|Parameters|GetHeight))
        (Effects|Components|ParticleSystem|SetFloatParameter _returnvalue_6 "User.Size" (Variables|Parameters|GetEffect_Size)))
      (:CastFailed
        (Rendering|Material|SetScalarParameterValueonMaterials (.AsMesh%20Component (Utilities|Casting|CastToMeshComponent (.component _array_element))) "Z_Location" (.z _returnvalue_2))
        (bind _returnvalue_7 (Niagara|SpawnSystemAttached "/Game/Teleportation_VFX/Particles/P_Spawn_StMesh.P_Spawn_StMesh" (.component _array_element) "None" "0, 0, 0" "0, 0, 0" "KeepRelativeOffset" true))
        (Effects|Components|ParticleSystem|SetColorParameter _returnvalue_7 "User.color" (Variables|Parameters|GetColor))
        (Effects|Components|ParticleSystem|SetFloatParameter _returnvalue_7 "User.ColorBoost" (Variables|Parameters|GetColorBoost))
        (Effects|Components|ParticleSystem|SetFloatParameter _returnvalue_7 "User.Height" (Variables|Parameters|GetHeight))
        (Effects|Components|ParticleSystem|SetFloatParameter _returnvalue_7 "User.Size" (Variables|Parameters|GetEffect_Size))))))

(event Custom|Dissolve
  ;[1 1 1] Dissolve components
  (Components|Timeline|SetPlayRate (Variables|Default|GetDissolveMesh_Timeline) (Variables|Parameters|GetSpeed))
  (bind _dissolve (Timeline|DissolveMesh_Timeline PlayFromStart)
    (:Update
      (for _array_element (Variables|Default|GetMeshesReferences)
        (bind _asmesh_component (Utilities|Casting|CastToMeshComponent (.component _array_element)))
        (Rendering|Material|SetScalarParameterValueonMaterials _asmesh_component "Boost" (Variables|Parameters|GetColorBoost))
        (Rendering|Material|SetScalarParameterValueonMaterials _asmesh_component "Z_Location" (.z (Transformation|GetActorLocation (Variables|Parameters|GetTarget)))))
      (for _array_element_2 (Variables|Default|GetMeshesReferences)
        (Utilities|FlowControl|Sequence
          (:then_0
            (bind _asmesh_component_2 (Utilities|Casting|CastToMeshComponent (.component _array_element_2)))
            (Rendering|Material|SetScalarParameterValueonMaterials _asmesh_component_2 "Dissolve_Amount" (* _dissolve (Variables|Parameters|GetHeight)))))))
    (:Finished
      (CallFunction|Teleportation))))

(event Custom|Spawn
  ;[1 1 1] Dissolve components
  (Components|Timeline|SetPlayRate (Variables|Default|GetSpawn_Timeline) (Variables|Parameters|GetSpeed))
  (bind _spawn (Timeline|Spawn_Timeline PlayFromStart)
    (:Update
      (for _array_element (Variables|Default|GetMeshesReferences)
        (bind _asmesh_component (Utilities|Casting|CastToMeshComponent (.component _array_element)))
        (Rendering|Material|SetScalarParameterValueonMaterials _asmesh_component "Dissolve_Amount" (* _spawn (Variables|Parameters|GetHeight)))
        (Rendering|Material|SetScalarParameterValueonMaterials _asmesh_component "Z_Location" (.z (Transformation|GetActorLocation (Variables|Parameters|GetTarget))))))
    (:Finished
      (for _array_element_2 (Variables|Default|GetMeshesReferences)
        (bind _asmesh_component_2 (Utilities|Casting|CastToMeshComponent (.component _array_element_2)))
        (Rendering|Material|SetScalarParameterValueonMaterials _asmesh_component_2 "Boost" 0.0)
        (Rendering|Material|SetScalarParameterValueonMaterials _asmesh_component_2 "Dissolve_Amount" -1e+04)
        (Actor|DestroyActor)))))

(event EventBeginPlay
  (bind _effectrotation (Variables|Parameters|GetEffectRotation))
  (bind _color (Variables|Parameters|GetColor))
  (bind _target (Variables|Parameters|GetTarget))
  (bind _dissoveeffect_choice (Variables|Parameters|GetDissoveEffect_Choice))
  (bind (_r _g _b) (Math|Color|BreakColor _color))
  (bind _returnvalue (Transformation|GetActorLocation _target))
  ;[1 1 1] Get all components
  (for _array_element (Actor|GetComponentsByClass (Variables|Parameters|GetTarget) "/Script/Engine.SceneComponent")
    (bind _asmesh_component (Utilities|Casting|CastToMeshComponent _array_element))
    (Utilities|Array|AddUnique (Variables|Default|GetMeshesReferences) (Utilities|Struct|MakeST_Meshes_References _asmesh_component (Rendering|Material|GetMaterials _asmesh_component))))
  ;[1 1 1] Initialize material parameters
  (for _array_element_2 (Variables|Default|GetMeshesReferences)
    (bind _asmesh_component_2 (Utilities|Casting|CastToMeshComponent (.component _array_element_2)))
    (Rendering|Material|SetScalarParameterValueonMaterials _asmesh_component_2 "Z_Location" (.z (Transformation|GetActorLocation (Variables|Parameters|GetTarget))))
    (Rendering|Material|SetScalarParameterValueonMaterials _asmesh_component_2 "Height" (Variables|Parameters|GetHeight))
    (Rendering|Material|SetScalarParameterValueonMaterials _asmesh_component_2 "Boost" 0.0)
    (Rendering|Material|SetScalarParameterValueonMaterials _asmesh_component_2 "Red" _r)
    (Rendering|Material|SetScalarParameterValueonMaterials _asmesh_component_2 "Green" _g)
    (Rendering|Material|SetScalarParameterValueonMaterials _asmesh_component_2 "Blue" _b))
  ;[1 1 1] Spawn teleportation effect
  (CallFunction|Dissolve)
  (bind (_outhit _returnvalue_2) (Collision|LineTraceByChannel (+ _returnvalue "0, 0,10.000000") (- _returnvalue "0, 0,1000.000000") "TraceTypeQuery1" false (Utilities|Array|MakeArray _target) "None"))
  (if _returnvalue_2
    (bind _returnvalue_3 (Niagara|SpawnSystematLocation _dissoveeffect_choice (.ImpactPoint (Collision|BreakHitResult _outhit)) _effectrotation))
    (Variables|Default|SetEffect _returnvalue_3)
    (else
      (bind _returnvalue_4 (Niagara|SpawnSystematLocation _dissoveeffect_choice (Transformation|GetActorLocation (Variables|Parameters|GetTarget)) _effectrotation))
      (Variables|Default|SetEffect _returnvalue_4)))
  (Effects|Components|ParticleSystem|SetColorParameter (Variables|Default|GetEffect) "User.color" (Variables|Parameters|GetColor))
  (Effects|Components|ParticleSystem|SetFloatParameter (Variables|Default|GetEffect) "User.ColorBoost" (Variables|Parameters|GetColorBoost))
  (Effects|Components|ParticleSystem|SetFloatParameter (Variables|Default|GetEffect) "User.Height" (Variables|Parameters|GetHeight))
  (Effects|Components|ParticleSystem|SetFloatParameter (Variables|Default|GetEffect) "User.Speed" (/ 1.0 (Variables|Parameters|GetSpeed)))
  (Effects|Components|ParticleSystem|SetFloatParameter (Variables|Default|GetEffect) "User.Size" (Variables|Parameters|GetEffect_Size))
  (Effects|Components|ParticleSystem|SetFloatParameter (Variables|Default|GetEffect) "User.Thickness" (Variables|Parameters|GetCircle_Thickness))
  ;[1 1 1] Dissolve components
  (for _array_element_3 (Variables|Default|GetMeshesReferences)
    (bind _asskeletal_mesh_component (Utilities|Casting|CastToSkeletalMeshComponent (.component _array_element_3))
      (:then
        (bind _returnvalue_5 (Niagara|SpawnSystemAttached "/Game/Teleportation_VFX/Particles/P_Dissolve_SkMesh.P_Dissolve_SkMesh" _asskeletal_mesh_component "None" "0, 0, 0" "0, 0, 0" "KeepRelativeOffset" true))
        (Effects|Components|ParticleSystem|SetColorParameter _returnvalue_5 "User.color" (Variables|Parameters|GetColor))
        (Effects|Components|ParticleSystem|SetFloatParameter _returnvalue_5 "User.ColorBoost" (Variables|Parameters|GetColorBoost))
        (Effects|Components|ParticleSystem|SetFloatParameter _returnvalue_5 "User.Height" (Variables|Parameters|GetHeight)))
      (:CastFailed
        (bind _returnvalue_6 (Niagara|SpawnSystemAttached "/Game/Teleportation_VFX/Particles/P_Dissolve_StMesh.P_Dissolve_StMesh" (.component _array_element_3) "None" "0, 0, 0" "0, 0, 0" "KeepRelativeOffset" true))
        (Effects|Components|ParticleSystem|SetColorParameter _returnvalue_6 "User.color" (Variables|Parameters|GetColor))
        (Effects|Components|ParticleSystem|SetFloatParameter _returnvalue_6 "User.ColorBoost" (Variables|Parameters|GetColorBoost))
        (Effects|Components|ParticleSystem|SetFloatParameter _returnvalue_6 "User.Height" (Variables|Parameters|GetHeight))))))

(event EventTick
  (params (DeltaSeconds :type Float%20%28single-precision%29))
  (bind _target (Variables|Parameters|GetTarget))
  (bind _effect (Variables|Default|GetEffect))
  (bind _returnvalue (Transformation|GetActorLocation _target))
  ;[1 1 1] Update effect location
  (if (Variables|Parameters|GetbFollowActor?)
    (Utilities|IsValid (Variables|Default|GetEffect)
      (:Is%20Valid
        (bind (_outhit _returnvalue_2) (Collision|LineTraceByChannel (+ _returnvalue "0, 0,10.000000") (- _returnvalue "0, 0,1000.000000") "TraceTypeQuery1" false (Utilities|Array|MakeArray _target) "None"))
        (if _returnvalue_2
          (Transformation|SetWorldLocation _effect (.ImpactPoint (Collision|BreakHitResult _outhit)) false true)
          (else
            (Transformation|SetWorldLocation _effect (Transformation|GetActorLocation (Variables|Parameters|GetTarget)) false true)))))))

(fn ConstructionScript)