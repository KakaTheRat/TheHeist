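; Example actor for the Teleportation VFX content that continuously demonstrates teleport spawn effects on sample characters.
; From BeginPlay, a FlipFlop alternates between spawning running and idle characters at random horizontal offsets around the actor.
; Each character gets a BP_SpawnActor using the same particle effect, with follow enabled for the runner and rings for the idle one.
; After a delay the character is destroyed and a custom event restarts the cycle.
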(event Custom|SpawnActor
  (bind _returnvalue (Transformation|GetActorLocation))
  (bind _returnvalue_2 (Transformation|GetActorRotation))
  (bind _returnvalue_3 (Math|Random|RandomFloatinRange -2e+02 2e+02))
  (bind _returnvalue_4 (Math|Random|RandomFloatinRange -2e+02 2e+02))
  (bind _returnvalue_5 (+ _returnvalue (Math|Vector|MakeVector _returnvalue_4 _returnvalue_3 0.0)))
  (Utilities|FlowControl|FlipFlop
    (:A
      (bind _returnvalue_6 (Game|SpawnActorfromClass "/Game/Teleportation_VFX/Blueprints/BP_Character_Ex_Run.BP_Character_Ex_Run_C" (Math|Transform|MakeTransform _returnvalue_5 _returnvalue_2 "1,1,1") "Undefined" 0 1.8e+02 0))
      (bind _output_get (Variables|Default|SetActor _returnvalue_6))
      (Game|SpawnActorfromClass "/Game/Teleportation_VFX/Blueprints/BP_SpawnActor.BP_SpawnActor_C" (Math|Transform|MakeTransform "0, 0, 0" "0, 0, 0" "1,1,1") "Undefined" 0 _output_get false true true "(R=0.000000,G=0.565187,B=0.963542,A=1.000000)" 5e+01 1.0 2e+02 1.0 1.0 "0.000000,0.000000,0.000000" "/Game/Teleportation_VFX/Particles/P_TeleportSpawn_01.P_TeleportSpawn_01" 0))
    (:B
      (bind _returnvalue_7 (Game|SpawnActorfromClass "/Game/Teleportation_VFX/Blueprints/BP_Character_Ex_Idle.BP_Character_Ex_Idle_C" (Math|Transform|MakeTransform _returnvalue_5 _returnvalue_2 "1,1,1") "Undefined" 0 1.8e+02 0))
      (bind _output_get_2 (Variables|Default|SetActor _returnvalue_7))
      (Game|SpawnActorfromClass "/Game/Teleportation_VFX/Blueprints/BP_SpawnActor.BP_SpawnActor_C" (Math|Transform|MakeTransform "0, 0, 0" "0, 0, 0" "1,1,1") "Undefined" 0 _output_get_2 true true false "(R=0.000000,G=0.565187,B=0.963542,A=1.000000)" 5e+01 1.0 2e+02 1.0 1.0 "0.000000,0.000000,0.000000" "/Game/Teleportation_VFX/Particles/P_TeleportSpawn_01.P_TeleportSpawn_01" 0)))
  (Utilities|FlowControl|Delay 4.0)
  (Actor|DestroyActor (Variables|Default|GetActor))
  (CallFunction|SpawnActor))

(event EventBeginPlay
  (bind _returnvalue (Transformation|GetActorLocation))
  (bind _returnvalue_2 (Transformation|GetActorRotation))
  (bind _returnvalue_3 (Math|Random|RandomFloatinRange -2e+02 2e+02))
  (bind _returnvalue_4 (Math|Random|RandomFloatinRange -2e+02 2e+02))
  (bind _returnvalue_5 (+ _returnvalue (Math|Vector|MakeVector _returnvalue_4 _returnvalue_3 0.0)))
  (Utilities|FlowControl|FlipFlop
    (:A
      (bind _returnvalue_6 (Game|SpawnActorfromClass "/Game/Teleportation_VFX/Blueprints/BP_Character_Ex_Run.BP_Character_Ex_Run_C" (Math|Transform|MakeTransform _returnvalue_5 _returnvalue_2 "1,1,1") "Undefined" 0 1.8e+02 0))
      (bind _output_get (Variables|Default|SetActor _returnvalue_6))
      (Game|SpawnActorfromClass "/Game/Teleportation_VFX/Blueprints/BP_SpawnActor.BP_SpawnActor_C" (Math|Transform|MakeTransform "0, 0, 0" "0, 0, 0" "1,1,1") "Undefined" 0 _output_get false true true "(R=0.000000,G=0.565187,B=0.963542,A=1.000000)" 5e+01 1.0 2e+02 1.0 1.0 "0.000000,0.000000,0.000000" "/Game/Teleportation_VFX/Particles/P_TeleportSpawn_01.P_TeleportSpawn_01" 0))
    (:B
      (bind _returnvalue_7 (Game|SpawnActorfromClass "/Game/Teleportation_VFX/Blueprints/BP_Character_Ex_Idle.BP_Character_Ex_Idle_C" (Math|Transform|MakeTransform _returnvalue_5 _returnvalue_2 "1,1,1") "Undefined" 0 1.8e+02 0))
      (bind _output_get_2 (Variables|Default|SetActor _returnvalue_7))
      (Game|SpawnActorfromClass "/Game/Teleportation_VFX/Blueprints/BP_SpawnActor.BP_SpawnActor_C" (Math|Transform|MakeTransform "0, 0, 0" "0, 0, 0" "1,1,1") "Undefined" 0 _output_get_2 true true false "(R=0.000000,G=0.565187,B=0.963542,A=1.000000)" 5e+01 1.0 2e+02 1.0 1.0 "0.000000,0.000000,0.000000" "/Game/Teleportation_VFX/Particles/P_TeleportSpawn_01.P_TeleportSpawn_01" 0)))
  (Utilities|FlowControl|Delay 4.0)
  (Actor|DestroyActor (Variables|Default|GetActor))
  (CallFunction|SpawnActor))

(fn ConstructionScript)