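; Example actor from the teleportation VFX content that repeatedly spawns BP_TeleportationWithoutEffect on a Target, passing through its exposed appearance and timing settings.
; BeginPlay triggers the first spawn, and a Delay on Tick repeats it at an interval inversely scaled by Speed.
; It uses the set Destination if ChooseDestination is true; otherwise a FlipFlop alternates Y offsets from the Target's current location, overriding its rotation.
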(event EventBeginPlay
  (bind _spawneffectchoice (Variables|Default|GetSpawnEffectChoice))
  (bind _dissolveeffect_choice (Variables|Default|GetDissolveEffect_Choice))
  (bind _target (Variables|Default|GetTarget))
  (bind _bfollowactor_ (Variables|Default|GetbFollowActor?))
  (bind _speed (Variables|Default|GetSpeed))
  (bind _effect_size (Variables|Default|GetEffect_Size))
  (bind _circle_thickness (Variables|Default|GetCircle_Thickness))
  (bind _returnvalue (Transformation|GetActorLocation _target))
  (if (Variables|Default|GetbChooseDestination?)
    (Game|SpawnActorfromClass "/Game/Teleportation_VFX/Blueprints/BP_TeleportationWithoutEffect.BP_TeleportationWithoutEffect_C" (Math|Transform|MakeTransform "0, 0, 0" "0, 0, 0" "1,1,1") "Undefined" 0 (Variables|Default|GetTarget) (Variables|Default|GetHeight) (Variables|Default|GetDestination) (Variables|Default|GetColor) (Variables|Default|GetBoost) true "0.000000,0.000000,0.000000" (Variables|Default|GetbFollowActor?) (Variables|Default|GetSpeed) (Variables|Default|GetEffect_Size) (Variables|Default|GetCircle_Thickness) (Variables|Default|GetDissolveEffect_Choice) (Variables|Default|GetSpawnEffectChoice) (Variables|Default|GetEffectRotation) 0)
    (else
      (Utilities|FlowControl|FlipFlop
        (:A
          (Game|SpawnActorfromClass "/Game/Teleportation_VFX/Blueprints/BP_TeleportationWithoutEffect.BP_TeleportationWithoutEffect_C" (Math|Transform|MakeTransform "0, 0, 0" "0, 0, 0" "1,1,1") "Undefined" 0 _target (Variables|Default|GetHeight) (+ _returnvalue "0.000000,-200.000000,0.000000") (Variables|Default|GetColor) (Variables|Default|GetBoost) false "0.000000,180.000000,0.000000" _bfollowactor_ _speed _effect_size _circle_thickness _dissolveeffect_choice _spawneffectchoice (Variables|Default|GetEffectRotation) 0))
        (:B
          (Game|SpawnActorfromClass "/Game/Teleportation_VFX/Blueprints/BP_TeleportationWithoutEffect.BP_TeleportationWithoutEffect_C" (Math|Transform|MakeTransform "0, 0, 0" "0, 0, 0" "1,1,1") "Undefined" 0 _target (Variables|Default|GetHeight) (+ _returnvalue "0.000000,200.000000,0.000000") (Variables|Default|GetColor) (Variables|Default|GetBoost) false "0.000000,0.000000,0.000000" _bfollowactor_ _speed _effect_size _circle_thickness _dissolveeffect_choice _spawneffectchoice (Variables|Default|GetEffectRotation) 0))))))

(event EventTick
  (params (DeltaSeconds :type Float%20%28single-precision%29))
  (bind _spawneffectchoice (Variables|Default|GetSpawnEffectChoice))
  (bind _dissolveeffect_choice (Variables|Default|GetDissolveEffect_Choice))
  (bind _target (Variables|Default|GetTarget))
  (bind _bfollowactor_ (Variables|Default|GetbFollowActor?))
  (bind _speed (Variables|Default|GetSpeed))
  (bind _effect_size (Variables|Default|GetEffect_Size))
  (bind _circle_thickness (Variables|Default|GetCircle_Thickness))
  (bind _returnvalue (Transformation|GetActorLocation _target))
  (Utilities|FlowControl|Delay (* 7.0 (/ 1.0 (Variables|Default|GetSpeed))))
  (if (Variables|Default|GetbChooseDestination?)
    (Game|SpawnActorfromClass "/Game/Teleportation_VFX/Blueprints/BP_TeleportationWithoutEffect.BP_TeleportationWithoutEffect_C" (Math|Transform|MakeTransform "0, 0, 0" "0, 0, 0" "1,1,1") "Undefined" 0 (Variables|Default|GetTarget) (Variables|Default|GetHeight) (Variables|Default|GetDestination) (Variables|Default|GetColor) (Variables|Default|GetBoost) true "0.000000,0.000000,0.000000" (Variables|Default|GetbFollowActor?) (Variables|Default|GetSpeed) (Variables|Default|GetEffect_Size) (Variables|Default|GetCircle_Thickness) (Variables|Default|GetDissolveEffect_Choice) (Variables|Default|GetSpawnEffectChoice) (Variables|Default|GetEffectRotation) 0)
    (else
      (Utilities|FlowControl|FlipFlop
        (:A
          (Game|SpawnActorfromClass "/Game/Teleportation_VFX/Blueprints/BP_TeleportationWithoutEffect.BP_TeleportationWithoutEffect_C" (Math|Transform|MakeTransform "0, 0, 0" "0, 0, 0" "1,1,1") "Undefined" 0 _target (Variables|Default|GetHeight) (+ _returnvalue "0.000000,-200.000000,0.000000") (Variables|Default|GetColor) (Variables|Default|GetBoost) false "0.000000,180.000000,0.000000" _bfollowactor_ _speed _effect_size _circle_thickness _dissolveeffect_choice _spawneffectchoice (Variables|Default|GetEffectRotation) 0))
        (:B
          (Game|SpawnActorfromClass "/Game/Teleportation_VFX/Blueprints/BP_TeleportationWithoutEffect.BP_TeleportationWithoutEffect_C" (Math|Transform|MakeTransform "0, 0, 0" "0, 0, 0" "1,1,1") "Undefined" 0 _target (Variables|Default|GetHeight) (+ _returnvalue "0.000000,200.000000,0.000000") (Variables|Default|GetColor) (Variables|Default|GetBoost) false "0.000000,0.000000,0.000000" _bfollowactor_ _speed _effect_size _circle_thickness _dissolveeffect_choice _spawneffectchoice (Variables|Default|GetEffectRotation) 0))))))

(fn ConstructionScript)