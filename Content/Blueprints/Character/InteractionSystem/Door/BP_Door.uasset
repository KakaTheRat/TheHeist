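; Interactable door actor that opens, closes or acts locked, with paired character and door animations.
; A DoOnce-gated Interaction picks the front or back anchor by the overlapping character's distance, then a timeline aligns the character while collision and movement input are off.
; Side and door state select montage and door animation; notifies trigger sounds.
; Camera view limits clamp after alignment; montage completion toggles open/closed and restores control.
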(event Custom|Interaction
  (Utilities|FlowControl|DoOnce false
    (:Completed
      (CallFunction|CheckEngagementPosition)
      (CallFunction|StartInteractionDoor))))

(event Custom|PlayInteractionMontage
  (bind _door (Variables|Default|GetDoor))
  (bind _character (Variables|Default|GetCharacter))
  (bind _returnvalue (Transformation|GetWorldLocation _door))
  (bind _returnvalue_2 (Class|EntitiesInterface|GetSkeletalMeshComponent(Message) (Variables|Default|GetCharacter)))
  (bind _notifyname (Animation|Montage|PlayMontage _returnvalue_2 (CallFunction|FindCharacterMontage))
    (:then
      (Components|Animation|PlayAnimation (Variables|Default|GetDoor) (CallFunction|FindDoorAnimation) false))
    (:OnCompleted
      (Variables|Default|SetDoorState (Utilities|Select :Index (Variables|Default|GetDoorState) :NewEnumerator0 "NewEnumerator1" :NewEnumerator1 "NewEnumerator0" :NewEnumerator2 "NewEnumerator2"))
      (Input|ResetIgnoreMoveInput (Game|GetPlayerController 0))
      (Collision|SetCollisionEnabled (Variables|/Script/Engine.Character|GetCapsuleComponent _character) "QueryAndPhysics")
      (Pawn|Components|CharacterMovement|SetMovementMode (Variables|/Script/Engine.Character|GetCharacterMovement _character) "MOVE_Walking" 0)
      (CallFunction|UnlockCamera)
      (CallFunction|ResetInteraction))
    (:OnNotifyBegin
      (switch name _notifyname
        (:Locked
          (Audio|PlaySoundatLocation "/Game/Audio/SFX/Interaction/Door/S_DoorLock.S_DoorLock" _returnvalue "0, 0, 0" 1.0 1.0 0.0 0 0 0 0))
        (:Open
          (Audio|PlaySoundatLocation "/Game/Audio/SFX/Interaction/Door/S_DoorOpen.S_DoorOpen" _returnvalue "0, 0, 0" 1.0 1.0 0.0 0 0 0 0))
        (:Close
          (Audio|PlaySoundatLocation "/Game/Audio/SFX/Interaction/Door/S_DoorClose.S_DoorClose" _returnvalue "0, 0, 0" 1.0 1.0 0.0 0 0 0 0))))))

(event Custom|StartInteractionDoor
  (bind _returnvalue (Game|GetPlayerController 0))
  (bind _character (Variables|Default|GetCharacter))
  (bind _returnvalue_2 (Pawn|GetControlRotation _returnvalue :!class /Script/Engine.Controller))
  (bind (_roll _pitch) (Math|Rotator|BreakRotator _returnvalue_2))
  ;[0.15 0.15 0.15 0.5] Start Interaction Door Position
  (Collision|SetCollisionEnabled (Variables|/Script/Engine.Character|GetCapsuleComponent _character) "NoCollision")
  (Pawn|Components|CharacterMovement|SetMovementMode (Variables|/Script/Engine.Character|GetCharacterMovement _character) "MOVE_Flying" 0)
  (Input|SetIgnoreMoveInput (Game|GetPlayerController 0) true)
  (CallFunction|PlayInteractionMontage)
  (bind _alpha (Timeline|SetPlayerPositionTimeline PlayFromStart)
    (:Update
      (Pawn|SetControlRotation (Game|GetPlayerController 0) (Math|Rotator|Lerp(Rotator) _returnvalue_2 (Math|Rotator|MakeRotator _roll _pitch (.yaw (Transformation|GetWorldRotation (Utilities|Select :Index (Variables|Default|GetPosition) :NewEnumerator0 (Variables|Default|GetFrontPosition) :NewEnumerator1 (Variables|Default|GetBackPosition))))) _alpha true))
      (Transformation|SetActorLocationAndRotation (Variables|Default|GetCharacter) (Math|Vector|Lerp(Vector) (Transformation|GetActorLocation (Variables|Default|GetCharacter)) (Transformation|GetWorldLocation (Utilities|Select :Index (Variables|Default|GetPosition) :NewEnumerator0 (Variables|Default|GetFrontPosition) :NewEnumerator1 (Variables|Default|GetBackPosition))) _alpha) (Math|Rotator|Lerp(Rotator) (Transformation|GetActorRotation (Variables|Default|GetCharacter)) (Transformation|GetWorldRotation (Utilities|Select :Index (Variables|Default|GetPosition) :NewEnumerator0 (Variables|Default|GetFrontPosition) :NewEnumerator1 (Variables|Default|GetBackPosition))) _alpha true)))
    (:Finished
      (CallFunction|DoorCameraLock))))

(event Custom|ResetInteraction
  (Utilities|FlowControl|DoOnce false) ; enters at Reset
)

(event Custom|UnlockCamera
  (bind _returnvalue (Game|GetPlayerController 0))
  (bind _playercameramanager (Variables|/Script/Engine.PlayerController|GetPlayerCameraManager _returnvalue))
  (Utilities|IsValid _returnvalue
    (:Is%20Valid
      (Variables|/Script/Engine.PlayerCameraManager|SetViewYawMin _playercameramanager 0.0)
      (Variables|/Script/Engine.PlayerCameraManager|SetViewYawMax _playercameramanager 359.998993)
      (Variables|/Script/Engine.PlayerCameraManager|SetViewPitchMin _playercameramanager -75.0)
      (Variables|/Script/Engine.PlayerCameraManager|SetViewPitchMax _playercameramanager 75.0))))

(event Custom|DoorCamera%20Lock
  (bind _returnvalue (Game|GetPlayerController 0))
  (bind _position (Variables|Default|GetPosition))
  (bind _frontposition (Variables|Default|GetFrontPosition))
  (bind _backposition (Variables|Default|GetBackPosition))
  (bind _returnvalue_2 (Utilities|Select :Index _position :NewEnumerator0 _frontposition :NewEnumerator1 _backposition))
  (bind _playercameramanager (Variables|/Script/Engine.PlayerController|GetPlayerCameraManager _returnvalue))
  (bind _returnvalue_3 (Transformation|GetWorldRotation _returnvalue_2))
  ;[0.15 0.15 0.15 0.5] Ladder Lock Camera
  (Utilities|IsValid _returnvalue
    (:Is%20Valid
      (Variables|/Script/Engine.PlayerCameraManager|SetViewYawMin _playercameramanager (- (.yaw _returnvalue_3) 1.2e+02))
      (Variables|/Script/Engine.PlayerCameraManager|SetViewYawMax _playercameramanager (+ (.yaw _returnvalue_3) 75.0))
      (Variables|/Script/Engine.PlayerCameraManager|SetViewPitchMin _playercameramanager (- (.pitch _returnvalue_3) 75.0))
      (Variables|/Script/Engine.PlayerCameraManager|SetViewPitchMax _playercameramanager (+ (.pitch _returnvalue_3) 75.0))
      (Development|PrintString "Hello"))))

(event EventBeginPlay)

(event Collision|EventActorBeginOverlap
  (params (OtherActor :type Actor%20Object%20Reference))
  (bind _ascharacter (Utilities|Casting|CastToCharacter OtherActor))
  (Utilities|IsValid _ascharacter
    (:Is%20Valid
      (Variables|Default|SetCharacter _ascharacter))))

(event EventTick
  (params (DeltaSeconds :type Float%20%28single-precision%29)))

(event Collision|EventActorEndOverlap
  (params (OtherActor :type Actor%20Object%20Reference)))

(event EventInteract
  (params (HitComponent :type Scene%20Component%20Object%20Reference) (InteractingActor :type Actor%20Object%20Reference) (Context :type EInteractionContext%20Enum :default "Default") (Data :type Interaction%20Data%20Object%20Reference))
  (Utilities|FlowControl|DoOnce false
    (:Completed
      (CallFunction|CheckEngagementPosition)
      (CallFunction|StartInteractionDoor))))

(fn ConstructionScript)

(fn CheckEngagementPosition
  (if (<= (Math|Vector|VectorLength (- (Transformation|GetActorLocation (Variables|Default|GetCharacter)) (Transformation|GetWorldLocation (Variables|Default|GetFrontPosition)))) 5e+01)
    (Variables|Default|SetPosition "NewEnumerator0")
    (elif (<= (Math|Vector|VectorLength (- (Transformation|GetActorLocation (Variables|Default|GetCharacter)) (Transformation|GetWorldLocation (Variables|Default|GetBackPosition)))) 5e+01)
      (Variables|Default|SetPosition "NewEnumerator1"))))

(fn FindCharacterMontage
  (return (Utilities|Select :Index (Variables|Default|GetPosition) :NewEnumerator0 (Utilities|Select :Index (Variables|Default|GetDoorState) :NewEnumerator0 "/Game/11_Animations/Door/AnimatedDoor/A_Idle_Door_Front_OpenFull_MontageReal.A_Idle_Door_Front_OpenFull_MontageReal" :NewEnumerator1 "/Game/11_Animations/Door/AnimatedDoor/A_Idle_Door_Front_CloseFull_MontageReal.A_Idle_Door_Front_CloseFull_MontageReal" :NewEnumerator2 "/Game/11_Animations/CardReader/A_Cardrider_Activate_Montage.A_Cardrider_Activate_Montage") :NewEnumerator1 (Utilities|Select :Index (Variables|Default|GetDoorState) :NewEnumerator0 "/Game/11_Animations/Door/AnimatedDoor/A_Idle_Door_Back_OpenFull_MontageReal.A_Idle_Door_Back_OpenFull_MontageReal" :NewEnumerator1 "/Game/11_Animations/Door/AnimatedDoor/A_Idle_Door_Back_CloseFull_MontageReal.A_Idle_Door_Back_CloseFull_MontageReal" :NewEnumerator2 "/Game/Characters/Animations/Interaction/Door/A_Idle_Door_Back_LockedFull_Montage.A_Idle_Door_Back_LockedFull_Montage"))))

(fn FindDoorAnimation
  (return (Utilities|Select :Index (Variables|Default|GetPosition) :NewEnumerator0 (Utilities|Select :Index (Variables|Default|GetDoorState) :NewEnumerator0 "/Game/Meshes/Interaction/Door/Animation/A_Door_Open_F_Full.A_Door_Open_F_Full" :NewEnumerator1 "/Game/Meshes/Interaction/Door/Animation/A_Door_Open_F_CloseFull.A_Door_Open_F_CloseFull" :NewEnumerator2 "/Game/Meshes/Interaction/Door/Animation/A_Door_Locked.A_Door_Locked") :NewEnumerator1 (Utilities|Select :Index (Variables|Default|GetDoorState) :NewEnumerator0 "/Game/Meshes/Interaction/Door/Animation/A_Door_Open_B_Full.A_Door_Open_B_Full" :NewEnumerator1 "/Game/Meshes/Interaction/Door/Animation/A_Door_Close_B_Full.A_Door_Close_B_Full" :NewEnumerator2 "/Game/Meshes/Interaction/Door/Animation/A_Door_Close_B_Locked.A_Door_Close_B_Locked"))))