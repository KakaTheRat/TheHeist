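; Base interactable actor that the player picks up by hand, registering with the player's BPInteractionComponent on overlap and highlighting through custom depth.
; Interaction disables physics and collision, then requests a pickup montage, which plays only if the player is neither falling nor mid-montage.
; The mesh location feeds the AnimBlueprint's hand IK target.
; Montage notifies trigger attachment to the hand socket with a sound, then destroy the actor and finish the interaction.
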(event Collision|EventHit
  (params (MyComp :type Primitive%20Component%20Object%20Reference) (Other :type Actor%20Object%20Reference) (OtherComp :type Primitive%20Component%20Object%20Reference) (bSelfMoved :type Boolean) (HitLocation :type Vector :default "0, 0, 0") (HitNormal :type Vector :default "0, 0, 0") (NormalImpulse :type Vector :default "0, 0, 0") (Hit :type Hit%20Result%20Structure%20%28by%20ref%29)))

(event EventBeginPlay)

(event EventInteraction
  (params (Player :type BP%20Player%20Object%20Reference))
  (bind _output_get (Variables|Default|SetPlayer Player))
  (Variables|Default|SetBP%20Interaction%20Component (.BP_InteractionComponent (Variables|/Game/Blueprints/Character/BP_Player.BP_Player_C|GetBP_InteractionComponent _output_get)))
  (CallFunction|InteractionEnable false)
  (Utilities|PlayInteractableMontage "/Game/Characters/Animations/Interaction/PickUp_R_Hand_Bottle_Montage.PickUp_R_Hand_Bottle_Montage"
    (:then
      (CallFunction|UpdateInteractLocation)
      (Rendering|SetRenderCustomDepth (Variables|Default|GetStaticMesh) false))
    (:Interact
      (CallFunction|AttachtoHand))
    (:Destroy
      (Actor|DestroyActor)
      (Default|FinishInteraction (Variables|Default|GetBP%20Interaction%20Component)))))

(event EventDefineActor
  (params (Result :type Boolean))
  (Rendering|SetRenderCustomDepth (Variables|Default|GetStaticMesh) Result))

(event Collision|EventActorBeginOverlap
  (params (OtherActor :type Actor%20Object%20Reference))
  (bind _playercharacter (Class|BPIPlayer|GetPlayer(Message) OtherActor))
  (Utilities|IsValid _playercharacter
    (:Is%20Valid
      (Default|HandleRegister (.BP_InteractionComponent (Variables|/Game/Blueprints/Character/BP_Player.BP_Player_C|GetBP_InteractionComponent _playercharacter)) self))))

(event Collision|EventActorEndOverlap
  (params (OtherActor :type Actor%20Object%20Reference))
  (bind _playercharacter (Class|BPIPlayer|GetPlayer(Message) OtherActor))
  (Utilities|IsValid _playercharacter
    (:Is%20Valid
      (Default|HandleUnregister (.BP_InteractionComponent (Variables|/Game/Blueprints/Character/BP_Player.BP_Player_C|GetBP_InteractionComponent _playercharacter)) self))))

(fn ConstructionScript)

(fn InteractionEnable
  (params (Enable? :type Boolean))
  (Physics|SetSimulatePhysics (Variables|Default|GetStaticMesh) Enable?)
  (Collision|SetActorEnableCollision Enable?)
  (Variables|/Game/Blueprints/Character/InteractionSystem/BP_InteractionComponent.BP_InteractionComponent_C|SetInteractionEnable? (.BP_InteractionComponent (Variables|/Game/Blueprints/Character/BP_Player.BP_Player_C|GetBP_InteractionComponent (Variables|Default|GetPlayer))) Enable?)
  (return))

(fn AttachtoHand
  (Transformation|AttachComponentToComponent (Variables|/Script/Engine.Character|GetMesh (Variables|Default|GetPlayer)) "weapon_r" "SnapToTarget" "SnapToTarget" "KeepRelative" true)
  (Audio|PlaySoundatLocation "/Game/Audio/Foley/MetaSounds/MSS_FoleySound_Handplant.MSS_FoleySound_Handplant" (Transformation|GetActorLocation) "0, 0, 0" 1.0 1.0 0.0 0 0 0 0)
  (return))

(fn UpdateInteractLocation
  (bind _staticmesh (Variables|Default|GetStaticMesh))
  (bind _returnvalue (Transformation|GetWorldLocation _staticmesh))
  (bind (_x _y _z) (Math|Vector|BreakVector _returnvalue))
  (Variables|/Game/Characters/Animations/ABP_Character.ABP_Character_C|SetInteraction%20Hand%20IK%20Position (Variables|/Game/Blueprints/Character/BP_Player.BP_Player_C|GetAnim%20Blueprint (Variables|Default|GetPlayer)) (Math|Vector|MakeVector _x _y _z)))

(fn TargetCenterOfMass
  (return (Variables|Default|GetStaticMesh)))