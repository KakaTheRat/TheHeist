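; BP_Cardrider is an interactable card reader that plays a swipe animation and activates linked actors.
; Overlapping actors register it with their interaction component; interaction is DoOnce-gated, disables input and lerps character and camera yaw to the Arrow.
; During the montage the card attaches to the character's hand.
; A montage notify messages ActivationActors and updates the screen widget, light and sounds; completion restores input and walking and re-arms interaction.
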(event Custom|UpdatePlayerPosition
  (bind _returnvalue (Game|GetPlayerController 0))
  (bind _arrow (Variables|Default|GetArrow))
  (bind _returnvalue_2 (Pawn|GetControlRotation _returnvalue :!class /Script/Engine.Controller))
  (bind (_roll _pitch) (Math|Rotator|BreakRotator _returnvalue_2))
  (CallFunction|PlayMontageCardrider)
  (bind _alpha (Timeline|SetPosition PlayFromStart)
    (:Update
      (Pawn|SetControlRotation (Game|GetPlayerController 0) (Math|Rotator|Lerp(Rotator) _returnvalue_2 (Math|Rotator|MakeRotator _roll _pitch (.yaw (Transformation|GetWorldRotation (Variables|Default|GetArrow)))) _alpha true))
      (Transformation|SetActorLocationAndRotation (Variables|Default|GetCharacter) (Math|Vector|Lerp(Vector) (Transformation|GetActorLocation (Variables|Default|GetCharacter)) (Transformation|GetWorldLocation _arrow) _alpha) (Math|Rotator|Lerp(Rotator) (Transformation|GetActorRotation (Variables|Default|GetCharacter)) (Transformation|GetWorldRotation _arrow) _alpha true)))))

(event Custom|PlayMontageCardrider
  (bind _card (Variables|Default|GetCard))
  (bind _card_2 (Variables|Default|GetCard))
  (bind _character (Variables|Default|GetCharacter))
  (bind _character_2 (Variables|Default|GetCharacter))
  (Variables|/Game/Characters/Animations/ABP_Character.ABP_Character_C|SetbEnableRootYawOffset (Variables|/Game/Blueprints/Character/BP_Player.BP_Player_C|GetAnim%20Blueprint _character) false)
  (Pawn|Components|CharacterMovement|SetMovementMode (Variables|/Script/Engine.Character|GetCharacterMovement _character) "MOVE_Flying" 0)
  (bind _notifyname (Animation|Montage|PlayMontage (Variables|/Script/Engine.Character|GetMesh (Variables|Default|GetCharacter)) "/Game/Characters/Animations/Interaction/Cardrider/A_Cardrider_Activate_Montage.A_Cardrider_Activate_Montage")
    (:then
      (Transformation|AttachComponentToComponent _card_2 (Variables|/Script/Engine.Character|GetMesh (Variables|Default|GetCharacter)) "Weapon_r" "SnapToTarget" "SnapToTarget" "SnapToTarget" true)
      (Rendering|SetVisibility _card_2 true false))
    (:OnCompleted
      (CallFunction|ResetInteraction)
      (Variables|/Game/Characters/Animations/ABP_Character.ABP_Character_C|SetbEnableRootYawOffset (Variables|/Game/Blueprints/Character/BP_Player.BP_Player_C|GetAnim%20Blueprint (Variables|Default|GetCharacter)) true)
      (Input|EnableInput _character_2 (Game|GetPlayerController 0))
      (Pawn|Components|CharacterMovement|SetMovementMode (Variables|/Script/Engine.Character|GetCharacterMovement _character_2) "MOVE_Walking" 0))
    (:OnBlendOut
      (Transformation|AttachComponentToComponent _card (Variables|Default|GetRoot) "Card" "SnapToTarget" "SnapToTarget" "SnapToTarget" true)
      (Rendering|SetVisibility _card false false))
    (:OnNotifyBegin
      (switch name _notifyname
        (:Attach
          (Variables|Light|SetActivate true)
          (Audio|PlaySoundatLocation "/Engine/VREditor/Sounds/UI/Gizmo_Handle_Clicked.Gizmo_Handle_Clicked" (Transformation|GetWorldLocation (Variables|Default|GetRoot)) "0, 0, 0" 1.0 1.0 0.0 "/Game/Audio/Attenuation/Small_Attenuation_200_1000.Small_Attenuation_200_1000" "/Game/Audio/Class/SoundConcurrency_Base.SoundConcurrency_Base" 0 0)
          (for _array_element (Variables|Light|GetActivationActors)
            (Utilities|IsValid _array_element
              (:Is%20Valid
                (Class|BPIActorActivation|Activation(Message) _array_element (Variables|Light|GetActivate)))))
          (Default|UpdateVisualCode (Variables|Default|GetAs%20UI%20Cardrider%20Screen) true)
          (Rendering|Components|Light|SetLightColor (Variables|Default|GetPointLight) "(R=0.003677,G=0.030713,B=0.000000,A=1.000000)" true)
          (Audio|PlaySoundatLocation "/Engine/VREditor/Sounds/UI/Invalid_Action.Invalid_Action" (Transformation|GetWorldLocation (Variables|Default|GetRoot)) "0, 0, 0" 1.0 1.0 0.0 "/Game/Audio/Attenuation/Small_Attenuation_200_1000.Small_Attenuation_200_1000" "/Game/Audio/Class/SoundConcurrency_Base.SoundConcurrency_Base" 0 0))))))

(event Custom|ResetInteraction
  (Utilities|FlowControl|DoOnce false) ; enters at Reset
)

(event EventBeginPlay
  (bind _asui_cardrider_screen (Utilities|Casting|CastToUI_CardriderScreen (UserInterface|GetWidget (Variables|Default|GetWidget))))
  (Variables|Default|SetAs%20UI%20Cardrider%20Screen _asui_cardrider_screen))

(event Collision|EventActorBeginOverlap
  (params (OtherActor :type Actor%20Object%20Reference))
  ;[0.15 0.15 0.15 0.5] Register/Unregister Actor
  (bind _playercharacter (Class|BPIPlayer|GetPlayer(Message) OtherActor))
  (Utilities|IsValid _playercharacter
    (:Is%20Valid
      (Default|HandleRegister (.BP_InteractionComponent (Variables|/Game/Blueprints/Character/BP_Player.BP_Player_C|GetBP_InteractionComponent _playercharacter)) self))))

(event Collision|EventActorEndOverlap
  (params (OtherActor :type Actor%20Object%20Reference))
  ;[0.15 0.15 0.15 0.5] Register/Unregister Actor
  (bind _playercharacter (Class|BPIPlayer|GetPlayer(Message) OtherActor))
  (Utilities|IsValid _playercharacter
    (:Is%20Valid
      (Default|HandleUnregister (.BP_InteractionComponent (Variables|/Game/Blueprints/Character/BP_Player.BP_Player_C|GetBP_InteractionComponent _playercharacter)) self))))

(event EventDefineActor
  (params (Result :type Boolean))
  ;[0.15 0.15 0.15 0.5] Visualization
  (Rendering|SetRenderCustomDepth (Variables|Default|GetRoot) Result))

(event EventTick
  (params (DeltaSeconds :type Float%20%28single-precision%29)))

(event EventInteraction
  (params (Player :type BP%20Player%20Object%20Reference))
  ;[0.15 0.15 0.15 0.5] Interaction
  (Variables|Default|SetCharacter Player)
  (Utilities|FlowControl|DoOnce false
    (:Completed
      (CallFunction|UpdatePlayerPosition)
      (Input|DisableInput (Variables|Default|GetCharacter) (Game|GetPlayerController 0)))))

(fn ConstructionScript)

(fn TargetCenterOfMass
  (return (Variables|Default|GetRoot)))