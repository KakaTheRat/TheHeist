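; Interactable keypad actor that takes a typed code and, when it is correct, sends an activation message to its linked actors.
; Interaction plays an enter montage, timeline-aligns the player to an arrow and moves input to the keypad until exit.
; WASD or numpad selects a key, with the character's IK hand interpolating to its socket.
; Push montage notifies edit or validate the code, updating the screen widget, while a timeline depresses the button.
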(event Custom|UpdatePlayerPosition
  (bind _returnvalue (Game|GetPlayerController 0))
  (bind _returnvalue_2 (Game|GetPlayerController 0))
  (bind _arrow (Variables|Default|GetArrow))
  (bind _returnvalue_3 (Pawn|GetControlRotation _returnvalue :!class /Script/Engine.Controller))
  (bind (_roll _pitch) (Math|Rotator|BreakRotator _returnvalue_3))
  (bind _alpha (Timeline|Timeline PlayFromStart)
    (:Update
      (Pawn|SetControlRotation (Game|GetPlayerController 0) (Math|Rotator|Lerp(Rotator) _returnvalue_3 (Math|Rotator|MakeRotator _roll _pitch (.yaw (Transformation|GetWorldRotation (Variables|Default|GetArrow)))) _alpha true))
      (Transformation|SetActorLocationAndRotation (Variables|Reference|GetCharacter) (Math|Vector|Lerp(Vector) (Transformation|GetActorLocation (Variables|Reference|GetCharacter)) (Transformation|GetWorldLocation _arrow) _alpha) (Math|Rotator|Lerp(Rotator) (Transformation|GetActorRotation (Variables|Reference|GetCharacter)) (Transformation|GetWorldRotation _arrow) _alpha true)))
    (:Finished
      (Input|DisableInput (Variables|Reference|GetCharacter) _returnvalue_2)
      (Input|EnableInput _returnvalue_2)
      (Variables|Default|SetActivateKaypad? true))))

(event Custom|PlayPushMontage
  (bind _returnvalue (Transformation|GetActorLocation))
  (bind _ikpositions (Variables|IK|GetIKPositions))
  (bind _currentindex (Variables|IK|GetCurrentIndex))
  (bind _indextokey (Variables|Code|GetIndexToKey))
  (bind _currentindex_2 (Variables|IK|GetCurrentIndex))
  (bind _value (Utilities|Map|Find _indextokey _currentindex_2))
  (bind _output (Utilities|Array|Get(acopy) _ikpositions _currentindex))
  (bind _relativelocation (Variables|/Script/Engine.SceneComponent|GetRelativeLocation _output))
  (bind _notifyname (Animation|Montage|PlayMontage (Variables|/Script/Engine.Character|GetMesh (Variables|Reference|GetCharacter)) "/Game/Characters/Animations/Interaction/Keypad/A_Keypad_Push_Montage.A_Keypad_Push_Montage")
    (:then
      (bind _alpha (Timeline|LerpButtonLocation PlayFromStart)
        (:Update
          (Transformation|SetRelativeLocation _output (Math|Vector|MakeVector (.x _relativelocation) (.y _relativelocation) (Math|Float|Lerp 1.0 0.5 _alpha)) false false))
        (:Finished
          (CallFunction|ResetPush)
          (Input|EnableInput (Game|GetPlayerController 0)))))
    (:OnNotifyBegin
      (switch name _notifyname
        (:Tuch
          (Audio|PlaySoundatLocation "/Engine/VREditor/Sounds/UI/Click_on_Button_Cue.Click_on_Button_Cue" (Transformation|GetActorLocation) "0, 0, 0" 1.0 1.0 0.0 "/Game/Audio/Attenuation/Small_Attenuation_200_1000.Small_Attenuation_200_1000" "/Game/Audio/Class/SoundConcurrency_Base.SoundConcurrency_Base" 0 0)
          (switch string _value
            (:Default
              (if (not (> (Utilities|String|Len (Variables|Code|GetCurrentCode)) (Variables|Code|GetCodeMaxLenght)))
                (bind _output_get (Variables|Code|SetCurrentCode (Utilities|String|Append (Variables|Code|GetCurrentCode) _value)))
                (Default|UpdateVisualCode (Variables|Reference|GetAs%20UI%20Kaypad%20Screen) _output_get false false)))
            (:Delete
              (bind _output_get_2 (Variables|Code|SetCurrentCode (Utilities|String|Left (Variables|Code|GetCurrentCode) (Math|Integer|Clamp(Integer) (- (Utilities|String|Len (Variables|Code|GetCurrentCode)) 1) 0 (Utilities|String|Len (Variables|Code|GetCurrentCode))))))
              (Default|UpdateVisualCode (Variables|Reference|GetAs%20UI%20Kaypad%20Screen) _output_get_2 false false))
            (:Enter
              (if (Utilities|Enum|Equal(Enum) (Variables|Code|GetCurrentCode) (Variables|Code|GetValidCode))
                (Audio|PlaySoundatLocation "/Engine/EditorSounds/Notifications/CompileStart_Cue.CompileStart_Cue" _returnvalue "0, 0, 0" 1.0 1.0 0.0 "/Game/Audio/Attenuation/Small_Attenuation_200_1000.Small_Attenuation_200_1000" "/Game/Audio/Class/SoundConcurrency_Base.SoundConcurrency_Base" 0 0)
                (Default|UpdateVisualCode (Variables|Reference|GetAs%20UI%20Kaypad%20Screen) (Variables|Code|GetValidCode) true true)
                (CallFunction|ExitKeypad)
                (Collision|SetCollisionEnabled (Variables|Default|GetBox) "NoCollision")
                (for _array_element (Variables|Activation|GetActivationActors)
                  (Utilities|IsValid _array_element
                    (:Is%20Valid
                      (Class|BPIActorActivation|Activation(Message) _array_element true))))
                (else
                  (Audio|PlaySoundatLocation "/Engine/EditorSounds/Notifications/CompileFailed.CompileFailed" _returnvalue "0, 0, 0" 1.0 1.0 0.0 "/Game/Audio/Attenuation/Small_Attenuation_200_1000.Small_Attenuation_200_1000" "/Game/Audio/Class/SoundConcurrency_Base.SoundConcurrency_Base" 0 0)
                  (bind _output_get_3 (Variables|Code|SetCurrentCode ""))
                  (Default|UpdateVisualCode (Variables|Reference|GetAs%20UI%20Kaypad%20Screen) _output_get_3 true false))))))))))

(event Custom|ResetPush
  (Utilities|FlowControl|DoOnce false) ; enters at Reset
)

(event Custom|ExitKeypad
  (bind _returnvalue (Game|GetPlayerController 0))
  (bind _returnvalue_2 (Game|GetPlayerController 0))
  (bind _notifyname (Animation|Montage|PlayMontage (Variables|/Script/Engine.Character|GetMesh (Variables|Reference|GetCharacter)) "/Game/Characters/Animations/Interaction/Keypad/A_Keypad_Exit_Montage.A_Keypad_Exit_Montage")
    (:OnNotifyBegin
      (switch name _notifyname
        (:Exit
          (Variables|/Game/Characters/Animations/ABP_Character.ABP_Character_C|SetGlobalState (Variables|/Game/Blueprints/Character/BP_Player.BP_Player_C|GetAnim%20Blueprint (Variables|Reference|GetCharacter)) "NewEnumerator0")
          (Variables|/Game/Blueprints/Character/InteractionSystem/BP_InteractionComponent.BP_InteractionComponent_C|SetInteractionEnable? (.BP_InteractionComponent (Variables|/Game/Blueprints/Character/BP_Player.BP_Player_C|GetBP_InteractionComponent (Variables|Reference|GetCharacter))) true)
          (Variables|Default|SetActivateKaypad? false)
          (Input|SetIgnoreMoveInput _returnvalue_2 false)
          (Input|SetIgnoreLookInput _returnvalue_2 false)
          (Input|DisableInput _returnvalue)
          (Input|EnableInput (Variables|Reference|GetCharacter) _returnvalue)
          (CallFunction|ResetInteraction))))))

(event Custom|ResetInteraction
  (bind _returnvalue (Game|GetPlayerController 0))
  (Utilities|FlowControl|DoOnce false) ; enters at Reset
)

(event Custom|NumPushAction
  (Utilities|FlowControl|Delay (select (== (Variables|IK|GetLastIndex) (Variables|IK|GetCurrentIndex)) 0.0 0.2))
  (CallFunction|PlayPushMontage))

(event EventBeginPlay
  (Variables|IK|SetIKPositions (Utilities|Array|MakeArray (Variables|Default|GetKey1) (Variables|Default|GetKey2) (Variables|Default|GetKey3) (Variables|Default|GetKey4) (Variables|Default|GetKey5) (Variables|Default|GetKey6) (Variables|Default|GetKey7) (Variables|Default|GetKey8) (Variables|Default|GetKey9) (Variables|Default|GetKey10) (Variables|Default|GetKey11) (Variables|Default|GetKey12)))
  (bind _asui_kaypad_screen (Utilities|Casting|CastToUI_KaypadScreen (UserInterface|GetWidget (Variables|Default|GetWidget))))
  (Variables|Reference|SetAs%20UI%20Kaypad%20Screen _asui_kaypad_screen))

(event Collision|EventActorBeginOverlap
  (params (OtherActor :type Actor%20Object%20Reference))
  ;[0.15 0.15 0.15 0.5] Register/Unregister Actor
  (bind _playercharacter (Class|BPIPlayer|GetPlayer(Message) OtherActor))
  (Utilities|IsValid _playercharacter
    (:Is%20Valid
      (Default|HandleRegister (.BP_InteractionComponent (Variables|/Game/Blueprints/Character/BP_Player.BP_Player_C|GetBP_InteractionComponent _playercharacter)) self))))

(event EventDefineActor
  (params (Result :type Boolean))
  ;[0.15 0.15 0.15 0.5] Visualization
  (Rendering|SetRenderCustomDepth (Variables|Default|GetBody) Result))

(event Collision|EventActorEndOverlap
  (params (OtherActor :type Actor%20Object%20Reference))
  ;[0.15 0.15 0.15 0.5] Register/Unregister Actor
  (bind _playercharacter (Class|BPIPlayer|GetPlayer(Message) OtherActor))
  (Utilities|IsValid _playercharacter
    (:Is%20Valid
      (Default|HandleUnregister (.BP_InteractionComponent (Variables|/Game/Blueprints/Character/BP_Player.BP_Player_C|GetBP_InteractionComponent _playercharacter)) self))))

(event EventTick
  (params (DeltaSeconds :type Float%20%28single-precision%29))
  (if (Variables|Default|GetActivateKaypad?)
    (Variables|/Game/Characters/Animations/ABP_Character.ABP_Character_C|SetInteraction%20Hand%20IK%20Position (Variables|/Game/Blueprints/Character/BP_Player.BP_Player_C|GetAnim%20Blueprint (Variables|Reference|GetCharacter)) (Math|Interpolation|VInterpTo (Variables|/Game/Characters/Animations/ABP_Character.ABP_Character_C|GetInteraction%20Hand%20IK%20Position (Variables|/Game/Blueprints/Character/BP_Player.BP_Player_C|GetAnim%20Blueprint (Variables|Reference|GetCharacter))) (Transformation|GetSocketLocation (Utilities|Array|Get(acopy) (Variables|IK|GetIKPositions) (Variables|IK|GetCurrentIndex)) "Position") (Utilities|Time|GetWorldDeltaSeconds) 1e+01))
    (Development|PrintString (Utilities|String|Append "" (Utilities|String|ToString(Integer) (Variables|IK|GetCurrentRow)) " / " "" (Utilities|String|ToString(Integer) (Variables|IK|GetCurrentColumn))) true true "(R=1.000000,G=0.000000,B=0.052408,A=1.000000)" 0.0)))

(event EventInteraction
  (params (Player :type BP%20Player%20Object%20Reference))
  (bind _returnvalue (Game|GetPlayerController 0))
  ;[0.15 0.15 0.15 0.5] Interaction
  (Variables|Reference|SetCharacter Player)
  (Utilities|FlowControl|DoOnce false
    (:Completed
      (bind _output_get (Variables|IK|SetLastIndex 0))
      (bind _output_get_2 (Variables|IK|SetCurrentIndex _output_get))
      (bind _output_get_3 (Variables|IK|SetCurrentRow _output_get_2))
      (Variables|IK|SetCurrentColumn _output_get_3)
      (Variables|/Game/Characters/Animations/ABP_Character.ABP_Character_C|SetInteraction%20Hand%20IK%20Position (Variables|/Game/Blueprints/Character/BP_Player.BP_Player_C|GetAnim%20Blueprint (Variables|Reference|GetCharacter)) (Transformation|GetSocketLocation (Variables|Default|GetKey1) "Position"))
      (Input|SetIgnoreMoveInput _returnvalue true)
      (Input|SetIgnoreLookInput _returnvalue true)
      (bind _notifyname (Animation|Montage|PlayMontage (Variables|/Script/Engine.Character|GetMesh (Variables|Reference|GetCharacter)) "/Game/Characters/Animations/Interaction/Keypad/A_Keypad_Enter_Montage.A_Keypad_Enter_Montage")
        (:OnNotifyBegin
          (switch name _notifyname
            (:Enter
              (CallFunction|UpdatePlayerPosition)
              (Variables|/Game/Characters/Animations/ABP_Character.ABP_Character_C|SetGlobalState (Variables|/Game/Blueprints/Character/BP_Player.BP_Player_C|GetAnim%20Blueprint (Variables|Reference|GetCharacter)) "NewEnumerator2")
              (Variables|/Game/Blueprints/Character/InteractionSystem/BP_InteractionComponent.BP_InteractionComponent_C|SetInteractionEnable? (.BP_InteractionComponent (Variables|/Game/Blueprints/Character/BP_Player.BP_Player_C|GetBP_InteractionComponent (Variables|Reference|GetCharacter))) false)
              (Rendering|SetRenderCustomDepth (Variables|Default|GetBody) false))))))))

(event Input|KeyboardEvents|Enter
  (params (Key :type Key%20Structure))
  (:Pressed
    (CallFunction|NumAction 11 3 2)))

(event Input|KeyboardEvents|NumPadSeven
  (params (Key :type Key%20Structure))
  (:Pressed
    (CallFunction|NumAction 6 2)))

(event Input|KeyboardEvents|NumPadOne
  (params (Key :type Key%20Structure))
  (:Pressed
    (CallFunction|NumAction)))

(event Input|KeyboardEvents|NumPadTwo
  (params (Key :type Key%20Structure))
  (:Pressed
    (CallFunction|NumAction 1 0 1)))

(event Input|KeyboardEvents|NumPadThree
  (params (Key :type Key%20Structure))
  (:Pressed
    (CallFunction|NumAction 2 0 2)))

(event Input|KeyboardEvents|NumPadFour
  (params (Key :type Key%20Structure))
  (:Pressed
    (CallFunction|NumAction 3 1)))

(event Input|KeyboardEvents|NumPadEight
  (params (Key :type Key%20Structure))
  (:Pressed
    (CallFunction|NumAction 7 2 1)))

(event Input|KeyboardEvents|NumPadNine
  (params (Key :type Key%20Structure))
  (:Pressed
    (CallFunction|NumAction 8 2 2)))

(event Input|KeyboardEvents|NumPadZero
  (params (Key :type Key%20Structure))
  (:Pressed
    (CallFunction|NumAction 10 3 1)))

(event Input|KeyboardEvents|Decimal
  (params (Key :type Key%20Structure))
  (:Pressed
    (CallFunction|NumAction 9 3)))

(event Input|KeyboardEvents|NumPadFive
  (params (Key :type Key%20Structure))
  (:Pressed
    (CallFunction|NumAction 4 1 1)))

(event Input|KeyboardEvents|NumPadSix
  (params (Key :type Key%20Structure))
  (:Pressed
    (CallFunction|NumAction 5 1 2)))

(event Input|MouseEvents|LeftMouseButton
  (params (Key :type Key%20Structure))
  (:Pressed
    (Utilities|FlowControl|DoOnce false
      (:Completed
        (CallFunction|PlayPushMontage)
        (Input|DisableInput (Game|GetPlayerController 0))))))

(event Input|KeyboardEvents|E
  (params (Key :type Key%20Structure))
  (:Pressed
    (CallFunction|ExitKeypad)))

(event Input|KeyboardEvents|W
  (params (Key :type Key%20Structure))
  (:Pressed
    (CallFunction|UpdateRow false)
    (CallFunction|UpdateCurrentIndex)))

(event Input|KeyboardEvents|S
  (params (Key :type Key%20Structure))
  (:Pressed
    (CallFunction|UpdateRow true)
    (CallFunction|UpdateCurrentIndex)))

(event Input|KeyboardEvents|A
  (params (Key :type Key%20Structure))
  (:Pressed
    (CallFunction|UpdateColumn false)
    (CallFunction|UpdateCurrentIndex)))

(event Input|KeyboardEvents|D
  (params (Key :type Key%20Structure))
  (:Pressed
    (CallFunction|UpdateColumn true)
    (CallFunction|UpdateCurrentIndex)))

(fn ConstructionScript)

(fn UpdateColumn
  (params (Add :type Boolean))
  (Variables|IK|SetCurrentColumn (Math|Integer|Clamp(Integer) (select Add (+ (Variables|IK|GetCurrentColumn) 1) (- (Variables|IK|GetCurrentColumn) 1)) 0 (Variables|IK|GetNumRows))))

(fn UpdateRow
  (params (Add :type Boolean))
  (Variables|IK|SetCurrentRow (Math|Integer|Clamp(Integer) (select Add (+ (Variables|IK|GetCurrentRow) 1) (- (Variables|IK|GetCurrentRow) 1)) 0 (Variables|IK|GetNumColumns))))

(fn UpdateCurrentIndex
  (Variables|IK|SetLastIndex (Variables|IK|GetCurrentIndex))
  (Variables|IK|SetCurrentIndex (+ (* (Variables|IK|GetCurrentRow) (Variables|IK|GetNumColumns)) (Variables|IK|GetCurrentColumn))))

(fn NumAction
  (params (Index :type Integer) (CurrentRow :type Integer) (CurrentColumn :type Integer))
  (Variables|IK|SetLastIndex Index)
  (Variables|IK|SetCurrentRow CurrentRow)
  (Variables|IK|SetCurrentColumn CurrentColumn)
  (Variables|Default|SetActiveElement (Utilities|Array|Get(acopy) (Variables|IK|GetIKPositions) Index))
  (CallFunction|NumPushAction)
  (Variables|IK|SetCurrentIndex (Variables|IK|GetLastIndex))
  (Input|DisableInput (Game|GetPlayerController 0)))

(fn TargetCenterOfMass
  (return (Variables|Default|GetBody)))