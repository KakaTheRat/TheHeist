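; BP_Light is a switchable lamp actor in the interaction system's Switcher folder, with optional flicker.
; An Activation event sets the on/off state and calls UpdateLight, which the construction script also runs.
; UpdateLight toggles point and spot light visibility and applies a flicker light function material when enabled.
; It also creates a dynamic lamp material instance whose glow and flicker parameters match that state.
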(event EventBeginPlay)

(event Collision|EventActorBeginOverlap
  (params (OtherActor :type Actor%20Object%20Reference)))

(event EventTick
  (params (DeltaSeconds :type Float%20%28single-precision%29)))

(event EventActivation
  (params (Activation :type Boolean))
  (Variables|Light|SetOff\On Activation)
  (CallFunction|UpdateLight))

(fn ConstructionScript
  (CallFunction|UpdateLight))

(fn UpdateLight
  (bind _off_on (Variables|Light|GetOff\On))
  (Rendering|Components|Light|SetLightFunctionMaterial (Variables|Default|GetPointLight) (select (Variables|Light|GetIsFlickers) "/Game/Meshes/Interaction/Light/Materials/M_LightFlikers.M_LightFlikers" 0))
  (Rendering|SetVisibility (Variables|Default|GetPointLight) _off_on false)
  (bind _returnvalue (Rendering|Material|CreateDynamicMaterialInstance (Variables|Default|GetLamp) 0 "/Game/Meshes/Interaction/Light/M_Lamp.M_Lamp" "None" :!class /Script/Engine.PrimitiveComponent))
  (Rendering|Material|SetScalarParameterValue _returnvalue "Glow" (select _off_on 5.0 0.0) :!class /Script/Engine.MaterialInstanceDynamic)
  (Rendering|Material|SetScalarParameterValue _returnvalue "Flikers" (select (Variables|Light|GetIsFlickers) 1.0 0.0) :!class /Script/Engine.MaterialInstanceDynamic))