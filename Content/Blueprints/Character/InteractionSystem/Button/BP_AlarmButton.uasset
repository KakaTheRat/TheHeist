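; Interactable alarm button that the player pushes to toggle a list of linked activation actors on and off.
; Overlap registers it with the player's interaction component, and custom depth highlights it.
; Interaction, gated by a DoOnce until the montage completes, locks input while a timeline aligns character and camera to an arrow.
; A montage notify flips the state, animates the button, plays a sound and messages each linked actor.
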(event Custom|UpdatePlayerPosition
  (bind _returnvalue (Game|GetPlayerController 0))
  (bind _returnvalue_2 (Game|GetPlayerController 0))
  (bind _returnvalue_3 (Game|GetPlayerController 0))
  (bind _arrow (Variables|Default|GetArrow))
  (bind _returnvalue_4 (Pawn|GetControlRotation _returnvalue :!class /Script/Engine.Controller))
  (bind (_roll _pitch) (Math|Rotator|BreakRotator _returnvalue_4))
  (Input|SetIgnoreMoveInput _returnvalue_3 true)
  (Input|SetIgnoreLookInput _returnvalue_3 true)
  (CallFunction|PlayMontageSwitcher)
  (bind _alpha (Timeline|SetPosition PlayFromStart)
    (:Update
      (Pawn|SetControlRotation (Game|GetPlayerController 0) (Math|Rotator|Lerp(Rotator) _returnvalue_4 (Math|Rotator|MakeRotator _roll _pitch (.yaw (Transformation|GetWorldRotation (Variables|Default|GetArrow)))) _alpha true))
      (Transformation|SetActorLocationAndRotation (Variables|Default|GetCharacter) (Math|Vector|Lerp(Vector) (Transformation|GetActorLocation (Variables|Default|GetCharacter)) (Transformation|GetWorldLocation _arrow) _alpha) (Math|Rotator|Lerp(Rotator) (Transformation|GetActorRotation (Variables|Default|GetCharacter)) (Transformation|GetWorldRotation _arrow) _alpha true)))
    (:Finished
      (Input|SetIgnoreMoveInput _returnvalue_2 false)
      (Input|SetIgnoreLookInput _returnvalue_2 false))))

(event Custom|PlayMontageSwitcher
  (Variables|/Game/Characters/Animations/ABP_Character.ABP_Character_C|SetbEnableRootYawOffset (Variables|/Game/Blueprints/Character/BP_Player.BP_Player_C|GetAnim%20Blueprint (Variables|Default|GetCharacter)) false)
  (bind _notifyname (Animation|Montage|PlayMontage (Variables|/Script/Engine.Character|GetMesh (Variables|Default|GetCharacter)) "/Game/Characters/Animations/Interaction/Button/A_ButtonPush_Montage.A_ButtonPush_Montage")
    (:OnCompleted
      (CallFunction|ResetInteraction)
      (Variables|/Game/Characters/Animations/ABP_Character.ABP_Character_C|SetbEnableRootYawOffset (Variables|/Game/Blueprints/Character/BP_Player.BP_Player_C|GetAnim%20Blueprint (Variables|Default|GetCharacter)) true))
    (:OnNotifyBegin
      (switch name _notifyname
        (:Tuch
          (bind _output_get (Variables|Light|SetOff/On (not (Variables|Light|GetOff/On))))
          (CallFunction|ActivateAnimation _output_get)
          (Audio|PlaySoundatLocation "/Engine/VREditor/Sounds/UI/Dockable_Window_Drop.Dockable_Window_Drop" (Transformation|GetWorldLocation (Variables|Default|GetRoot)) "0, 0, 0" 1.0 1.0 0.0 "/Game/Audio/Attenuation/Small_Attenuation_200_1000.Small_Attenuation_200_1000" "/Game/Audio/Class/SoundConcurrency_Base.SoundConcurrency_Base" 0 0)
          (for _array_element (Variables|Light|GetActivationActors)
            (Utilities|IsValid _array_element
              (:Is%20Valid
                (Class|BPIActorActivation|Activation(Message) _array_element (Variables|Light|GetOff/On))))))))))

(event Custom|ActivateAnimation
  (params (Activate :type Boolean))
  ;[1 1 1] Static Mesh Animation Time Line
  (if Activate
    (bind _alph (Timeline|StaticAnimation PlayFromStart)
      (:Update
        (Transformation|SetRelativeLocation (Variables|Default|GetButton) (Math|Vector|Lerp(Vector) "0, 0, 0" "0.000000,0.800000,0.000000" _alph) false false)))
    (else
      (Timeline|StaticAnimation ReverseFromEnd))))

(event Custom|ResetInteraction
  (Utilities|FlowControl|DoOnce false) ; enters at Reset
)

(event EventBeginPlay)

(event Collision|EventActorBeginOverlap
  (params (OtherActor :type Actor%20Object%20Reference))
  ;[0.15 0.15 0.15 0.5] Register/Unregister Actor
  (bind _playercharacter (Class|BPIPlayer|GetPlayer(Message) OtherActor))
  (Utilities|IsValid _playercharacter
    (:Is%20Valid
      (Default|HandleRegister (.BP_InteractionComponent (Variables|/Game/Blueprints/Character/BP_Player.BP_Player_C|GetBP_InteractionComponent _playercharacter)) self))))

(event Collision|EventActorEndOverlap
  (params (OtherActor :type Actor%20Object%20Reference))
  ;[0.15 0.15 0.15 0.5] Register/Unregister Actor
  (bind _playercharacter (Class|BPIPlayer|GetPlayer(Message) OtherActor))
  (Utilities|IsValid _playercharacter
    (:Is%20Valid
      (Default|HandleUnregister (.BP_InteractionComponent (Variables|/Game/Blueprints/Character/BP_Player.BP_Player_C|GetBP_InteractionComponent _playercharacter)) self))))

(event EventDefineActor
  (params (Result :type Boolean))
  ;[0.15 0.15 0.15 0.5] Visualization
  (Rendering|SetRenderCustomDepth (Variables|Default|GetRoot) Result))

(event EventTick
  (params (DeltaSeconds :type Float%20%28single-precision%29)))

(event EventInteraction
  (params (Player :type BP%20Player%20Object%20Reference))
  ;[0.15 0.15 0.15 0.5] Interaction
  (Variables|Default|SetCharacter Player)
  (Utilities|FlowControl|DoOnce false
    (:Completed
      (CallFunction|UpdatePlayerPosition))))

(fn ConstructionScript)

(fn TargetCenterOfMass
  (return (Variables|Default|GetButton)))