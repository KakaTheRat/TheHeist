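; Large double gateway door from the modular dungeon pack that swings open automatically at BeginPlay.
; Open and Close play or reverse a timeline that lerps each leaf's yaw 45 degrees in opposite directions from its initial rotation.
; When the timeline finishes, two plank meshes are hidden if open or shown if closed.
; Initial rotations are captured in world space but applied as relative rotations.
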(event EventBeginPlay
  (Variables|Default|SetDoorRInitialPosition (Transformation|GetWorldRotation (Variables|Default|GetMOD_Gateway_Door_01_large_door_R)))
  (Variables|Default|SetDoorLInitialPosition_ (Transformation|GetWorldRotation (Variables|Default|GetMOD_Gateway_Door_01_large_door_L)))
  (CallFunction|Open))

(event Collision|EventActorBeginOverlap
  (params (OtherActor :type Actor%20Object%20Reference)))

(event EventTick
  (params (DeltaSeconds :type Float%20%28single-precision%29)))

(event EventClose
  (bind _doorrinitialposition (Variables|Default|GetDoorRInitialPosition))
  (bind _doorlinitialposition_ (Variables|Default|GetDoorLInitialPosition_))
  (bind (_roll _pitch _yaw) (Math|Rotator|BreakRotator _doorlinitialposition_))
  (Variables|Default|SetIsOpen false)
  (bind _newtrack_0 (Timeline|Timeline Reverse)
    (:Update
      (Transformation|SetRelativeRotation (Variables|Default|GetMOD_Gateway_Door_01_large_door_R) (Math|Rotator|Lerp(Rotator) (Variables|Default|GetDoorRInitialPosition) (Math|Rotator|MakeRotator (.roll _doorrinitialposition) (.pitch _doorrinitialposition) (+ (.yaw _doorrinitialposition) 45.0)) _newtrack_0 true) false false)
      (Transformation|SetRelativeRotation (Variables|Default|GetMOD_Gateway_Door_01_large_door_L) (Math|Rotator|Lerp(Rotator) _doorlinitialposition_ (Math|Rotator|MakeRotator _roll _pitch (+ _yaw -45.0)) _newtrack_0 true) false false))
    (:Finished
      (Rendering|SetVisibility (Variables|Default|GetMOD_Gateway_Door_01_large_plank_02) (not (Variables|Default|GetIsOpen)) false))))

(event EventOpen
  (bind _doorrinitialposition (Variables|Default|GetDoorRInitialPosition))
  (bind _doorlinitialposition_ (Variables|Default|GetDoorLInitialPosition_))
  (bind (_roll _pitch _yaw) (Math|Rotator|BreakRotator _doorlinitialposition_))
  (Variables|Default|SetIsOpen true)
  (bind _newtrack_0 (Timeline|Timeline Play)
    (:Update
      (Transformation|SetRelativeRotation (Variables|Default|GetMOD_Gateway_Door_01_large_door_R) (Math|Rotator|Lerp(Rotator) (Variables|Default|GetDoorRInitialPosition) (Math|Rotator|MakeRotator (.roll _doorrinitialposition) (.pitch _doorrinitialposition) (+ (.yaw _doorrinitialposition) 45.0)) _newtrack_0 true) false false)
      (Transformation|SetRelativeRotation (Variables|Default|GetMOD_Gateway_Door_01_large_door_L) (Math|Rotator|Lerp(Rotator) _doorlinitialposition_ (Math|Rotator|MakeRotator _roll _pitch (+ _yaw -45.0)) _newtrack_0 true) false false))
    (:Finished
      (Rendering|SetVisibility (Variables|Default|GetMOD_Gateway_Door_01_large_plank_02) (not (Variables|Default|GetIsOpen)) false))))

(fn ConstructionScript)