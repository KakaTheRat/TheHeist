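; Interactable dungeon brazier prop that the player can light once through a "Light Up" prompt.
; Interacting marks it activated, which disables further interaction, turns on the Niagara fire effect and spawns an attenuated fire sound at its location.
; It also sends a quest counter "Activated" event with its class and a count of one through the GameInstance's game manager message system.
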(event EventBeginPlay)

(event Collision|EventActorBeginOverlap
  (params (OtherActor :type Actor%20Object%20Reference)))

(event EventTick
  (params (DeltaSeconds :type Float%20%28single-precision%29)))

(event EventInteract
  (params (Instigator :type Actor%20Object%20Reference))
  (Variables|Default|SetActivated true)
  (Components|Activation|Activate (Variables|Default|GetPS_FX_fire_dungeon_01_Niagara) false)
  (bind _gamemanager (Class|IGameInstance|GetGameManager(Message) (Game|GetGameInstance)))
  (Default|NotifyEvent _gamemanager "(TagName=\"Quest.Event.Counter.Activated\")" self (Utilities|Struct|MakeST_EventPayload "(TagName=\"\")" (Utilities|GetClass self) 1))
  (Audio|SpawnSoundatLocation "/Game/Audio/SFX/Misc/Fire/sfx_Ambient_VeryCUFire_02.sfx_Ambient_VeryCUFire_02" (Transformation|GetActorLocation) "0, 0, 0" 1.0 1.0 0.0 "/Game/_ChargeGatherVFX/_GenericSource/SFX/GenericSoundAttenuation.GenericSoundAttenuation" 0 false))

(fn ConstructionScript)

(fn GetInteractionText
  (return "Light Up"))

(fn IsInteractable
  (return (not (Variables|Default|GetActivated))))