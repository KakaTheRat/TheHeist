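; BP_Stall is a toilet stall whose door swings open and closed when triggered while something is near it.
; A box collision's begin and end overlaps set a NearDoor flag without filtering the overlapping actor.
; Door_Open_Event checks that flag, then a FlipFlop alternately plays and reverses a timeline that drives the door's relative yaw.
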(event OnComponentBeginOverlap(BoxCollision)
  (params (OverlappedComponent :type Primitive%20Component%20Object%20Reference) (OtherActor :type Actor%20Object%20Reference) (OtherComp :type Primitive%20Component%20Object%20Reference) (OtherBodyIndex :type Integer) (bFromSweep :type Boolean) (SweepResult :type Hit%20Result%20Structure%20%28by%20ref%29))
  ;[1 1 1] Near Door Detection
  (Variables|Default|SetNearDoor true))

(event OnComponentEndOverlap(BoxCollision)
  (params (OverlappedComponent :type Primitive%20Component%20Object%20Reference) (OtherActor :type Actor%20Object%20Reference) (OtherComp :type Primitive%20Component%20Object%20Reference) (OtherBodyIndex :type Integer))
  ;[1 1 1] Near Door Detection
  (Variables|Default|SetNearDoor false))

(event Custom|Door_Open_Event
  (if (Variables|Default|GetNearDoor)
    (Utilities|FlowControl|FlipFlop
      (:A
        (bind _doorrotamount (Timeline|DoorRotAmount Play)
          (:Update
            (Transformation|SetRelativeRotation (Variables|Default|GetStall_Door) (Math|Rotator|MakeRotator 0.0 0.0 _doorrotamount) false false))))
      (:B
        (Timeline|DoorRotAmount Reverse)))))

(fn ConstructionScript)