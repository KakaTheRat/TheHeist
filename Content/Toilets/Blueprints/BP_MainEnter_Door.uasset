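; BP_MainEnter_Door is a swinging door actor, apparently the main entrance to the toilets, that opens and closes on demand.
; Overlap begin and end set a NearDoor flag for any actor, with no filtering.
; Door_Open_Event acts only while that flag is set, using a FlipFlop to alternate playing and reversing a timeline.
; The timeline's DoorRotAmount track drives the relative yaw of MainDoorDoor.
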(event Custom|Door_Open_Event
  (if (Variables|Default|GetNearDoor)
    (Utilities|FlowControl|FlipFlop
      (:A
        (bind _doorrotamount (Timeline|Timeline_0 Play)
          (:Update
            (Transformation|SetRelativeRotation (Variables|Default|GetMainDoor_Door) (Math|Rotator|MakeRotator 0.0 0.0 _doorrotamount) false false))))
      (:B
        (Timeline|Timeline_0 Reverse)))))

(event Collision|EventActorBeginOverlap
  (params (OtherActor :type Actor%20Object%20Reference))
  (Variables|Default|SetNearDoor true))

(event Collision|EventActorEndOverlap
  (params (OtherActor :type Actor%20Object%20Reference))
  (Variables|Default|SetNearDoor false))

(fn ConstructionScript)