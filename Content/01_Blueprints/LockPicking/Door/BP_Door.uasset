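; BP_Door is a lockpickable door that an actor with a BPC_LockPick component can interact with.
; Interacting registers the door as that component's picked object via BPI_LockPicking, disables the owner's movement and streams in LockPickingLevel to run the picking.
; On a successful pick it swings open after a short delay, then auto-closes, snapping rotation without animation.
; It also exposes its Difficulty through GetDifficulty.
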(event Custom|Close%20Door
  ;[1 0.7187 0.6486] Handles Closing Of Door After Opened
  (Transformation|SetRelativeRotation (Variables|Default|GetDoor) (Math|Rotator|MakeRotator 0.0 0.0 0.0) false true))

(event EventInteract
  (params (HitComponent :type Scene%20Component%20Object%20Reference) (InteractingActor :type Actor%20Object%20Reference) (Context :type EInteractionContext%20Enum :default "Default"))
  (bind _returnvalue (Actor|GetComponentbyClass InteractingActor "/Game/01_Blueprints/Components/Player/BPC_LockPick.BPC_LockPick_C"))
  (Utilities|IsValid _returnvalue
    (:Is%20Valid
      (bind _asbpi_lock_picking (Utilities|Casting|CastToBPI_LockPicking self)
        (:then
          (Variables|/Game/01_Blueprints/Components/Player/BPC_LockPick.BPC_LockPick_C|SetObjectBeingPicked _returnvalue _asbpi_lock_picking)
          ;[1 0.376 0.7236] Stops Player Moving When Interacting With Door
          (Pawn|Components|CharacterMovement|DisableMovement (Variables|/Script/Engine.Character|GetCharacterMovement (Variables|/Game/01_Blueprints/Components/Player/BPC_LockPick.BPC_LockPick_C|GetOwner _returnvalue)))
          ;[1 0.1667 0.00675] Streams In Level That Will Be Handling The Code For Lock Picking
          (Game|LoadStreamLevel(byName) "LockPickingLevel" true)
          (Development|PrintString "Ici"))
        (:CastFailed
          (Development|PrintString "Failed"))))
    (:Is%20Not%20Valid
      (Development|PrintString "Not Valid"))))

(event EventOnPicked
  ;[0.28 1 0.6233] Easy Debut To Notify Player Of Success
  (Development|PrintString "You Successfully Picked The Door Lock")
  (Utilities|FlowControl|Delay 1.5)
  ;[0.97 0.6319 1] Opens Door
  (Transformation|SetRelativeRotation (Variables|Default|GetDoor) (Math|Rotator|MakeRotator 0.0 0.0 9e+01) false true)
  ;[0.06198 1 0.9702] Auto Close Door After 6.5 Seconds
  (Utilities|FlowControl|Delay 6.5)
  (CallFunction|CloseDoor))

(fn ConstructionScript)

(fn GetDifficulty
  (return (Variables|Default|GetDifficulty)))