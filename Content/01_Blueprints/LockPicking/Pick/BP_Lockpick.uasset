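; Lockpicking minigame actor where the player angles a bobby pin, then turns the inner lock, rendered in isolation by a scene capture.
; The construction script randomizes a sweet spot sized by difficulty.
; Each tick, pick closeness to that range caps lock rotation; hitting the cap triggers a timeline shake, and releasing input springs the lock back.
; Reaching full rotation calls OnPicked and disables tick, which also locks pick input.
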(event Custom|BeginPickShake
  ;[0 0.4479 0.0327] Shaking Of Lock Pick When Trying To Open Lock But Not At Unlock Area
  ;;[0.3021 0.2533 0] If Pick Is Not Already Shaking, Proceed True
  (if (not (Variables|Private|GetPickShaking?))
    (Variables|Private|SetPickShaking? true)
    ;;[1 0.6067 0.2543] Shaking Of Pick By Changing Location Of Y Axis
    (bind _pickoffsetamount (Timeline|PickShake%20Timeline PlayFromStart)
      (:Update
        (Private|SetPickOffset _pickoffsetamount)))))

(event Custom|EndPickShake
  ;[0 0.4479 0.0327] Shaking Of Lock Pick When Trying To Open Lock But Not At Unlock Area
  (if (Variables|Private|GetPickShaking?)
    (Variables|Private|SetPickShaking? false)
    (Utilities|FlowControl|Sequence
      (:then_0
        ;;[1 0.6067 0.2543] Shaking Of Pick By Changing Location Of Y Axis
        (bind _pickoffsetamount (Timeline|PickShake%20Timeline Stop)
          (:Update
            (Private|SetPickOffset _pickoffsetamount))))
      (:then_1
        (Private|SetPickOffset 0.0)))))

(event EventTick
  (params (DeltaSeconds :type Float%20%28single-precision%29))
  ;[0.4386 0 0.4688] Handle Tick
  (Private|HandleTick DeltaSeconds))

(event Input|AxisEvents|InputAxisRotateLock
  (params (AxisValue :type Float%20%28single-precision%29))
  ;[0.1895 0.1055 0.3333] Input Axis Rotate Lock
  (bind _output_get (Variables|Private|SetRotateLockAxis AxisValue))
  (if (== _output_get 0.0)
    (CallFunction|EndPickShake)))

(event Input|AxisEvents|InputAxisRotatePick
  (params (AxisValue :type Float%20%28single-precision%29))
  ;[0.4062 0 0.08345] Input Axis Rotate Pick
  (Utilities|AllowPickRotation
    (:true
      (Private|RotatePick (* AxisValue -1.0)))))

(fn ConstructionScript
  ;[1 0.4432 0.6049] Used For Displaying The Lock Pick Mechanism
  (Rendering|SceneCapture|ShowOnlyActorComponents (Variables|Default|GetSceneCaptureComponent2D) self false)
  (LocalVariables|SetUnlockHalfRange (/ (Utilities|Select :Index (Variables|Constants|GetDifficulty) :NewEnumerator0 15.0 :NewEnumerator1 1e+01 :NewEnumerator2 5.0) 2.0))
  ;[0.6679 1 0.2163] Middle Of Unlock Angle (The Sweet Spot)
  (LocalVariables|SetUnlockAngle (Math|Random|RandomFloatinRange (* (- (Variables|Constants|GetAbsMaxPickAngle) (LocalVariables|GetUnlockHalfRange)) -1.0) (- (Variables|Constants|GetAbsMaxPickAngle) (LocalVariables|GetUnlockHalfRange))))
  ;[0.5938 1 1] Min Unlock Angle
  (Variables|Private|SetMinUnlockAngle (- (LocalVariables|GetUnlockAngle) (LocalVariables|GetUnlockHalfRange)))
  ;[1 0.7692 0.1892] Max Unlock Angle
  (Variables|Private|SetMaxUnlockAngle (+ (LocalVariables|GetUnlockAngle) (LocalVariables|GetUnlockHalfRange))))

(fn GetLockRotation
  ;[1 1 1] Gets Rotation Of Inner Lock
  (return (.roll (Variables|/Script/Engine.SceneComponent|GetRelativeRotation (Variables|Default|GetInnerLock)))))

(fn GetPickRotation
  ;[1 1 1] Get's X Axis Rotation Of Pick
  (return (.roll (Variables|/Script/Engine.SceneComponent|GetRelativeRotation (Variables|Default|GetBobbyPin)))))

(fn IsPickinUnlockRange
  ;[1 1 1] Is The Pick WIthin The Min And Max Unlock Angles?
  (return (Math|Float|InRange(Float) (Private|GetPickRotation) (Variables|Private|GetMinUnlockAngle) (Variables|Private|GetMaxUnlockAngle))))

(fn RotateLock
  (params (Rotation :type Float%20%28double-precision%29))
  (Utilities|FlowControl|Sequence
    (:then_0
      (if (> Rotation 0.0)
        (if (>= (+ Rotation (Private|GetLockRotation)) (Variables|Constants|GetMaxLockAngle))
          ;[1 0.9504 0.4624] Ensures Lock Doesn't Glitch Passed 90 Degrees
          (Private|SetLockRotation (Variables|Constants|GetMaxLockAngle))
          (Default|CallOnPicked)
          ;[0.5297 1 0.5153] Prevents Player Input Once Picked
          (Actor|Tick|SetActorTickEnabled false)
          (return)
          (elif (>= (+ Rotation (Private|GetLockRotation)) (Variables|Private|GetAllowedLockRotation))
            ;[0.04201 1 0.3096] Starts To Shack Pick After Allowed Rotation
            (Private|SetLockRotation (Variables|Private|GetAllowedLockRotation))
            (CallFunction|BeginPickShake)
            (return)))))
    (:then_1
      (Transformation|AddLocalRotation (Variables|Default|GetInnerLock) (Math|Rotator|MakeRotator Rotation 0.0 0.0) false true))))

(fn HandleTick
  (params (Delta%20Seconds :type Float%20%28double-precision%29))
  (Private|UpdateAllowedLockRotation)
  ;[1 0.5506 0.1137] Is Player Rotating Lock?
  (if (> (Variables|Private|GetRotateLockAxis) 0.0)
    ;[0.8874 1 0.6951] Rotate Lock based On Speed And Time
    (Private|RotateLock (* (Variables|Private|GetRotateLockAxis) (Variables|Constants|GetLockRotationSpeed) Delta%20Seconds))
    (else
      ;[1 0.3718 0.332] Player Is No Longer Trying To Pick Lock
      (if (> (Private|GetLockRotation) 0.0)
        ;;[0.3476 1 0.4402] Starts Rotating Lock Back To Start
        (Private|RotateLock (* -1.0 (Variables|Constants|GetLockRotationSpeed) Delta%20Seconds))
        ;;[0.1241 0.3177 0.07171] Makes Sure Lock Doesn't Pass 0
        (if (< (Private|GetLockRotation) 0.0)
          (Private|SetLockRotation 0.0))))))

(fn SetLockRotation
  (params (Rotation :type Float%20%28double-precision%29))
  (Transformation|SetRelativeRotation (Variables|Default|GetInnerLock) (Math|Rotator|MakeRotator Rotation 0.0 0.0) false false))

(fn RotatePick
  (params (Rotation :type Float%20%28double-precision%29))
  ;[1 0.1314 0.4581] get current rotation and add to it
  (Transformation|SetRelativeRotation (Variables|Default|GetBobbyPin) (Math|Rotator|MakeRotator (Math|Float|Clamp(Float) (+ Rotation (Private|GetPickRotation)) (* (Variables|Constants|GetAbsMaxPickAngle) -1.0) (Variables|Constants|GetAbsMaxPickAngle)) 0.0 0.0) false true))

(fn UpdateAllowedLockRotation
  (bind _rotation (Private|GetPickRotation))
  (bind _minunlockangle (Variables|Private|GetMinUnlockAngle))
  (bind _returnvalue (- _minunlockangle _rotation))
  (Utilities|FlowControl|Sequence
    (:then_0
      ;[1 1 1] Is Pick In Unlock Range?
      (if (Private|IsPickinUnlockRange)
        (LocalVariables|SetPickCloseness 1.0)
        (else
          ;[1 0.383 0.5032] How Close Is Pick From 1?
          (bind _output_get (LocalVariables|SetPickAngleFromValid (select (> _returnvalue 0.0) _returnvalue (- (Private|GetPickRotation) (Variables|Private|GetMaxUnlockAngle)))))
          (LocalVariables|SetPickCloseness (- 1.0 (Math|Float|Clamp(Float) (/ _output_get (Variables|Constants|GetMaxLockMoveAngle))))))))
    (:then_1
      (Variables|Private|SetAllowedLockRotation (* (LocalVariables|GetPickCloseness) (Variables|Constants|GetMaxLockAngle))))))

(fn SetPickOffset
  (params (Offset :type Float%20%28double-precision%29))
  (bind _bobbypin (Variables|Default|GetBobbyPin))
  (bind _relativelocation (Variables|/Script/Engine.SceneComponent|GetRelativeLocation _bobbypin))
  (Transformation|SetRelativeLocation _bobbypin (Math|Vector|MakeVector (.x _relativelocation) (* Offset (Variables|Constants|GetPickShakeAmount)) (.z _relativelocation)) false true))