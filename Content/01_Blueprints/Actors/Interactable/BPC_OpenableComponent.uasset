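; Actor component that gives openable interactables an activation state and an on/off switch for interaction.
; On BeginPlay it sends InteractMessage to its owner if the current state differs from the default, then sets the state to that default.
; TryInteract forwards InteractMessage only when interaction is enabled and the owner implements BPI_Interactable.
; IsInNormalState reports whether the state still matches its default.
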(event Custom|OnBeginFocus)

(event Custom|OnEndFocus)

(event EventBeginPlay
  ;[0.15 0.15 0.15 0.5] Object state setter at start of the game
  (if (!= (Variables|Default|GetbIsActivatedByDefault) (Variables|Default|GetbIsActivated))
    (Class|BPIInteractable|Interact(Message) (Components|GetOwner self)))
  (Variables|Default|SetbIsActivated (Variables|Default|GetbIsActivatedByDefault)))

(event EventTick
  (params (DeltaSeconds :type Float%20%28single-precision%29)))

(fn TryInteract
  (bind _self self)
  (bind _returnvalue (Components|GetOwner _self))
  (if (Variables|Default|GetbIsInteractable)
    (if (Utilities|DoesObjectImplementInterface _returnvalue "/Game/01_Blueprints/Interfaces/BPI_Interactable.BPI_Interactable_C")
      (Class|BPIInteractable|Interact(Message) _returnvalue))))

(fn EnableInteraction
  (Variables|Default|SetbIsInteractable true))

(fn DisableInteraction
  (Variables|Default|SetbIsInteractable false))

(fn IsinNormalState
  (if (== (Variables|Default|GetbIsActivated) (Variables|Default|GetbIsActivatedByDefault))
    (return true)
    (else
      (return false))))