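; BP_InteractableObjects is an interactable actor that lets the player choose between several interactions on the component that was hit.
; Interact spawns a widget actor at that component's location and adds a button for each InteractableComponent whose interaction data matches the component's name.
; Component-to-data pairs are cached in a map.
; A click matches the button text against that map, runs the corresponding component's interaction and destroys the widget.
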(event Custom|Clicked_Event
  (params (Text :type Text))
  (CallFunction|InteractwithComponent Text))

(event EventInteract
  (params (HitComponent :type Scene%20Component%20Object%20Reference))
  ;[0.15 0.15 0.15 0.5] Widget creation to chose between several interactions
  (Variables|Default|SetHit%20Component HitComponent)
  (bind _widget (Variables|Default|GetWidget)
    (:then
      (Actor|DestroyActor _widget))
    (:else
      _))
  (bind _returnvalue (Game|SpawnActorfromClass "/Game/03_UI/W_est.W_est_C" (Math|Conversions|ToTransform(Vector) (Transformation|GetWorldLocation (Variables|Default|GetHit%20Component))) "Undefined" "MultiplyWithRoot" 0 0))
  (Variables|Default|SetWidget _returnvalue)
  (EventDispatchers|AssignClicked (Variables|/Game/03_UI/W_est.W_est_C|GetMyWidget _returnvalue) (delegate Custom|Clicked_Event))
  ;[0.15 0.15 0.15 0.5] Add a button on the widget for each interactable component attached to the hit component
  (for _array_element (Actor|GetComponentsByClass "/Script/TheHeist.InteractableComponent")
    (bind _returnvalue_2 (Class|InteractableComponent|GetInteractionbyComponentName _array_element (Utilities|GetObjectName (Variables|Default|GetHit%20Component))))
    (Utilities|IsValid _returnvalue_2
      (:Is%20Valid
        (if (Utilities|Enum|Equal(Enum) (Utilities|GetObjectName (Variables|Default|GetHit%20Component)) (Variables|/Script/TheHeist.InteractionData|GetAttachedComponentName _returnvalue_2))
          (Default|AddInteraction (Variables|/Game/03_UI/W_est.W_est_C|GetMyWidget _returnvalue) (Utilities|Text|ToText(String) (Variables|/Script/TheHeist.InteractionData|GetInteractText _returnvalue_2)))
          (Utilities|Map|Add (Variables|Default|GetInteractionComponentPerData) _array_element _returnvalue_2))))))

(fn ConstructionScript)

(fn InteractwithComponent
  (params (InteractionText :type Text))
  (bind (_keypin _valuepin) (Utilities|Map|ForEachLoop(Map) (Variables|Default|GetInteractionComponentPerData))
    (:then
      ;[0.15 0.15 0.15 0.5] Call interaction with the right interactable component, based of the name of the interaction text.
      (Utilities|IsValid _keypin
        (:Is%20Valid
          (Utilities|IsValid _valuepin
            (:Is%20Valid
              (if (Utilities|Enum|Equal(Enum) (Variables|/Script/TheHeist.InteractionData|GetInteractText _valuepin) (Utilities|String|ToString(Text) InteractionText))
                (Class|InteractableComponent|RunInteraction _keypin (Variables|Default|GetHit%20Component) _valuepin)
                (bind _widget (Variables|Default|GetWidget)
                  (:then
                    (Actor|DestroyActor _widget))
                  (:else))))))))))

(fn IsCurrentlyActive
  (return false))