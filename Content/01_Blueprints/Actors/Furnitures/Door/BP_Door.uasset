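; Interactive door actor that an overlapping character can open, close or find locked, using synchronized character and door animations.
; On interaction it picks the nearer front or back anchor, disables movement and collision, and lerps the character into place while clamping the local player's camera.
; Side and door state select the montage and door animation.
; Notifies play sounds, and montage completion toggles open/closed, restores control and re-arms the do-once gate.
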(event Custom|Interaction
  ;[0.15 0.15 0.15 0.5] Start interaction
  (Utilities|FlowControl|DoOnce false
    (:Completed
      (CallFunction|CheckEngagementPosition)
      (CallFunction|StartInteractionDoor))))

(event Custom|PlayInteractionMontage
  (bind _door (Variables|Default|GetDoor))
  (bind _character (Variables|Default|GetCharacter))
  (bind _character_2 (Variables|Default|GetCharacter))
  (bind _returnvalue (Transformation|GetWorldLocation _door))
  ;[0.15 0.15 0.15 0.5] Montage management
  (Variables|/Script/Engine.Pawn|SetbUseControllerRotationYaw _character false)
  (bind _returnvalue_2 (Class|EntitiesInterface|GetSkeletalMeshComponent(Message) _character))
  (bind _notifyname (Animation|Montage|PlayMontage _returnvalue_2 (CallFunction|FindCharacterMontage))
    (:then
      (Components|Animation|PlayAnimation (Variables|Default|GetDoor) (CallFunction|FindDoorAnimation) false))
    (:OnCompleted
      (Variables|Default|SetDoorState (Utilities|Select :Index (Variables|Default|GetDoorState) :NewEnumerator0 "NewEnumerator1" :NewEnumerator1 "NewEnumerator0" :NewEnumerator2 "NewEnumerator2"))
      (Input|ResetIgnoreMoveInput (Pawn|GetController (Variables|Default|GetCharacter)))
      (Collision|SetCollisionEnabled (Variables|/Script/Engine.Character|GetCapsuleComponent _character_2) "QueryAndPhysics")
      (Pawn|Components|CharacterMovement|SetMovementMode (Variables|/Script/Engine.Character|GetCharacterMovement _character_2) "MOVE_Walking" 0)
      (CallFunction|UnlockCamera)
      (Variables|/Script/Engine.Pawn|SetbUseControllerRotationYaw (Variables|Default|GetCharacter) true)
      (Class|InteractionData|EndOfInteraction (Variables|Default|GetInteractionData))
      (CallFunction|ResetInteraction))
    (:OnNotifyBegin
      (switch name _notifyname
        (:Locked
          (Audio|PlaySoundatLocation "/Game/06_Sounds/Door/S_DoorLock.S_DoorLock" _returnvalue "0, 0, 0" 1.0 1.0 0.0 0 0 0 0))
        (:Open
          (Audio|PlaySoundatLocation "/Game/06_Sounds/Door/S_DoorOpen.S_DoorOpen" _returnvalue "0, 0, 0" 1.0 1.0 0.0 0 0 0 0))
        (:Close
          (Audio|PlaySoundatLocation "/Game/06_Sounds/Door/S_DoorClose.S_DoorClose" _returnvalue "0, 0, 0" 1.0 1.0 0.0 0 0 0 0))))))

(event Custom|StartInteractionDoor
  (bind _character (Variables|Default|GetCharacter))
  (bind _character_2 (Variables|Default|GetCharacter))
  (bind _returnvalue (Pawn|GetController _character))
  (bind _returnvalue_2 (Pawn|GetControlRotation _returnvalue :!class /Script/Engine.Controller))
  (bind (_roll _pitch) (Math|Rotator|BreakRotator _returnvalue_2))
  ;[0.15 0.15 0.15 0.5] Start Interaction Door Position
  (Collision|SetCollisionEnabled (Variables|/Script/Engine.Character|GetCapsuleComponent _character_2) "NoCollision")
  (Pawn|Components|CharacterMovement|SetMovementMode (Variables|/Script/Engine.Character|GetCharacterMovement _character_2) "MOVE_Flying" 0)
  (Input|SetIgnoreMoveInput (Pawn|GetController (Variables|Default|GetCharacter)) true)
  (CallFunction|PlayInteractionMontage)
  (bind _alpha (Timeline|SetPlayerPositionTimeline PlayFromStart)
    (:Update
      (Pawn|SetControlRotation (Game|GetPlayerController 0) (Math|Rotator|Lerp(Rotator) _returnvalue_2 (Math|Rotator|MakeRotator _roll _pitch (.yaw (Transformation|GetWorldRotation (Utilities|Select :Index (Variables|Default|GetPosition) :NewEnumerator0 (Variables|Default|GetFrontPosition) :NewEnumerator1 (Variables|Default|GetBackPosition))))) _alpha true))
      (Transformation|SetActorLocationAndRotation (Variables|Default|GetCharacter) (Math|Vector|Lerp(Vector) (Transformation|GetActorLocation (Variables|Default|GetCharacter)) (Transformation|GetWorldLocation (Utilities|Select :Index (Variables|Default|GetPosition) :NewEnumerator0 (Variables|Default|GetFrontPosition) :NewEnumerator1 (Variables|Default|GetBackPosition))) _alpha) (Math|Rotator|Lerp(Rotator) (Transformation|GetActorRotation (Variables|Default|GetCharacter)) (Transformation|GetWorldRotation (Utilities|Select :Index (Variables|Default|GetPosition) :NewEnumerator0 (Variables|Default|GetFrontPosition) :NewEnumerator1 (Variables|Default|GetBackPosition))) _alpha true)))
    (:Finished
      (CallFunction|DoorCameraLock))))

(event Custom|ResetInteraction
  ;[0.15 0.15 0.15 0.5] Start interaction
  (Utilities|FlowControl|DoOnce false) ; enters at Reset
)

(event Custom|UnlockCamera
  (bind _returnvalue (Game|GetPlayerController 0))
  (bind _playercameramanager (Variables|/Script/Engine.PlayerController|GetPlayerCameraManager _returnvalue))
  (Utilities|IsValid _returnvalue
    (:Is%20Valid
      (Variables|/Script/Engine.PlayerCameraManager|SetViewYawMin _playercameramanager 0.0)
      (Variables|/Script/Engine.PlayerCameraManager|SetViewYawMax _playercameramanager 359.998993)
      (Variables|/Script/Engine.PlayerCameraManager|SetViewPitchMin _playercameramanager -75.0)
      (Variables|/Script/Engine.PlayerCameraManager|SetViewPitchMax _playercameramanager 75.0))))

(event Custom|DoorCamera%20Lock
  (bind _returnvalue (Game|GetPlayerController 0))
  (bind _character (Variables|Default|GetCharacter))
  (bind _position (Variables|Default|GetPosition))
  (bind _frontposition (Variables|Default|GetFrontPosition))
  (bind _backposition (Variables|Default|GetBackPosition))
  (bind _returnvalue_2 (Pawn|GetController _character))
  (bind _returnvalue_3 (Utilities|Select :Index _position :NewEnumerator0 _frontposition :NewEnumerator1 _backposition))
  (bind _playercameramanager (Variables|/Script/Engine.PlayerController|GetPlayerCameraManager _returnvalue))
  (bind _returnvalue_4 (Transformation|GetWorldRotation _returnvalue_3))
  ;[0.15 0.15 0.15 0.5] Door Lock Camera
  (if (== _returnvalue_2 _returnvalue)
    (Utilities|IsValid _returnvalue_2
      (:Is%20Valid
        (Variables|/Script/Engine.PlayerCameraManager|SetViewYawMin _playercameramanager (- (.yaw _returnvalue_4) 1.2e+02))
        (Variables|/Script/Engine.PlayerCameraManager|SetViewYawMax _playercameramanager (+ (.yaw _returnvalue_4) 75.0))
        (Variables|/Script/Engine.PlayerCameraManager|SetViewPitchMin _playercameramanager (- (.pitch _returnvalue_4) 75.0))
        (Variables|/Script/Engine.PlayerCameraManager|SetViewPitchMax _playercameramanager (+ (.pitch _returnvalue_4) 75.0))))))

(event Collision|EventActorBeginOverlap
  (params (OtherActor :type Actor%20Object%20Reference))
  ;[0.15 0.15 0.15 0.5] Overlap setup
  (bind _ascharacter (Utilities|Casting|CastToCharacter OtherActor))
  (Utilities|IsValid _ascharacter
    (:Is%20Valid
      (Variables|Default|SetCharacter _ascharacter))))

(event Collision|EventActorEndOverlap
  (params (OtherActor :type Actor%20Object%20Reference))
  ;[0.15 0.15 0.15 0.5] Overlap setup
  (if (== OtherActor (Variables|Default|GetCharacter))
    (Variables|Default|SetCharacter 0)))

(event EventInteract
  (params (HitComponent :type Scene%20Component%20Object%20Reference) (InteractingActor :type Actor%20Object%20Reference) (Context :type EInteractionContext%20Enum :default "Default") (Data :type Interaction%20Data%20Object%20Reference))
  ;[0.15 0.15 0.15 0.5] Start interaction
  (Utilities|IsValid (Variables|Default|GetCharacter)
    (:Is%20Valid
      (Variables|Default|SetInteractionData Data)
      (Utilities|FlowControl|DoOnce false
        (:Completed
          (CallFunction|CheckEngagementPosition)
          (CallFunction|StartInteractionDoor))))))

(fn ConstructionScript)

(fn CheckEngagementPosition
  (if (<= (Math|Vector|VectorLength (- (Transformation|GetActorLocation (Variables|Default|GetCharacter)) (Transformation|GetWorldLocation (Variables|Default|GetFrontPosition)))) (Math|Vector|VectorLength (- (Transformation|GetActorLocation (Variables|Default|GetCharacter)) (Transformation|GetWorldLocation (Variables|Default|GetBackPosition)))))
    (Variables|Default|SetPosition "NewEnumerator0")
    (else
      (Variables|Default|SetPosition "NewEnumerator1"))))

(fn FindCharacterMontage
  (return (Utilities|Select :Index (Variables|Default|GetPosition) :NewEnumerator0 (Utilities|Select :Index (Variables|Default|GetDoorState) :NewEnumerator0 "/Game/11_Animations/Door/AnimatedDoor/A_Idle_Door_Front_OpenFull_MontageReal.A_Idle_Door_Front_OpenFull_MontageReal" :NewEnumerator1 "/Game/11_Animations/Door/AnimatedDoor/A_Idle_Door_Front_CloseFull_MontageReal.A_Idle_Door_Front_CloseFull_MontageReal" :NewEnumerator2 "/Game/11_Animations/CardReader/A_Cardrider_Activate_Montage.A_Cardrider_Activate_Montage") :NewEnumerator1 (Utilities|Select :Index (Variables|Default|GetDoorState) :NewEnumerator0 "/Game/11_Animations/Door/AnimatedDoor/A_Idle_Door_Back_OpenFull_MontageReal.A_Idle_Door_Back_OpenFull_MontageReal" :NewEnumerator1 "/Game/11_Animations/Door/AnimatedDoor/A_Idle_Door_Back_CloseFull_MontageReal.A_Idle_Door_Back_CloseFull_MontageReal" :NewEnumerator2 "/Game/Characters/Animations/Interaction/Door/A_Idle_Door_Back_LockedFull_Montage.A_Idle_Door_Back_LockedFull_Montage"))))

(fn FindDoorAnimation
  (return (Utilities|Select :Index (Variables|Default|GetPosition) :NewEnumerator0 (Utilities|Select :Index (Variables|Default|GetDoorState) :NewEnumerator0 "/Game/Meshes/Interaction/Door/Animation/A_Door_Open_F_Full.A_Door_Open_F_Full" :NewEnumerator1 "/Game/Meshes/Interaction/Door/Animation/A_Door_Open_F_CloseFull.A_Door_Open_F_CloseFull" :NewEnumerator2 "/Game/Meshes/Interaction/Door/Animation/A_Door_Locked.A_Door_Locked") :NewEnumerator1 (Utilities|Select :Index (Variables|Default|GetDoorState) :NewEnumerator0 "/Game/Meshes/Interaction/Door/Animation/A_Door_Open_B_Full.A_Door_Open_B_Full" :NewEnumerator1 "/Game/Meshes/Interaction/Door/Animation/A_Door_Close_B_Full.A_Door_Close_B_Full" :NewEnumerator2 "/Game/Meshes/Interaction/Door/Animation/A_Door_Close_B_Locked.A_Door_Close_B_Locked"))))