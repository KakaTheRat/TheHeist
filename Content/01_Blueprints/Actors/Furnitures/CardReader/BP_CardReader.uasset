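; BP_CardReader is an interactable card reader that a character activates with a card-swipe montage.
; Interact runs once until reset, locking input and movement while the card attaches to the character's hand.
; A montage notify activates the reader, updating its screen widget, light color and sounds, then ends the interaction after a delay.
; Montage blend-out returns and hides the card, completion restores control, and DefineActor toggles custom-depth highlighting.
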(event Custom|PlayMontageCardrider
  (bind _card (Variables|Default|GetCard))
  (bind _card_2 (Variables|Default|GetCard))
  (Pawn|Components|CharacterMovement|SetMovementMode (Variables|/Script/Engine.Character|GetCharacterMovement (Variables|Default|GetInteracting%20Actor)) "MOVE_Flying" 0)
  (bind _notifyname (Animation|Montage|PlayMontage (Variables|/Script/Engine.Character|GetMesh (Variables|Default|GetInteracting%20Actor)) "/Game/11_Animations/CardReader/A_Cardrider_Activate_Montage.A_Cardrider_Activate_Montage")
    (:then
      ;[0.15 0.15 0.15 0.5] Card management
      (Transformation|AttachComponentToComponent _card_2 (Variables|/Script/Engine.Character|GetMesh (Variables|Default|GetInteracting%20Actor)) "weapon_right" "SnapToTarget" "SnapToTarget" "SnapToTarget" true)
      (Rendering|SetVisibility _card_2 true false))
    (:OnCompleted
      (CallFunction|ResetInteraction)
      (Input|EnableInput (Variables|Default|GetInteracting%20Actor) (Game|GetPlayerController 0))
      (Pawn|Components|CharacterMovement|SetMovementMode (Variables|/Script/Engine.Character|GetCharacterMovement (Variables|Default|GetInteracting%20Actor)) "MOVE_Walking" 0))
    (:OnBlendOut
      ;[0.15 0.15 0.15 0.5] Card management
      (Transformation|AttachComponentToComponent _card (Variables|Default|GetRoot) "Card" "SnapToTarget" "SnapToTarget" "SnapToTarget" true)
      (Rendering|SetVisibility _card false false))
    (:OnNotifyBegin
      (switch name _notifyname
        (:OnInteract
          (CallFunction|OnCardReaderActivated))))))

(event Custom|OnCardReaderActivated
  ;[0.15 0.15 0.15 0.5] Card received
  (Variables|Light|SetActivate true)
  (Audio|PlaySoundatLocation "/Engine/VREditor/Sounds/UI/Gizmo_Handle_Clicked.Gizmo_Handle_Clicked" (Transformation|GetWorldLocation (Variables|Default|GetRoot)) "0, 0, 0" 1.0 1.0 0.0 0 0 0 0)
  (Default|UpdateVisualCode (Variables|Default|GetAs%20UI%20Cardrider%20Screen) true)
  (Rendering|Components|Light|SetLightColor (Variables|Default|GetPointLight) "(R=0.003677,G=0.030713,B=0.000000,A=1.000000)" true)
  (Audio|PlaySoundatLocation "/Engine/VREditor/Sounds/UI/Invalid_Action.Invalid_Action" (Transformation|GetWorldLocation (Variables|Default|GetRoot)) "0, 0, 0" 1.0 1.0 0.0 0 0 0 0)
  (Utilities|FlowControl|Delay 1.0)
  (Class|InteractionData|EndOfInteraction (Variables|Default|GetData)))

(event Custom|ResetInteraction
  ;[0.15 0.15 0.15 0.5] Interaction setup
  (Utilities|FlowControl|DoOnce false) ; enters at Reset
)

(event EventBeginPlay
  (bind _asui_card_reader_screen (Utilities|Casting|CastToUI_CardReaderScreen (UserInterface|GetWidget (Variables|Default|GetWidget))))
  (Variables|Default|SetAs%20UI%20Cardrider%20Screen _asui_card_reader_screen))

(event EventDefineActor
  (params (Result :type Boolean))
  ;[0.15 0.15 0.15 0.5] Visualization
  (Rendering|SetRenderCustomDepth (Variables|Default|GetRoot) Result))

(event EventInteract
  (params (HitComponent :type Scene%20Component%20Object%20Reference) (InteractingActor :type Actor%20Object%20Reference) (Context :type EInteractionContext%20Enum :default "Default") (Data :type Interaction%20Data%20Object%20Reference))
  ;[0.15 0.15 0.15 0.5] Interaction setup
  (Variables|Default|SetData Data)
  (bind _ascharacter (Utilities|Casting|CastToCharacter InteractingActor))
  (Variables|Default|SetInteracting%20Actor _ascharacter)
  (Utilities|FlowControl|DoOnce false
    (:Completed
      (Input|DisableInput (Variables|Default|GetInteracting%20Actor) (Game|GetPlayerController 0))
      (CallFunction|PlayMontageCardrider))))

(event EventTick
  (params (DeltaSeconds :type Float%20%28single-precision%29)))

(fn ConstructionScript)