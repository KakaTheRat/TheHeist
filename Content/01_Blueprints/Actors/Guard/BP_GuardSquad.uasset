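; BP_GuardSquad is a squad manager that coordinates guard AI controllers, binding their events to share investigated actors, checked hideouts and area searches.
; Perception updates raise a shared alert score mapped to alert states, with one state making the perceiving guard a formation leader.
; Tick positions followers by rotated row offsets around the leader's patrol actor, with stop/resume requests controlling movement.
; It also sends nearest guards to locations and spawns backup.
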(event Custom|UpdateFormation
  (bind _spacing (Variables|Formation|GetSpacing))
  ;[0.15 0.15 0.15 0.5] Formation positions updated for each guard. Calculates the offset based on the leader. Current formation dictates how each guard will place around the leader
  (for _array_element (Variables|Formation|GetFormations)
    (Rendering|Material|SetMaterial (Variables|/Script/Engine.Character|GetMesh (.Leader (Utilities|Struct|BreakS_GuardsFormation _array_element))) 0 "/DatasmithContent/Materials/AliasReference.AliasReference")
    (bind _asaic_guard_aicontroller (Utilities|Casting|CastToAIC_GuardAIController (AI|GetAIController (.Leader (Utilities|Struct|BreakS_GuardsFormation _array_element)))))
    (Default|SetFormationPosition _asaic_guard_aicontroller "0, 0, 0" true true)
    (for _array_element_2 (.Followers (Utilities|Struct|BreakS_GuardsFormation _array_element))
      (bind _returnvalue (Class|FormationHelper|GetFormationOffset "/Game/16_Data/DataAssets/Guards/DA_RowFormationData.DA_RowFormationData" 1 _spacing _spacing))
      (bind _asaic_guard_aicontroller_2 (Utilities|Casting|CastToAIC_GuardAIController (AI|GetAIController _array_element_2)))
      (Default|SetFormationPosition _asaic_guard_aicontroller_2 (+ (Transformation|GetActorLocation (Variables|/Game/04_IA/Guard/AI_Controller/AIC_GuardAIController.AIC_GuardAIController_C|GetSmoothPatrolActor _asaic_guard_aicontroller)) (Math|Vector|RotateVector _returnvalue (Transformation|GetActorRotation (.Leader (Utilities|Struct|BreakS_GuardsFormation _array_element))))) true false))))

(event Custom|HideoutChecking
  (params (HideoutActor :type Actor%20Object%20Reference))
  ;[0.15 0.15 0.15 0.5] Initializes a new guard to enter the squad. This will mainly set all the events
  (Utilities|Array|AddUnique (Variables|Default|GetHiddenSpotsCovered) HideoutActor))

(event Custom|AddMemberToFormation
  (params (Formations :type S%20Guards%20Formation%20Structure%20%28by%20ref%29) (Guard :type BP%20Guard%20Object%20Reference) (Index :type Integer%20%28by%20ref%29))
  (bind _output (Utilities|Array|Get(acopy) (Variables|Formation|GetFormations) Index))
  (bind (_followers _leader) (Utilities|Struct|BreakS_GuardsFormation _output))
  ;[0.15 0.15 0.15 0.5] Formations
  ;;[0.15 0.15 0.15 0.5] Adds a new guard to an existing formation
  (bind _asaic_guard_aicontroller (Utilities|Casting|CastToAIC_GuardAIController (AI|GetAIController Guard)))
  (if (!= Guard _leader)
    (if (not (Variables|/Game/04_IA/Guard/AI_Controller/AIC_GuardAIController.AIC_GuardAIController_C|GetIsInFomation _asaic_guard_aicontroller))
      (Utilities|Array|AddUnique _followers Guard)
      (Variables|/Game/04_IA/Guard/AI_Controller/AIC_GuardAIController.AIC_GuardAIController_C|SetIsInFomation _asaic_guard_aicontroller true)
      (Variables|/Game/04_IA/Guard/AI_Controller/AIC_GuardAIController.AIC_GuardAIController_C|SetFormationIndex _asaic_guard_aicontroller Index)
      (Variables|/Game/04_IA/Guard/AI_Controller/AIC_GuardAIController.AIC_GuardAIController_C|SetFormation _asaic_guard_aicontroller Formations)
      (CallFunction|StopLeaderFormationMovement :GuardStopping Guard :FormationIndex Index))))

(event Custom|Stop
  (params (Formation :type S%20Guards%20Formation%20Structure) (GuardStopping :type BP%20Guard%20Object%20Reference))
  (bind (_followers _leader) (Utilities|Struct|BreakS_GuardsFormation Formation))
  ;[0.15 0.15 0.15 0.5] Stops the leader's movements. The one calling this event is still free to move
  (for _array_element _followers
    (if (not (== _array_element GuardStopping))
      (bind _asaic_guard_aicontroller (Utilities|Casting|CastToAIC_GuardAIController (AI|GetAIController _array_element)))
      (Default|SetGuardState _asaic_guard_aicontroller "NewEnumerator1")))
  (if (not (== _leader GuardStopping))
    (bind _asaic_guard_aicontroller_2 (Utilities|Casting|CastToAIC_GuardAIController (AI|GetAIController _leader)))
    (Default|SetGuardState _asaic_guard_aicontroller_2 "NewEnumerator1")))

(event Custom|ResumeFormationMovement
  (params (Formation :type S%20Guards%20Formation%20Structure%20%28by%20ref%29) (GuardStopping :type BP%20Guard%20Object%20Reference) (FormationIndex :type Integer))
  (bind _formations (Variables|Formation|GetFormations))
  (bind _output (Utilities|Array|Get(acopy) _formations FormationIndex))
  (bind (_followers _leader _followersaskingtostop) (Utilities|Struct|BreakS_GuardsFormation _output))
  ;[0.15 0.15 0.15 0.5] Formations
  ;;[0.15 0.15 0.15 0.5] Resumes the formation movement.
  (Utilities|Array|RemoveItem _followersaskingtostop GuardStopping)
  (if (Utilities|Array|IsEmpty _followersaskingtostop)
    (bind _asaic_guard_aicontroller (Utilities|Casting|CastToAIC_GuardAIController (AI|GetAIController _leader)))
    (Default|SetGuardState _asaic_guard_aicontroller "NewEnumerator0")
    (for _array_element _followers
      (bind _asaic_guard_aicontroller_2 (Utilities|Casting|CastToAIC_GuardAIController (AI|GetAIController _array_element)))
      (Default|SetGuardState _asaic_guard_aicontroller_2 "NewEnumerator0"))))

(event Custom|StopLeaderFormationMovement
  (params (Formation :type S%20Guards%20Formation%20Structure%20%28by%20ref%29) (GuardStopping :type BP%20Guard%20Object%20Reference) (FormationIndex :type Integer))
  (bind _formations (Variables|Formation|GetFormations))
  (bind _output (Utilities|Array|Get(acopy) _formations FormationIndex))
  (bind (_leader _followersaskingtostop) (Utilities|Struct|BreakS_GuardsFormation _output))
  ;[0.15 0.15 0.15 0.5] Formations
  ;;[0.15 0.15 0.15 0.5] Stops the leader's movements.
  (Utilities|Array|AddUnique _followersaskingtostop GuardStopping)
  (bind _asaic_guard_aicontroller (Utilities|Casting|CastToAIC_GuardAIController (AI|GetAIController _leader)))
  (Default|SetGuardState _asaic_guard_aicontroller "NewEnumerator1"))

(event Custom|CallGuardHere
  (params (ActorRef :type Actor%20Object%20Reference) (Location :type Vector) (AmountOfGuards :type Integer))
  (bind _returnvalue (Class|FormationHelper|GetClosestActors (Variables|Default|GetGuards) Location AmountOfGuards))
  (for _array_element _returnvalue
    (bind _asaic_guard_aicontroller (Utilities|Casting|CastToAIC_GuardAIController (AI|GetAIController _array_element)))
    (Default|Goto _asaic_guard_aicontroller ActorRef Location)))

(event Custom|CreateFormations
  (params (Leader :type BP%20Guard%20Object%20Reference))
  ;[0.15 0.15 0.15 0.5] Formations
  ;;[0.15 0.15 0.15 0.5] Creates a brand new formation.
  (bind _returnvalue (Utilities|Array|AddUnique (Variables|Formation|GetFormations) (Utilities|Struct|MakeS_GuardsFormation Leader)))
  (for _array_element (Variables|Default|GetGuards)
    (CallFunction|AddMembertoFormation :Guard _array_element :Index _returnvalue)
    (Variables|Default|SetShouldForme true)))

(event Custom|DisbandFormation
  (params (Formation :type S%20Guards%20Formation%20Structure%20%28by%20ref%29))
  ;[0.15 0.15 0.15 0.5] Formations
  ;;[0.15 0.15 0.15 0.5] Destroys a formation
  (for _array_element (Utilities|Struct|BreakS_GuardsFormation Formation)
    (Utilities|Casting|CastToAIC_GuardAIController (AI|GetAIController _array_element))))

(event Custom|CallBackup
  ;[0.15 0.15 0.15 0.5] Calls backup. Will instantiate a new guard in the linked spawner. (NB : need to change spawning by pooling later)
  (bind _returnvalue (Game|SpawnActorfromClass "/Game/01_Blueprints/Actors/Guard/BP_Guard.BP_Guard_C" (Math|Transform|MakeTransform (Transformation|GetWorldLocation (Variables|/Game/01_Blueprints/Actors/Guard/BP_GuardSpawnerDoor.BP_GuardSpawnerDoor_C|GetSpawnPoint (Variables|Default|GetGuardSpawner))) "0, 0, 0" "1.000000,1.000000,1.000000") "Undefined" "MultiplyWithRoot" 0 0))
  (CallFunction|InitializeGuard _returnvalue)
  (Utilities|Array|AddUnique (Variables|Default|GetGuards) _returnvalue)
  (Variables|Default|SetShouldForme true)
  (Default|CallSetAlertState "NewEnumerator2"))

(event Custom|InitializeGuard
  (params (NewGuard :type BP%20Guard%20Object%20Reference))
  ;[0.15 0.15 0.15 0.5] Initializes a new guard to enter the squad. This will mainly set all the events
  (bind _asaic_guard_aicontroller (Utilities|Casting|CastToAIC_GuardAIController (AI|GetAIController NewGuard)))
  (Utilities|Map|Add (Variables|Default|GetGuards/AIC) NewGuard _asaic_guard_aicontroller)
  (Default|Initialize _asaic_guard_aicontroller self (Utilities|Array|Get(acopy) (Variables|Default|GetPatrolPaths) (Math|Random|RandomIntegerinRange 0 0)))
  (EventDispatchers|BindEventtoPerceptionUpdated _asaic_guard_aicontroller (delegate Custom|PerceptionUpdate))
  (EventDispatchers|BindEventtoActorEndInvestigation _asaic_guard_aicontroller (delegate Custom|InvestigationEnded))
  (EventDispatchers|BindEventtoHideoutChecked _asaic_guard_aicontroller (delegate Custom|HideoutChecking))
  (EventDispatchers|BindEventtoAreatoCheck _asaic_guard_aicontroller (delegate Custom|AreaToCheck)))

(event Custom|PerceptionUpdate
  (params (ActorPerceived :type Actor%20Object%20Reference) (Guard :type BP%20Guard%20Object%20Reference))
  ;[0.15 0.15 0.15 0.5] Initializes a new guard to enter the squad. This will mainly set all the events
  (Utilities|Array|AddUnique (Variables|Percpetion|GetActorUnderInvestigation) ActorPerceived)
  (CallFunction|SetNewGuardAlertState 7e+01 Guard))

(event Custom|InvestigationEnded
  (params (ActorInvestigated :type Actor%20Object%20Reference))
  ;[0.15 0.15 0.15 0.5] Initializes a new guard to enter the squad. This will mainly set all the events
  (Utilities|Array|RemoveItem (Variables|Percpetion|GetActorUnderInvestigation) ActorInvestigated))

(event Custom|AreaToCheck
  (params (LocationsToCheck :type Array%20of%20Vectors))
  ;[0.15 0.15 0.15 0.5] Initializes a new guard to enter the squad. This will mainly set all the events
  (CallFunction|SearchAreas LocationsToCheck))

(event EventBeginPlay
  (for _array_element (Variables|Default|GetGuards)
    (CallFunction|InitializeGuard _array_element)))

(event EventTick
  (params (DeltaSeconds :type Float%20%28single-precision%29))
  (if (Variables|Default|GetShouldForme)
    (CallFunction|UpdateFormation)))

(fn ConstructionScript)

(fn IsBeingInvestigated
  (params (ActorToInvestigate :type Actor%20Object%20Reference))
  (return (Utilities|Array|ContainsItem (Variables|Percpetion|GetActorUnderInvestigation) ActorToInvestigate)))

(fn IsHideoutChecked
  (params (HideoutActor :type Actor%20Object%20Reference))
  (return (Utilities|Array|ContainsItem (Variables|Default|GetHiddenSpotsCovered) HideoutActor)))

(fn SearchAreas
  (params (LocationsToCheck :type Array%20of%20Vectors))
  (for (_array_element _array_index) (Variables|Default|GetGuards)
    (bind _asaic_guard_aicontroller (Utilities|Casting|CastToAIC_GuardAIController (AI|GetAIController _array_element)))
    (Default|Goto _asaic_guard_aicontroller _asaic_guard_aicontroller (Utilities|Array|Get(acopy) LocationsToCheck _array_index))))

(fn SetNewGuardAlertState
  (params (Add/Remove :type Float%20%28double-precision%29) (Guard :type BP%20Guard%20Object%20Reference%20%28by%20ref%29))
  (if (not (>= (Variables|Alert|GetAlertStateScore) (Variables|Alert|GetMaxAlertScore)))
    (Variables|Alert|SetAlertStateScore (Math|Float|Clamp(Float) (+ Add/Remove (Variables|Alert|GetAlertStateScore)) 0.0 (Variables|Alert|GetMaxAlertScore)))
    (bind (_array_element _array_index) (Utilities|Array|ForEachLoopwithBreak (Variables|Alert|GetAlertStepScore) :!label _label)
      (:LoopBody
        (if (>= _array_element (Variables|Alert|GetAlertStateScore))
          (bind _enumvalue (|ForEachE_GuardAlertState)
            (:LoopBody
              (if (== (Math|Conversions|ToInteger(Byte) _enumvalue) _array_index)
                (if (!= (Math|Conversions|ToInteger(Byte) _enumvalue) (Math|Conversions|ToInteger(Byte) (Variables|Alert|GetCurrentAlertState)))
                  (if (Utilities|Enum|Equal(Enum) _enumvalue "NewEnumerator2")
                    (Development|PrintString "Hello")
                    (CallFunction|CreateFormations Guard))
                  (Default|CallSetAlertState _enumvalue)
                  (goto _label Break)
                  (else
                    (goto _label Break)))))))))))