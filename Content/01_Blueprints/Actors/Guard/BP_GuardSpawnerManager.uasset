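; BP_GuardSpawnerManager is an actor that spawns a backup guard when a guard's AI controller reports max stress.
; On BeginPlay it caches all spawner doors and binds to each existing guard controller's OnMaxLevelStress event.
; It spawns at the door nearest the stored Guard, copies that guard's patrol path and opens the door.
; Guard holds the last guard iterated at BeginPlay, not necessarily the stressed one.
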(event Custom|SpawnBackupGuard
  (CallFunction|SpawnGuard))

(event EventBeginPlay
  (bind _outactors (Actor|GetAllActorsOfClass "/Game/01_Blueprints/Actors/Guard/BP_GuardSpawnerDoor.BP_GuardSpawnerDoor_C"))
  (Variables|Default|SetSpawnersList _outactors)
  (bind _outactors_2 (Actor|GetAllActorsOfClass "/Game/01_Blueprints/Actors/Guard/BP_Guard.BP_Guard_C"))
  (for _array_element _outactors_2
    (bind _output_get (Variables|Default|SetGuard _array_element))
    (bind _asaic_guard_aicontroller (Utilities|Casting|CastToAIC_GuardAIController (Pawn|GetController _output_get)))
    (EventDispatchers|BindEventtoOnMaxLevelStress _asaic_guard_aicontroller (delegate Custom|SpawnBackupGuard))))

(fn ConstructionScript)

(fn SpawnGuard
  (bind _guard (Variables|Default|GetGuard))
  (for (_array_element _array_index) (Variables|Default|GetSpawnersList)
    (if (== _array_index 0)
      (Variables|Default|SetClosestSpawner _array_element)
      (elif (< (Transformation|GetDistanceTo _guard _array_element) (Transformation|GetDistanceTo _guard (Variables|Default|GetClosestSpawner)))
        (Variables|Default|SetClosestSpawner _array_element))))
  (bind _returnvalue (Game|SpawnActorfromClass "/Game/01_Blueprints/Actors/Guard/BP_Guard.BP_Guard_C" (Math|Conversions|ToTransform(Vector) (Transformation|GetWorldLocation (Variables|/Game/01_Blueprints/Actors/Guard/BP_GuardSpawnerDoor.BP_GuardSpawnerDoor_C|GetSpawnPoint (Variables|Default|GetClosestSpawner)))) "Undefined" "MultiplyWithRoot" 0 0))
  (Variables|/Game/01_Blueprints/Actors/Guard/BP_Guard.BP_Guard_C|SetPatrolPath _returnvalue (Variables|/Game/01_Blueprints/Actors/Guard/BP_Guard.BP_Guard_C|GetPatrolPath (Variables|Default|GetGuard)))
  (Default|OpenDoor (Variables|Default|GetClosestSpawner)))