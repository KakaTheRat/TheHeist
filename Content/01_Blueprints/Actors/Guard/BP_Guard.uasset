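; BP_Guard is a guard character that kicks off its action component shortly after spawning and can be moved to a given position while facing a target.
; MoveandLookEntity switches movement to Flying, then runs a timeline that lerps horizontal location and, given a valid target, control rotation, restoring Walking when finished.
; CheckClosest, LookatTarget and GetAnimationBlueprint are empty stubs; GetSkeletalMeshComponent returns the mesh.
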(event EventBeginPlay
  (Utilities|FlowControl|Delay 2.0)
  (Default|OnAction (Variables|Default|GetBP_ActionComp)))

(event Collision|EventActorBeginOverlap
  (params (OtherActor :type Actor%20Object%20Reference)))

(event EventMoveandLookEntity
  (params (Position :type Scene%20Component%20Object%20Reference) (LookTarget :type Scene%20Component%20Object%20Reference))
  (bind _returnvalue (Transformation|GetActorLocation))
  (bind _charactermovement (Variables|Character|GetCharacterMovement))
  (Pawn|Components|CharacterMovement|SetMovementMode _charactermovement "MOVE_Flying" 0)
  (bind _newtrack_0 (Timeline|Timeline PlayFromStart)
    (:Update
      (Transformation|SetActorLocation (Math|Vector|MakeVector (.x (Math|Vector|Lerp(Vector) (Math|Vector|MakeVector (.x _returnvalue) (.y _returnvalue) (.z _returnvalue)) (Transformation|GetWorldLocation Position) _newtrack_0)) (.y (Math|Vector|Lerp(Vector) (Math|Vector|MakeVector (.x _returnvalue) (.y _returnvalue) (.z _returnvalue)) (Transformation|GetWorldLocation Position) _newtrack_0)) (.z _returnvalue)) false false)
      (Utilities|IsValid LookTarget
        (:Is%20Valid
          (Pawn|SetControlRotation (Pawn|GetController) (Math|Rotator|Lerp(Rotator) (Transformation|GetActorRotation) (Math|Rotator|FindLookatRotation (Transformation|GetWorldLocation (Variables|Character|GetMesh)) (Transformation|GetWorldLocation LookTarget)) _newtrack_0 true)))))
    (:Finished
      (Pawn|Components|CharacterMovement|SetMovementMode _charactermovement "MOVE_Walking" 0))))

(event EventCheckClosest
  (params (InPosition :type Scene%20Component%20Object%20Reference) (OutPosition :type Scene%20Component%20Object%20Reference)))

(event EventLookatTarget
  (params (Target :type Scene%20Component%20Object%20Reference) (BlendTime :type Float%20%28single-precision%29)))

(fn ConstructionScript)

(fn GetAnimationBlueprint
  (return 0))

(fn GetSkeletalMeshComponent
  (return (Variables|Character|GetMesh)))