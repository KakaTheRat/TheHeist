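; BP_HidingSpot is a hideout actor that a hider can enter and quit.
; Entering and quitting move the hider to the hiding or unhide position component's location and update an occupied flag, which CheckHidingSpot returns.
; The construction script picks one of three simple meshes based on the hide spot type.
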(event EventEnterHidingSpot
  (params (Hider :type Actor%20Object%20Reference))
  ;[1 1 1] Enter hideout
  (Transformation|SetActorLocation Hider (Transformation|GetWorldLocation (Variables|Default|GetHidingPosition)) false false)
  (Variables|Default|SetisOccupied true))

(event EventQuitHidingSpot
  (params (Hider :type Actor%20Object%20Reference))
  ;[1 1 1] Quit Hideout
  (Transformation|SetActorLocation Hider (Transformation|GetWorldLocation (Variables|Default|GetUnhidePosition)) false false)
  (Variables|Default|SetisOccupied false))

(fn ConstructionScript
  (bind _staticmesh (Variables|Default|GetStaticMesh))
  (if (== (Variables|Default|GetHideSpotType) 0)
    (Components|StaticMesh|SetStaticMesh _staticmesh "/Engine/EditorMeshes/ArcadeEditorSphere.ArcadeEditorSphere")
    (elif (== (Variables|Default|GetHideSpotType) 1)
      (Components|StaticMesh|SetStaticMesh _staticmesh "/Engine/EditorMeshes/Cascade/BackgroundCube.BackgroundCube")
      (else
        (Components|StaticMesh|SetStaticMesh _staticmesh "/Engine/BasicShapes/Cone.Cone")))))

(fn CheckHidingSpot
  (return (Variables|Default|GetisOccupied)))