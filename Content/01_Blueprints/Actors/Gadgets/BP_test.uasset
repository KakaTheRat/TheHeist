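; BP_test is a gadget actor, apparently a test, that launches its static mesh as a projectile when use is released.
; OnUseReleased activates ProjectileMovement, detaches the mesh in world space, sets it to query-only collision and makes it the movement's updated component.
; Velocity follows player pawn 0's forward vector at the component's initial speed, so aim ignores the gadget's own orientation.
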(event EventBeginPlay)

(event Collision|EventActorBeginOverlap
  (params (OtherActor :type Actor%20Object%20Reference)))

(event EventTick
  (params (DeltaSeconds :type Float%20%28single-precision%29)))

(event EventOnUseReleased
  (bind _staticmesh (Variables|Default|GetStaticMesh))
  (bind _projectilemovement (Variables|Default|GetProjectileMovement))
  (Components|Activation|Activate (Variables|Default|GetProjectileMovement) false)
  (Transformation|DetachFromComponent _staticmesh "KeepWorld" "KeepWorld" "KeepWorld" false)
  (Collision|SetCollisionEnabled _staticmesh "QueryOnly")
  (Components|Movement|SetUpdatedComponent _projectilemovement (Variables|Default|GetStaticMesh))
  (Variables|/Script/Engine.MovementComponent|SetVelocity _projectilemovement (* (Transformation|GetActorForwardVector (Game|Player|GetPlayerPawn 0)) (Variables|/Script/Engine.ProjectileMovementComponent|GetInitialSpeed (Variables|Default|GetProjectileMovement)))))

(fn ConstructionScript)