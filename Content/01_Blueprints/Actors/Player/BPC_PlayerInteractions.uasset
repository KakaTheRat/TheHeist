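; Player component that handles interacting with world objects, clicking widgets and hiding from AI.
; Interact input line traces from the owner along camera forward and sends InteractMessage to BPI_Interactable actors; left mouse drives the WidgetInteraction pointer.
; Hide unregisters AI sight stimuli and disables collision; QuitHidding reverses both and restores walking.
; Both events set IsHidden to false, and the node disabling movement is unwired.
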(event Custom|Hide
  (bind _owneraistimulis (Variables|Default|GetOwnerAiStimulis))
  ;[0.15 0.15 0.15 0.5] Hidding
  (Variables|Default|SetisHidden false)
  (Utilities|IsValid _owneraistimulis
    (:Is%20Valid
      (Class|AIPerceptionStimuliSourceComponent|UnregisterfromSense _owneraistimulis "/Script/AIModule.AISense_Sight")
      (Collision|SetActorEnableCollision (Variables|Default|GetOwner) false))))

(event Custom|QuitHidding
  (bind _owneraistimulis (Variables|Default|GetOwnerAiStimulis))
  (bind _owner (Variables|Default|GetOwner))
  ;[0.15 0.15 0.15 0.5] Quit Hidding
  (Variables|Default|SetisHidden false)
  (Utilities|IsValid _owneraistimulis
    (:Is%20Valid
      (Class|AIPerceptionStimuliSourceComponent|RegisterforSense _owneraistimulis "/Script/AIModule.AISense_Sight")
      (Pawn|Components|CharacterMovement|SetMovementMode (Actor|GetComponentbyClass _owner "/Script/Engine.CharacterMovementComponent") "MOVE_Walking" 0)
      (Collision|SetActorEnableCollision _owner true))))

(event Input|EnhancedActionEvents|EnhancedInputActionIA_Interact
  (params (ActionValue :type Boolean) (ElapsedSeconds :type Float%20%28double-precision%29) (TriggeredSeconds :type Float%20%28double-precision%29) (InputAction :type Input%20Action%20Object%20Reference :default "/Game/09_Input/Actions/IA_Interact.IA_Interact"))
  (bind _owner (Variables|Default|GetOwner))
  (bind _returnvalue (Transformation|GetActorLocation _owner))
  ;[1 1 1] Interact
  (:Started
    (bind _outhit (Collision|LineTraceByChannel _returnvalue (+ _returnvalue (* (Math|Vector|GetForwardVector (Actor|GetComponentbyClass (Variables|Default|GetOwner) "/Script/Engine.CameraComponent")) (Variables|Default|GetRaycastDistance))) "TraceTypeQuery1" false 0 "Persistent"))
    (Variables|Default|SetInteractedObject (.hitactor _outhit))
    (if (Utilities|DoesObjectImplementInterface (Variables|Default|GetInteractedObject) "/Game/01_Blueprints/Interfaces/BPI_Interactable.BPI_Interactable_C")
      (Class|BPIInteractable|Interact(Message) (Variables|Default|GetInteractedObject) (.hitcomponent _outhit)))))

(event EventBeginPlay
  (Variables|Default|SetOwnerAiStimulis (Actor|GetComponentbyClass (Components|GetOwner) "/Script/AIModule.AIPerceptionStimuliSourceComponent"))
  (Variables|Default|SetOwner (Components|GetOwner)))

(event Input|MouseEvents|LeftMouseButton
  (params (Key :type Key%20Structure :default "None"))
  (bind _owner (Variables|Default|GetOwner))
  (bind _returnvalue (Actor|GetComponentbyClass _owner "/Script/UMG.WidgetInteractionComponent"))
  ;[0.15 0.15 0.15 0.5] Widget interaction
  (:Pressed
    (Class|WidgetInteractionComponent|PressPointerKey _returnvalue "LeftMouseButton"))
  (:Released
    (Class|WidgetInteractionComponent|ReleasePointerKey _returnvalue "LeftMouseButton")))