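; Keypad (digicode) actor that takes a four-digit code from nine widget buttons and fires Success or Fail.
; On BeginPlay it gives each button widget its zero-based array index as ID and binds its click event.
; Clicks append IDs to an input string shown on a text render, which is compared to Code at four characters.
; A match permanently unbinds the buttons, while a miss briefly shows an error before re-enabling entry.
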(event Custom|Cliqued
  (params (Id :type Integer))
  (bind _output_get (Variables|Default|SetInput (Utilities|String|Append (Variables|Default|GetInput) (Utilities|String|ToString(Integer) Id))))
  (Rendering|Components|TextRender|SetText (Variables|Default|GetTextRender) (Utilities|Text|ToText(String) _output_get))
  (if (== 4 (Utilities|String|Len _output_get))
    (CallFunction|CheckValid)))

(event Custom|CheckValid
  (if (Utilities|Enum|Equal(Enum) (Variables|Default|GetInput) (Utilities|String|ToString(Integer) (Variables|Default|GetCode)))
    (Default|CallSuccess)
    (CallFunction|Disable)
    (Rendering|Components|TextRender|SetText (Variables|Default|GetTextRender) (Utilities|String|SelectText "CODE VALID" "" true))
    (else
      (Default|CallFail)
      (CallFunction|Restart))))

(event Custom|Disable
  (for _array_element (Variables|Default|GetButtons)
    (EventDispatchers|UnbindallEventsfromClicked _array_element)))

(event Custom|Restart
  (CallFunction|Disable)
  (Variables|Default|SetInput "")
  (Rendering|Components|TextRender|SetText (Variables|Default|GetTextRender) (Utilities|String|SelectText "Error" "" true))
  (Utilities|FlowControl|Delay 1.0)
  (CallFunction|Subscribe)
  (Rendering|Components|TextRender|SetText (Variables|Default|GetTextRender) (Utilities|String|SelectText "ENTER CODE" "" true)))

(event Custom|Subscribe
  (for _array_element (Variables|Default|GetButtons)
    (EventDispatchers|BindEventtoClicked _array_element (delegate Custom|Cliqued))))

(event EventBeginPlay
  (for _array_element (Utilities|Array|MakeArray (Variables|Default|GetButton1) (Variables|Default|GetButton2) (Variables|Default|GetButton3) (Variables|Default|GetButton4) (Variables|Default|GetButton5) (Variables|Default|GetButton6) (Variables|Default|GetButton7) (Variables|Default|GetButton8) (Variables|Default|GetButton9))
    (bind _aswbp_digicode_button (Utilities|Casting|CastToWBP_DigicodeButton (UserInterface|GetWidget _array_element)))
    (bind _returnvalue (Utilities|Array|Add (Variables|Default|GetButtons) _aswbp_digicode_button))
    (Variables|/Game/01_Blueprints/Digicode/Widget/WBP_DigicodeButton.WBP_DigicodeButton_C|SetButtonId _aswbp_digicode_button _returnvalue))
  (CallFunction|Subscribe))

(fn ConstructionScript)