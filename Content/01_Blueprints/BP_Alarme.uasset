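; BP_Alarme is an alarm light actor that flashes red once a player has been found.
; On BeginPlay it turns its SpotLight off, gets the BP_CheckActor in the level and binds to its OnFindPlayer dispatcher.
; When that fires, a looping one-second timer drives a FlipFlop that alternates the light between intense red and off, with no logic to stop it.
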(event Custom|OnFindPlayer_Event
  (Utilities|Time|SetTimerbyEvent (delegate Custom|SwitchLight_Event) 1.0 true))

(event Custom|SwitchLight_Event
  (Utilities|FlowControl|FlipFlop
    (:A
      (Rendering|Components|Light|SetIntensity (Variables|Default|GetSpotLight) 1e+05)
      (Rendering|Components|Light|SetLightColor (Variables|Default|GetSpotLight) "(R=1.000000,G=0.029833,B=0.000115,A=1.000000)" true))
    (:B
      (Rendering|Components|Light|SetIntensity (Variables|Default|GetSpotLight) 0.0))))

(event EventBeginPlay
  (Rendering|Components|Light|SetIntensity (Variables|Default|GetSpotLight) 0.0)
  (bind _returnvalue (Actor|GetActorOfClass "/Game/01_Blueprints/BP_CheckActor.BP_CheckActor_C"))
  (EventDispatchers|BindEventtoOnFindPlayer _returnvalue (delegate Custom|OnFindPlayer_Event)))

(fn ConstructionScript)