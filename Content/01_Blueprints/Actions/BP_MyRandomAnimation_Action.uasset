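; BP_MyRandomAnimation_Action is a guard action that plays a random montage from its Animations array on the owning guard.
; On execute, it gets the guard's skeletal mesh via GetSkeletalMeshComponentMessage, prints a randomly picked animation name, then plays a montage.
; The print and playback each make their own random pick, so the printed name can differ from the montage played.
; Only the montage's Completed output calls OnActionEnded.
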(event EventOnExecute
  (params (OwningGuard :type Actor%20Object%20Reference))
  (bind _animations (Variables|Default|GetAnimations))
  (bind _animations_2 (Variables|Default|GetAnimations))
  (bind _returnvalue (Utilities|Array|Length _animations_2))
  (bind _returnvalue_2 (- _returnvalue 1))
  (bind _returnvalue_3 (Math|Random|RandomIntegerinRange 0 _returnvalue_2))
  (bind _output (Utilities|Array|Get(acopy) _animations _returnvalue_3))
  (bind _returnvalue_4 (Class|EntitiesInterface|GetSkeletalMeshComponent(Message) OwningGuard))
  (Development|PrintString OwningGuard (Utilities|GetDisplayName _output))
  (Animation|Montage|PlayMontage _returnvalue_4 _output
    (:OnCompleted
      (Class|ActionBase|OnActionEnded))))