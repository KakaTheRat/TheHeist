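; Coffee machine action actor that has the interacting character play a sequence of grabbing a cup, starting the machine and drinking.
; LaunchAction triggers the Interactable component, and Interact caches the actor's skeletal mesh through a message call.
; Chained montages drive the steps, with pickup notifies snapping the cup cylinder to the right hand or holder.
; After a short delay the machine montage plays (notify only prints debug text), then drinking attaches the cup to the left hand.
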(event Custom|Grab%20Cup
  (bind _notifyname (Animation|Montage|PlayMontage (Variables|Default|GetNewVar) "/Game/11_Animations/PickUp_R_Hand_Bottle_Montage1.PickUp_R_Hand_Bottle_Montage1")
    (:OnCompleted
      (Utilities|FlowControl|Delay 3.0)
      (CallFunction|StartMachine))
    (:OnNotifyBegin
      (switch name _notifyname
        (:OnInteract
          (Transformation|AttachComponentToComponent (Variables|Default|GetCylinder) (stale EventInteract _returnvalue) "weapon_right" "SnapToTarget" "SnapToTarget" "KeepWorld" true))
        (:Destroy
          (Transformation|AttachComponentToComponent (Variables|Default|GetCylinder) (Variables|Default|GetCupHolder) "None" "SnapToTarget" "SnapToTarget" "KeepWorld" true))))))

(event Custom|Start%20Machine
  (bind _notifyname (Animation|Montage|PlayMontage (Variables|Default|GetNewVar) "/Game/11_Animations/A_TestSwitcherAction_Montage.A_TestSwitcherAction_Montage")
    (:OnCompleted
      (CallFunction|Drink))
    (:OnNotifyBegin
      (switch name _notifyname
        (:OnInteract
          (Development|PrintString "fggh"))))))

(event Custom|Drink
  (Animation|Montage|PlayMontage (Variables|Default|GetNewVar) "/Game/11_Animations/Actions/CoffeeMachine/Drinking_Anim_Montage.Drinking_Anim_Montage"
    (:then
      (Transformation|AttachComponentToComponent (Variables|Default|GetCylinder) (Variables|Default|GetNewVar) "weapon_left" "SnapToTarget" "SnapToTarget" "KeepWorld" true))))

(event EventBeginPlay)

(event Collision|EventActorBeginOverlap
  (params (OtherActor :type Actor%20Object%20Reference)))

(event EventTick
  (params (DeltaSeconds :type Float%20%28single-precision%29)))

(event EventLaunchAction
  (params (NewParam :type Actor%20Object%20Reference))
  (Class|InteractableComponent|InteractwithSpecificInteraction (Variables|Default|GetInteractable) "/Script/TheHeist.CustomInteractionData" 0 NewParam "Default"))

(event EventInteract
  (params (HitComponent :type Scene%20Component%20Object%20Reference) (InteractingActor :type Actor%20Object%20Reference) (Context :type EInteractionContext%20Enum :default "Default") (Data :type Interaction%20Data%20Object%20Reference))
  (bind _returnvalue (Class|EntitiesInterface|GetSkeletalMeshComponent(Message) InteractingActor))
  (Variables|Default|SetNewVar _returnvalue)
  (CallFunction|GrabCup))

(fn ConstructionScript)