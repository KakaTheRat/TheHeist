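; Actor component that runs one randomly chosen action at a time on its owner.
; When triggered while idle, OnAction constructs an object from a random class in Actions and executes it with the owner.
; It then flags itself busy and binds to the action's ended delegate, whose callback unbinds, clears the current action and frees the component.
; The delegate is bound after execution starts, so an action ending synchronously is not caught.
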(event Custom|OnAction
  (if (not (Variables|Default|GetisInAction))
    (bind _returnvalue (Game|ConstructObjectfromClass (Utilities|Array|Get(acopy) (Variables|Default|GetActions) (Math|Random|RandomIntegerinRange 0 (- (Utilities|Array|Length (Variables|Default|GetActions)) 1)))))
    (bind _output_get (Variables|Default|SetCurrentAction _returnvalue))
    (Class|ActionBase|OnExecute _output_get (Components|GetOwner))
    (Variables|Default|SetisInAction true)
    (EventDispatchers|BindEventtoOnActionEndedDelegate (Variables|Default|GetCurrentAction) (delegate Custom|ActionEnd))))

(event Custom|ActionEnd
  (EventDispatchers|UnbindallEventsfromOnActionEndedDelegate (Variables|Default|GetCurrentAction))
  (Variables|Default|SetCurrentAction 0)
  (Variables|Default|SetisInAction false))

(event EventBeginPlay)

(event EventTick
  (params (DeltaSeconds :type Float%20%28single-precision%29)))