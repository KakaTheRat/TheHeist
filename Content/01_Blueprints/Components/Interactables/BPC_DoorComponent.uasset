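; Door interactable component that toggles its attached component between open and closed by swinging it around yaw.
; Open calls the parent logic, flips IsOpened, captures the current relative rotation, then restarts a timeline.
; Each update lerps yaw from that captured value to Angle or back to zero, keeping roll and pitch fixed.
; An OpeningDirection switch exists but is never executed.
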(event EventOpen
  (params (MeshInteracted :type Scene%20Component%20Object%20Reference))
  (bind _attachedcomponent (Variables|Default|GetAttachedComponent))
  (bind _relativerotation (Variables|/Script/Engine.SceneComponent|GetRelativeRotation _attachedcomponent))
  (|CallParentFunction MeshInteracted)
  (Variables|Default|SetisOpened (not (Variables|Default|GetisOpened)))
  (Class|ComponentTimelineLibrary|InitializeComponentTimelines)
  (Variables|Default|SetRelative%20Rotation%20X (.roll _relativerotation))
  (Variables|Default|SetRelative%20Rotation%20Y (.pitch _relativerotation))
  (Variables|Default|SetRelative%20Rotation%20Z (.yaw _relativerotation))
  (bind _alpha (|ComponentTimeline 0.0) ; enters at PlayFromStart
    (:Update
      (Variables|Default|SetAlpha _alpha)
      (Transformation|SetRelativeRotation (Variables|Default|GetAttachedComponent) (Math|Rotator|MakeRotator (Variables|Default|GetRelative%20Rotation%20X) (Variables|Default|GetRelative%20Rotation%20Y) (select (Variables|Default|GetisOpened) (Math|Float|Lerp (Variables|Default|GetRelative%20Rotation%20Z) (Variables|Default|GetAngle) (Variables|Default|GetAlpha)) (Math|Float|Lerp (Variables|Default|GetRelative%20Rotation%20Z) 0.0 (Variables|Default|GetAlpha)))) false false))))