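; Interactable component that toggles its owner's light or audio on Interact, according to its ActivationType.
; Lights switch via intensity; audio plays or stops, with a looping timer re-reporting noise events to AI perception while active.
; BeginPlay applies the default activation state.
; Helpers enable or disable interaction and report whether the object is still in its default state.
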(event Custom|OnBeginFocus)

(event Custom|OnEndFocus)

(event EventBeginPlay
  (|CallParentFunction)
  ;[0.15 0.15 0.15 0.5] Object state setter at start of the game
  (if (!= (Variables|Default|GetbIsActivatedByDefault) (Variables|Default|GetbIsActivated))
    (CallFunction|ActivateObject))
  (Variables|Default|SetbIsActivated (Variables|Default|GetbIsActivatedByDefault)))

(event EventTick
  (params (DeltaSeconds :type Float%20%28single-precision%29)))

(event EventInteract
  (params (HitComponent :type Scene%20Component%20Object%20Reference))
  (CallFunction|ActivateObject))

(fn ActivateObject
  (bind _returnvalue (Components|GetOwner))
  (bind _returnvalue_2 (Components|GetOwner))
  (bind _self self)
  (bind _returnvalue_3 (Actor|GetComponentbyClass _returnvalue "/Script/Engine.LightComponent"))
  (bind _returnvalue_4 (Components|GetOwner _self))
  (bind _returnvalue_5 (Actor|GetComponentbyClass _returnvalue_2 "/Script/Engine.AudioComponent"))
  (if (Variables|Default|GetbIsInteractable)
    (switch Utilities|FlowControl|Switch|SwitchonE_ActivationType (Variables|Default|GetActivationType)
      (:NewEnumerator0
        ;[0.15 0.15 0.15 0.5] Light Behavior
        (Utilities|IsValid _returnvalue_3
          (:Is%20Valid
            (Rendering|Components|Light|SetIntensity _returnvalue_3 (* (Variables|Light|GetLightIntensity) (not (Variables|Default|GetbIsActivated)))))))
      (:NewEnumerator1
        ;[0.15 0.15 0.15 0.5] Audio behavior
        (Utilities|IsValid _returnvalue_5
          (:Is%20Valid
            (if (Variables|Default|GetbIsActivated)
              (Audio|Components|Audio|Stop _returnvalue_5)
              (Utilities|Time|ClearTimerbyFunctionName 0 "NewFunction")
              (else
                (Audio|Components|Audio|Play _returnvalue_5 0.0)
                (Class|AISenseHearing|ReportNoiseEvent (Transformation|GetActorLocation _returnvalue_4) 1.0 _returnvalue_4 1.5e+03 "None")
                (Utilities|Time|SetTimerbyEvent (EventDispatchers|CreateEvent :!event NewFunction) 1.0 true)))))))
    (Variables|Default|SetbIsActivated (not (Variables|Default|GetbIsActivated)))))

(fn EnableInteraction
  (Variables|Default|SetbIsInteractable true))

(fn DisableInteraction
  (Variables|Default|SetbIsInteractable false))

(fn IsinNormalState
  (if (== (Variables|Default|GetbIsActivated) (Variables|Default|GetbIsActivatedByDefault))
    (return true)
    (else
      (return false))))

(fn NewFunction
  (bind _self self)
  (bind _returnvalue (Components|GetOwner _self))
  (Class|AISenseHearing|ReportNoiseEvent (Transformation|GetActorLocation _returnvalue) 1.0 _returnvalue 1.5e+03 "None"))