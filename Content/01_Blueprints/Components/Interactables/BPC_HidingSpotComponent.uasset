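; Hiding spot component that moves the player into and out of a hiding place on interaction.
; HidingInteract calls Hide on BPC_PlayerInteractions if the player is not hidden, then starts a looping frame-interval timer.
; The timer slides the player at constant speed toward HidingPosition or QuitPosition, depending on IsPlayerHidden.
; On arrival it clears the timers and flips that flag, calling QuitHidding on the player's component when leaving.
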(event Custom|Quit
  (if (Variables|Default|GetIsPlayerHidden)
    (Variables|Default|SetIsPlayerHidden false)
    (Default|QuitHidding (Actor|GetComponentbyClass (Variables|Default|GetPlayerRef) "/Game/01_Blueprints/Actors/Player/BPC_PlayerInteractions.BPC_PlayerInteractions_C"))
    (else
      (Variables|Default|SetIsPlayerHidden true))))

(event Custom|Hide
  (bind _playerref (Variables|Default|GetPlayerRef))
  (bind _isplayerhidden (Variables|Default|GetIsPlayerHidden))
  (Transformation|SetActorTransform _playerref (Math|Transform|MakeTransform (Math|Interpolation|VInterptoConstant (Transformation|GetActorLocation _playerref) (Transformation|GetWorldLocation (select _isplayerhidden (Variables|Default|GetQuitPosition) (Variables|Default|GetHidingPosition))) (Utilities|Time|GetWorldDeltaSeconds) 1e+03) "0, 0, 0" "1.000000,1.000000,1.000000"))
  (if (Utilities|Operators|EqualEqual (Transformation|GetActorLocation (Variables|Default|GetPlayerRef)) (Transformation|GetWorldLocation (select _isplayerhidden (Variables|Default|GetQuitPosition) (Variables|Default|GetHidingPosition))) 0.01)
    (Utilities|Time|ClearandInvalidateTimerbyHandle (stale Custom|HidingInteract _returnvalue_2))
    (Utilities|Time|ClearandInvalidateTimerbyHandle (stale Custom|HidingInteract _returnvalue))
    (CallFunction|Quit)))

(event Custom|HidingInteract
  (if (Variables|/Game/01_Blueprints/Actors/Player/BPC_PlayerInteractions.BPC_PlayerInteractions_C|GetisHidden (Actor|GetComponentbyClass (Variables|Default|GetPlayerRef) "/Game/01_Blueprints/Actors/Player/BPC_PlayerInteractions.BPC_PlayerInteractions_C"))
    (bind _returnvalue (Utilities|Time|SetTimerbyEvent (delegate Custom|Hide) (Utilities|Time|GetWorldDeltaSeconds) true))
    (else
      (Default|Hide (Actor|GetComponentbyClass (Variables|Default|GetPlayerRef) "/Game/01_Blueprints/Actors/Player/BPC_PlayerInteractions.BPC_PlayerInteractions_C"))
      (bind _returnvalue_2 (Utilities|Time|SetTimerbyEvent (delegate Custom|Hide) (Utilities|Time|GetWorldDeltaSeconds) true)))))

(event EventBeginPlay
  (Variables|Default|SetPlayerRef (Game|Player|GetPlayerPawn 0)))

(event EventTick
  (params (DeltaSeconds :type Float%20%28single-precision%29)))