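; Drawer interactable component that toggles the attached component between open and closed with a sliding motion.
; Open calls the parent implementation, flips IsOpened, caches the current relative location and plays a component timeline from the start.
; Each update lerps only local Y from the cached position toward Distance when opening or zero when closing, so the closed pose is assumed to sit at Y zero.
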(event EventOpen
  (params (MeshInteracted :type Scene%20Component%20Object%20Reference))
  (bind _attachedcomponent (Variables|Default|GetAttachedComponent))
  (bind _relativelocation (Variables|/Script/Engine.SceneComponent|GetRelativeLocation _attachedcomponent))
  (|CallParentFunction MeshInteracted)
  (Variables|Default|SetisOpened (not (Variables|Default|GetisOpened)))
  (Class|ComponentTimelineLibrary|InitializeComponentTimelines)
  (Variables|Default|SetRelative%20Location%20X (.x _relativelocation))
  (Variables|Default|SetRelative%20Location%20Y (.y _relativelocation))
  (Variables|Default|SetRelative%20Location%20Z (.z _relativelocation))
  (bind _alpha (|ComponentTimeline 0.0) ; enters at PlayFromStart
    (:Update
      (Variables|Default|SetAlpha _alpha)
      (Transformation|SetRelativeLocation (Variables|Default|GetAttachedComponent) (Math|Vector|MakeVector (Variables|Default|GetRelative%20Location%20X) (select (Variables|Default|GetisOpened) (Math|Float|Lerp (Variables|Default|GetRelative%20Location%20Y) (Variables|Default|GetDistance) (Variables|Default|GetAlpha)) (Math|Float|Lerp (Variables|Default|GetRelative%20Location%20Y) 0.0 (Variables|Default|GetAlpha))) (Variables|Default|GetRelative%20Location%20Z)) false false))))