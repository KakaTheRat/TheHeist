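; BPC_OpenableComponent is an interactable component for openable objects that manages their "Open" or "Close" interaction text.
; Interact forwards the hit component to Open, which acts only when it matches AttachedComponent and sets InteractText from IsOpened.
; The graph neither changes IsOpened nor moves anything, and IsCurrentlyActive always returns false.
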(event Custom|Open
  (params (MeshInteracted :type Scene%20Component%20Object%20Reference))
  (if (== MeshInteracted (Variables|Default|GetAttachedComponent))
    (if (Variables|Default|GetisOpened)
      (Variables|Default|SetInteractText "Close")
      (else
        (Variables|Default|SetInteractText "Open")))))

(event EventInteract
  (params (HitComponent :type Scene%20Component%20Object%20Reference))
  (CallFunction|Open HitComponent))

(fn IsCurrentlyActive
  (return false))