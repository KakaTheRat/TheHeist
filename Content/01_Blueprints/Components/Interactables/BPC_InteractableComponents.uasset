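; BPC_InteractableComponents is an interactable actor component that binds to one scene component on its owning actor.
; On BeginPlay it searches the owner's scene components and stores the first whose object name matches AttachedComponentName as AttachedComponent.
; Interact is an empty event and IsCurrentlyActive always returns false, so both act as stubs with no behavior here.
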(event EventBeginPlay
  ;[0.15 0.15 0.15 0.5] Attach the scene component to each interactable component. This way, every thing is assigned (using component name with "AttachedComponentName"). Each component is used for 1 scene component
  (bind _array_element (Utilities|Array|ForEachLoopwithBreak (Actor|GetComponentsByClass (Components|GetOwner) "/Script/Engine.SceneComponent") :!label _label)
    (:LoopBody
      (if (Utilities|Enum|Equal(Enum) (Utilities|GetObjectName _array_element) (Utilities|String|ToString(Name) (Variables|Default|GetAttachedComponentName)))
        (Variables|Default|SetAttachedComponent _array_element)
        (goto _label Break)))))

(event EventInteract
  (params (HitComponent :type Scene%20Component%20Object%20Reference)))

(fn IsCurrentlyActive
  (return false))