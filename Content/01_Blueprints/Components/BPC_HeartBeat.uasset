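; Actor component that gives its owner proximity feedback through a heartbeat sound and camera post-process as entities approach.
; On BeginPlay it spawns a 2D heartbeat sound and adds a MaxDistance-radius sphere to the owner, whose overlaps track actors implementing EntitiesInterface.
; While any are tracked, Tick maps the closest one's distance to the sound's Volume and HeartRate parameters and a camera post-process setting.
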(event Custom|Overlap
  (params (OverlappedComponent :type Primitive%20Component%20Object%20Reference) (OtherActor :type Actor%20Object%20Reference) (OtherComp :type Primitive%20Component%20Object%20Reference) (OtherBodyIndex :type Integer) (bFromSweep :type Boolean) (SweepResult :type Hit%20Result%20Structure%20%28by%20ref%29))
  (if (not (== OtherActor (Components|GetOwner)))
    (if (Utilities|DoesObjectImplementInterface OtherActor "/Script/TheHeist.EntitiesInterface")
      (Utilities|Array|AddUnique (Variables|Default|GetActors) OtherActor)
      (Variables|Default|SetIsDetected true))))

(event Custom|LeaveOverlap
  (params (OverlappedComponent :type Primitive%20Component%20Object%20Reference) (OtherActor :type Actor%20Object%20Reference) (OtherComp :type Primitive%20Component%20Object%20Reference) (OtherBodyIndex :type Integer))
  (bind _actors (Variables|Default|GetActors))
  (bind _returnvalue (Utilities|Array|RemoveItem _actors OtherActor))
  (if _returnvalue
    (if (Utilities|Array|IsEmpty _actors)
      (Variables|Default|SetIsDetected false))))

(event EventBeginPlay
  (bind _returnvalue (Components|GetOwner))
  (bind _returnvalue_2 (Audio|SpawnSound2D (Variables|Default|GetHeartBeat) 1.0 1.0 0.0 0))
  (bind _output_get (Variables|Default|SetSoundComp _returnvalue_2))
  (Audio|Parameter|SetFloatParameter _output_get "Volume" 0.0 :!class /Script/AudioExtensions.AudioParameterControllerInterface)
  (bind _returnvalue_3 (Game|AddComponentbyClass _returnvalue "/Script/Engine.SphereComponent" false))
  (bind _output_get_2 (Variables|Default|SetSphereComp _returnvalue_3))
  (Transformation|AttachComponentToComponent _output_get_2 (Variables|/Script/Engine.Actor|GetRootComponent _returnvalue) "" "KeepRelative" "KeepRelative" "KeepRelative" true)
  (Components|Sphere|SetSphereRadius (Variables|Default|GetSphereComp) (Variables|Default|GetMaxDistance) true)
  (Collision|BindEventtoOnComponentBeginOverlap (Variables|Default|GetSphereComp) (delegate Custom|Overlap))
  (Collision|BindEventtoOnComponentEndOverlap (Variables|Default|GetSphereComp) (delegate Custom|LeaveOverlap)))

(event EventTick
  (params (DeltaSeconds :type Float%20%28single-precision%29))
  (bind _returnvalue (Components|GetOwner))
  (if (Variables|Default|GetIsDetected)
    (bind _returnvalue_2 (Class|FormationHelper|GetClosestActors (Variables|Default|GetActors) (Transformation|GetActorLocation _returnvalue) 1))
    (Audio|Parameter|SetFloatParameter (Variables|Default|GetSoundComp) "Volume" (Math|Float|Clamp(Float) (- 1.0 (/ (Transformation|GetDistanceTo (Utilities|Array|Get(acopy) _returnvalue_2) _returnvalue) (Variables|Default|GetMaxDistance)))) :!class /Script/AudioExtensions.AudioParameterControllerInterface)
    (Audio|Parameter|SetFloatParameter (Variables|Default|GetSoundComp) "HeartRate" (Math|Float|Clamp(Float) (- 1.0 (/ (Transformation|GetDistanceTo (Utilities|Array|Get(acopy) _returnvalue_2) _returnvalue) (Variables|Default|GetMaxDistance)))) :!class /Script/AudioExtensions.AudioParameterControllerInterface)
    (Variables|/Script/Engine.CameraComponent|SetPostProcessSettings (Actor|GetComponentbyClass (Components|GetOwner) "/Script/Engine.CameraComponent") (Utilities|Struct|MakePostProcessSettings (+ (* (Math|Float|Clamp(Float) (- 1.0 (/ (Transformation|GetDistanceTo (Utilities|Array|Get(acopy) _returnvalue_2) _returnvalue) (Variables|Default|GetMaxDistance)))) 2.0) 0.5) 2999.0))))