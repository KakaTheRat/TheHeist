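; Player component that detects and triggers interactions with InteractableComponent actors, and handles the player's hiding state.
; An added sphere collider runs a looping check timer, whose camera line trace picks the targeted component and toggles the prompt widget.
; IA_Interact runs a single interaction directly or shows a choice widget for several.
; Hiding disables collision and AI sight stimulus, with W triggering the stored interaction while hidden.
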(event Custom|OnColliderOverlapped
  (params (OverlappedComponent :type Primitive%20Component%20Object%20Reference) (OtherActor :type Actor%20Object%20Reference) (OtherComp :type Primitive%20Component%20Object%20Reference) (OtherBodyIndex :type Integer) (bFromSweep :type Boolean) (SweepResult :type Hit%20Result%20Structure%20%28by%20ref%29))
  ;[0.15 0.15 0.15 0.5] Manage the overlap event. If minimum a single overlapped, starts the interaction checking
  (Utilities|IsValid (Actor|GetComponentbyClass OtherActor "/Script/TheHeist.InteractableComponent")
    (:Is%20Valid
      (Utilities|Array|AddUnique (Variables|Overlapping|GetOverlappedInteractables) OtherActor)
      (bind _returnvalue (Utilities|Time|SetTimerbyEvent (delegate Custom|CheckForInteractionEvent) 0.1 true true))
      (Variables|Default|SetInteractionTimer _returnvalue))))

(event Custom|OnColliderEndOverlapped
  (params (OverlappedComponent :type Primitive%20Component%20Object%20Reference) (OtherActor :type Actor%20Object%20Reference) (OtherComp :type Primitive%20Component%20Object%20Reference) (OtherBodyIndex :type Integer))
  (bind _overlappedinteractables (Variables|Overlapping|GetOverlappedInteractables))
  ;[0.15 0.15 0.15 0.5] Manage the end overlap event. If not a single overlapped left, stops the interaction checking
  (Utilities|IsValid (Actor|GetComponentbyClass OtherActor "/Script/TheHeist.InteractableComponent")
    (:Is%20Valid
      (if true
        (Utilities|Array|RemoveItem _overlappedinteractables OtherActor)
        (if (Utilities|Array|IsEmpty _overlappedinteractables)
          (Utilities|Time|ClearandInvalidateTimerbyHandle (Variables|Default|GetInteractionTimer))
          (if (Variables|Widget|Getb_InteractionButtonWidgetActivated)
            (CallFunction|ShouldActivateButtonInteractionWidget false)))))))

(event Custom|CheckForInteractionEvent
  ;[0.15 0.15 0.15 0.5] Manage the overlap event. If minimum a single overlapped, starts the interaction checking
  (CallFunction|CheckforInteraction))

(event Custom|CheckForInteraction
  (bind _returnvalue (Game|GetPlayerCameraManager 0))
  (bind _returnvalue_2 (Camera|GetCameraLocation _returnvalue))
  ;[1 1 1] Checks for an interaction to communicate with. Will display the interaction button widget
  (if (not (Variables|Default|GetIsInteracting))
    (bind _outhit (Collision|LineTraceByChannel _returnvalue_2 (+ _returnvalue_2 (* (Math|Vector|GetForwardVector (Camera|GetCameraRotation (Game|GetPlayerCameraManager 0))) (Variables|LineTrace|GetRaycastDistance))) "TraceTypeQuery1" false 0 "ForOneFrame"))
    (if (.bblockinghit _outhit)
      (Utilities|IsValid (.hitactor _outhit)
        (:Is%20Valid
          (Utilities|IsValid (Actor|GetComponentbyClass (.hitactor _outhit) "/Script/TheHeist.InteractableComponent")
            (:Is%20Valid
              (Variables|LineTrace|SetInteractableObject (.hitactor _outhit))
              (for _array_element (Variables|/Script/TheHeist.InteractableComponent|GetAllComponentInteractablePlayer (Actor|GetComponentbyClass (.hitactor _outhit) "/Script/TheHeist.InteractableComponent"))
                (if (== (.hitcomponent _outhit) _array_element)
                  (Variables|LineTrace|SetHitComponent (.hitcomponent _outhit))
                  (Transformation|SetActorLocation (Variables|Default|GetInteractionSignalWidgetInstance) (.Origin (Collision|GetComponentBounds (.hitcomponent _outhit))) false false)
                  (if (not (Variables|Widget|Getb_InteractionButtonWidgetActivated))
                    (CallFunction|ShouldActivateButtonInteractionWidget true)))))
            (:Is%20Not%20Valid
              (if (Variables|Widget|Getb_InteractionButtonWidgetActivated)
                (CallFunction|ShouldActivateButtonInteractionWidget false))))))
      (elif (Variables|Widget|Getb_InteractionButtonWidgetActivated)
        (CallFunction|ShouldActivateButtonInteractionWidget false)))))

(event Custom|ShouldActivateButtonInteractionWidget
  (params (b_ShouldActivateButton :type Boolean))
  ;[0.15 0.15 0.15 0.5] Interaction Button Widget management
  (Default|CallOnInteractionButtonActivated b_ShouldActivateButton)
  (Variables|Widget|Setb_InteractionButtonWidgetActivated b_ShouldActivateButton))

(event Custom|EndOfInteraction
  (params (InteractingActor :type Actor%20Object%20Reference) (InteractionType :type Interaction%20Data%20Object%20Reference))
  ;[0.15 0.15 0.15 0.5] On interaction button pressed, trigger the interaction
  (Variables|Default|SetInteraction%20Type InteractionType)
  (Variables|Default|SetIsInteracting false)
  (Variables|LineTrace|SetInteractableObject 0)
  (Variables|LineTrace|SetCurrentInteractionComponentClicked 0))

(event Custom|OnInteractionBind
  (params (InteractionName :type String))
  ;[0.15 0.15 0.15 0.5] Begin, initialises, the interaction widgets mostly.
  (CallFunction|OnInteractionClicked InteractionName))

(event Custom|OnInteractionClicked
  (params (Interaction%20Name :type String))
  (bind _currentinteractionobjectclicked (Variables|Default|GetCurrentInteractionObjectClicked))
  (bind _returnvalue (Actor|GetComponentbyClass _currentinteractionobjectclicked "/Script/TheHeist.InteractableComponent"))
  ;[0.15 0.15 0.15 0.5] On interaction button pressed, trigger the interaction
  (Utilities|IsValid _returnvalue
    (:Is%20Valid
      (Class|InteractableComponent|InteractwithObject _returnvalue Interaction%20Name (Variables|LineTrace|GetCurrentInteractionComponentClicked) (Variables|Default|GetOwner) "Default")
      (Class|InteractionWidgetActor|HideWidget (Variables|Default|GetInteractionChoiceWidgetInstance))
      (Variables|Default|SetIsInteracting true)
      (CallFunction|ShouldActivateButtonInteractionWidget false)
      (EventDispatchers|BindEventtoOnInteractionEndedEvent _returnvalue (delegate Custom|EndOfInteraction)))))

(event Input|EnhancedActionEvents|EnhancedInputActionIA_Interact
  (params (ActionValue :type Boolean) (ElapsedSeconds :type Float%20%28double-precision%29) (TriggeredSeconds :type Float%20%28double-precision%29) (InputAction :type Input%20Action%20Object%20Reference :default "/Game/09_Input/Actions/IA_Interact.IA_Interact"))
  ;[0.15 0.15 0.15 0.5] On interaction button pressed, trigger the interaction
  (:Started
    (bind _interactableobject (Variables|LineTrace|GetInteractableObject)
      (:then
        (Variables|Default|SetCurrentInteractionObjectClicked _interactableobject)
        (Utilities|IsValid (Actor|GetComponentbyClass _interactableobject "/Script/TheHeist.InteractableComponent")
          (:Is%20Valid
            (bind _hitcomponent (Variables|LineTrace|GetHitComponent)
              (:then
                (Variables|LineTrace|SetCurrentInteractionComponentClicked _hitcomponent)
                (bind _returnvalue (Class|InteractableComponent|GetInteractionsforAComp (Actor|GetComponentbyClass _interactableobject "/Script/TheHeist.InteractableComponent") _hitcomponent))
                (Class|InteractionWidgetActor|ClearEntries (Variables|Default|GetInteractionChoiceWidgetInstance))
                (if (<= (Utilities|Array|Length _returnvalue) 1)
                  (CallFunction|OnInteractionClicked (Utilities|Array|Get(acopy) _returnvalue))
                  (else
                    (for _array_element _returnvalue
                      (Class|InteractionWidgetActor|AddInteractionEntry (Variables|Default|GetInteractionChoiceWidgetInstance) _array_element))
                    (Utilities|IsValid (Variables|Default|GetCurrentInteractionObjectClicked)
                      (:Is%20Valid
                        (Class|InteractionWidgetActor|ShowWidget (Variables|Default|GetInteractionChoiceWidgetInstance) (+ (.Origin (Collision|GetActorBounds (Variables|Default|GetCurrentInteractionObjectClicked) false false)) (Math|Vector|MakeVector 0.0 0.0 6e+01) (* (Transformation|GetActorForwardVector (Variables|Default|GetCurrentInteractionObjectClicked)) 5e+01) (* (Transformation|GetActorRightVector (Variables|Default|GetCurrentInteractionObjectClicked)) 8e+01))))))))
              (:else)))))
      (:else))))

(event EventHide
  (bind _owneraistimulis (Variables|Default|GetOwnerAiStimulis))
  ;[0.15 0.15 0.15 0.5] Hidding
  (Variables|Default|Setb_isHidden true)
  (Utilities|IsValid _owneraistimulis
    (:Is%20Valid
      (Class|AIPerceptionStimuliSourceComponent|UnregisterfromSense _owneraistimulis "/Script/AIModule.AISense_Sight")
      (Collision|SetActorEnableCollision (Variables|Default|GetOwner) false)
      (bind _ownerhud (Variables|Widget|GetOwnerHUD)
        (:then
          (Default|AddExtraInteraction _ownerhud "Sortir" "None"))
        (:else)))))

(event EventQuitHiding
  (bind _owneraistimulis (Variables|Default|GetOwnerAiStimulis))
  (bind _owner (Variables|Default|GetOwner))
  ;[0.15 0.15 0.15 0.5] Quit Hidding
  (Variables|Default|Setb_isHidden false)
  (Utilities|IsValid _owneraistimulis
    (:Is%20Valid
      (Class|AIPerceptionStimuliSourceComponent|RegisterforSense _owneraistimulis "/Script/AIModule.AISense_Sight")
      (Pawn|Components|CharacterMovement|SetMovementMode (Actor|GetComponentbyClass _owner "/Script/Engine.CharacterMovementComponent") "MOVE_Walking" 0)
      (Collision|SetActorEnableCollision _owner true)
      (bind _ownerhud (Variables|Widget|GetOwnerHUD)
        (:then
          (Default|RemoveExtraInteraction _ownerhud "Sortir" "None"))
        (:else)))))

(event EventBeginPlay
  ;[0.15 0.15 0.15 0.5] Begin, initialises, the interaction widgets mostly.
  (Variables|Default|SetOwnerAiStimulis (Actor|GetComponentbyClass (Components|GetOwner) "/Script/AIModule.AIPerceptionStimuliSourceComponent"))
  (bind _output_get (Variables|Default|SetOwner (Components|GetOwner)))
  (Utilities|FlowControl|Delay 0.1)
  (bind _asbp_player_character (Utilities|Casting|CastToBP_PlayerCharacter _output_get))
  (Variables|Widget|SetOwnerHUD (Variables|/Game/FirstPerson/Blueprints/BP_PlayerCharacter.BP_PlayerCharacter_C|GetHUD _asbp_player_character))
  (EventDispatchers|BindEventtoOnInteractionClicked (Variables|/Script/TheHeist.InteractionWidgetActor|GetMyWidget (Variables|Default|GetInteractionChoiceWidgetInstance)) (delegate Custom|OnInteractionBind))
  (bind _asw_interaction_signal_widget_actor (Utilities|Casting|CastToW_InteractionSignalWidgetActor (Variables|Default|GetInteractionSignalWidgetInstance)))
  (Default|Initilialise _asw_interaction_signal_widget_actor self)
  ;[0.15 0.15 0.15 0.5] SpehereCollider setup for the owner. Will control the activation of the interaction checking (to avoid ticking)
  (bind _returnvalue (Game|AddComponentbyClass (Variables|Default|GetOwner) "/Script/Engine.SphereComponent" false))
  (bind _output_get_2 (Variables|Default|SetInteractionSphereCollider _returnvalue))
  (Transformation|AttachComponentToComponent _output_get_2 (Variables|/Script/Engine.Actor|GetRootComponent (Variables|Default|GetOwner)) "" "KeepRelative" "KeepRelative" "KeepRelative" true)
  (Components|Sphere|SetSphereRadius (Variables|Default|GetInteractionSphereCollider) (Variables|Overlapping|GetInteractionRange) true)
  ;[0.15 0.15 0.15 0.5] Manage the overlap event. If minimum a single overlapped, starts the interaction checking
  (Collision|BindEventtoOnComponentBeginOverlap (Variables|Default|GetInteractionSphereCollider) (delegate Custom|OnColliderOverlapped))
  ;[0.15 0.15 0.15 0.5] Manage the end overlap event. If not a single overlapped left, stops the interaction checking
  (Collision|BindEventtoOnComponentEndOverlap (Variables|Default|GetInteractionSphereCollider) (delegate Custom|OnColliderEndOverlapped)))

(event EventTick
  (params (DeltaSeconds :type Float%20%28single-precision%29))
  (bind _returnvalue (Game|GetPlayerCameraManager 0))
  (bind _returnvalue_2 (Camera|GetCameraLocation _returnvalue))
  ;[1 1 1] Checks for an interaction to communicate with. Will display the interaction button widget
  (bind _outhit (Collision|LineTraceByChannel _returnvalue_2 (+ _returnvalue_2 (* (Math|Vector|GetForwardVector (Camera|GetCameraRotation (Game|GetPlayerCameraManager 0))) (Variables|LineTrace|GetRaycastDistance))) "TraceTypeQuery1" false 0 "ForOneFrame"))
  (if (.bblockinghit _outhit)
    (Utilities|IsValid (.hitactor _outhit)
      (:Is%20Valid
        (Utilities|IsValid (Actor|GetComponentbyClass (.hitactor _outhit) "/Script/TheHeist.InteractableComponent")
          (:Is%20Valid
            (Variables|LineTrace|SetInteractableObject (.hitactor _outhit))
            (for _array_element (Variables|/Script/TheHeist.InteractableComponent|GetAllComponentInteractablePlayer (Actor|GetComponentbyClass (.hitactor _outhit) "/Script/TheHeist.InteractableComponent"))
              (if (== (.hitcomponent _outhit) _array_element)
                (Variables|LineTrace|SetHitComponent (.hitcomponent _outhit))
                (Transformation|SetActorLocation (Variables|Default|GetInteractionSignalWidgetInstance) (.Origin (Collision|GetComponentBounds (.hitcomponent _outhit))) false false)
                (if (not (Variables|Widget|Getb_InteractionButtonWidgetActivated))
                  (CallFunction|ShouldActivateButtonInteractionWidget true)))))
          (:Is%20Not%20Valid
            (if (Variables|Widget|Getb_InteractionButtonWidgetActivated)
              (CallFunction|ShouldActivateButtonInteractionWidget false))))))
    (elif (Variables|Widget|Getb_InteractionButtonWidgetActivated)
      (CallFunction|ShouldActivateButtonInteractionWidget false))))

(event Input|MouseEvents|LeftMouseButton
  (params (Key :type Key%20Structure :default "None"))
  (bind _owner (Variables|Default|GetOwner))
  (bind _returnvalue (Actor|GetComponentbyClass _owner "/Script/UMG.WidgetInteractionComponent"))
  ;[0.15 0.15 0.15 0.5] Widget interaction
  (:Pressed
    (Class|WidgetInteractionComponent|PressPointerKey _returnvalue "LeftMouseButton"))
  (:Released
    (Class|WidgetInteractionComponent|ReleasePointerKey _returnvalue "LeftMouseButton")))

(event Input|KeyboardEvents|W
  (params (Key :type Key%20Structure :default "None"))
  ;[0.15 0.15 0.15 0.5] On interaction button pressed, trigger the interaction
  (:Pressed
    (if (Variables|Default|Getb_isHidden)
      (Class|InteractableComponent|InteractwithSpecificInteraction (Actor|GetComponentbyClass (Variables|Default|GetCurrentInteractionObjectClicked) "/Script/TheHeist.InteractableComponent") 0 0 (Variables|Default|GetOwner) "Default" (Variables|Default|GetInteraction%20Type)))))