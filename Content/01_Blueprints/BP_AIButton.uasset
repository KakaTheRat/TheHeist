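; BP_AIButton is an interactable button that toggles the AI of every BP_Guard in the level on and off.
; Each Interact flips the AiStopped flag, then gathers all guards and stops or restarts the brain component logic on their AI controllers.
; After a short delay it calls EndOfInteraction on the passed Data to finish the interaction.
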(event EventBeginPlay)

(event Collision|EventActorBeginOverlap
  (params (OtherActor :type Actor%20Object%20Reference)))

(event EventTick
  (params (DeltaSeconds :type Float%20%28single-precision%29)))

(event EventInteract
  (params (HitComponent :type Scene%20Component%20Object%20Reference) (InteractingActor :type Actor%20Object%20Reference) (Context :type EInteractionContext%20Enum :default "Default") (Data :type Interaction%20Data%20Object%20Reference))
  (Variables|Default|SetbAiStopped (not (Variables|Default|GetbAiStopped)))
  (if (Variables|Default|GetbAiStopped)
    (bind _outactors (Actor|GetAllActorsOfClass "/Game/01_Blueprints/Actors/Guard/BP_Guard.BP_Guard_C"))
    (for _array_element _outactors
      (AI|Logic|StopLogic (Variables|/Script/AIModule.AIController|GetBrainComponent (AI|GetAIController _array_element)) ""))
    (Utilities|FlowControl|Delay 0.2)
    (Class|InteractionData|EndOfInteraction Data)
    (else
      (bind _outactors_2 (Actor|GetAllActorsOfClass "/Game/01_Blueprints/Actors/Guard/BP_Guard.BP_Guard_C"))
      (for _array_element_2 _outactors_2
        (Class|BrainComponent|RestartLogic (Variables|/Script/AIModule.AIController|GetBrainComponent (AI|GetAIController _array_element_2))))
      (Utilities|FlowControl|Delay 0.2)
      (Class|InteractionData|EndOfInteraction Data))))

(fn ConstructionScript)