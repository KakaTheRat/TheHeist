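; Base projectile for abilities that damages the actor it hits, plays a sound, spawns a small explosion and destroys itself.
; On BeginPlay its sphere and mesh ignore the instigator, and an empty Launch event runs if AutoLaunch is set.
; Init stores radius, damage, hit VFX and target, then calls Launch.
; Init's sound argument is never stored, and Hit uses NS_SmallExplosion instead of the stored HitVFX.
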(event Custom|Launch)

(event EventBeginPlay
  (Collision|IgnoreActorwhenMoving (Variables|Default|GetSphere) (Game|GetInstigator) true)
  (Collision|IgnoreActorwhenMoving (Variables|Default|GetMesh) (Game|GetInstigator) true)
  (if (Variables|Default|GetAutoLaunch)
    (CallFunction|Launch)))

(event Collision|EventActorBeginOverlap
  (params (OtherActor :type Actor%20Object%20Reference)))

(event EventTick
  (params (DeltaSeconds :type Float%20%28single-precision%29)))

(event Collision|EventHit
  (params (MyComp :type Primitive%20Component%20Object%20Reference) (Other :type Actor%20Object%20Reference) (OtherComp :type Primitive%20Component%20Object%20Reference) (bSelfMoved :type Boolean) (HitLocation :type Vector :default "0, 0, 0") (HitNormal :type Vector :default "0, 0, 0") (NormalImpulse :type Vector :default "0, 0, 0") (Hit :type Hit%20Result%20Structure%20%28by%20ref%29))
  ;[0.1094 0.1094 0.1094] Damage first enemy hit and destroy elf
  (Audio|PlaySoundatLocation (Variables|Default|GetSound) HitLocation "0, 0, 0" 0.2 1.0 0.0 0 0 0 0)
  (Game|Damage|ApplyDamage (.HitActor (Collision|BreakHitResult Hit)) (Variables|Default|GetDamage) (Game|GetInstigatorController (Variables|Actor|GetInstigator)) self)
  (Niagara|SpawnSystematLocation "/Game/2-Art/VFX/Niagara/NS_SmallExplosion.NS_SmallExplosion" HitLocation)
  (Actor|DestroyActor))

(fn ConstructionScript)

(fn Init
  (params (Radius :type Float%20%28double-precision%29) (Damage :type Float%20%28double-precision%29) (DamageVFX :type Particle%20System%20Object%20Reference) (SoundVFX :type Sound%20Cue%20Object%20Reference) (Target :type Vector))
  (Variables|Default|SetRadius Radius)
  (Variables|Default|SetDamage Damage)
  (Variables|Default|SetHit_VFX DamageVFX)
  (Variables|Default|SetTarget Target)
  (CallFunction|Launch))