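; BP_Bomb is a projectile bomb ability that deals area damage when its movement stops.
; Stopping starts a timeline that pulses mesh scale with an accelerating sine as a fuse.
; It then spawns explosion effects and sphere-traces for damage via DamageEnemiesOnce.
; Instigator and causer come from the first BP_Base_Enemy found; damage and self-destruction require its valid controller, and the bounce count triggers nothing.
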(event OnProjectileBounce(ProjectileMovement)
  (params (ImpactResult :type Hit%20Result%20Structure%20%28by%20ref%29) (ImpactVelocity :type Vector%20%28by%20ref%29 :default "0, 0, 0"))
  (Math|Integer|IncrementInt (Variables|Default|GetCurrentBounces)
    (:%20%20
      (if (>= (Variables|Default|GetCurrentBounces) (Variables|Default|GetMaxBounces))
        _))))

(event OnProjectileStop(ProjectileMovement)
  (params (ImpactResult :type Hit%20Result%20Structure%20%28by%20ref%29))
  (CallFunction|Explode))

(event Custom|Explode
  (bind _returnvalue (Transformation|GetActorLocation))
  (bind _mesh (Variables|Character|GetMesh))
  (bind _returnvalue_2 (Transformation|GetWorldLocation _mesh))
  (bind _newtrack_0 (Timeline|Timeline Play)
    (:Update
      (Transformation|SetRelativeScale3D (Variables|Character|GetMesh) (* (Math|Float|MapRangeClamped (* _newtrack_0 (+ (/ (Math|Trig|Sin(Radians) (* (* _newtrack_0 _newtrack_0) 6e+01)) 2.0) 0.5)) 0.0 1.0 1.0 2.0) "3.000000,3.000000,3.000000")))
    (:Finished
      (Niagara|SpawnSystematLocation "/Game/2-Art/VFX/Niagara/NS_BombExplosion.NS_BombExplosion" _returnvalue_2)
      (Audio|PlaySoundatLocation "/Game/2-Art/SFX/Audio/SurvivorRoguelike/Sounds/Abilities/Cue_Explosion.Cue_Explosion" _returnvalue_2 "0, 0, 0" 1.0 1.0 0.0 0 0 0 0)
      (bind _outhits (Collision|MultiSphereTraceForObjects _returnvalue _returnvalue 6e+02 (Utilities|Array|MakeArray "ObjectTypeQuery3" "ObjectTypeQuery10" "ObjectTypeQuery7") false 0 "None"))
      (bind _returnvalue_3 (Actor|GetActorOfClass "/Game/SurvivorsTemplate/Blueprints/Enemies/BP_Base_Enemy.BP_Base_Enemy_C"))
      (Utilities|IsValid (Game|GetInstigatorController (Game|GetInstigator _returnvalue_3))
        (:Is%20Valid
          (CallFunction|DamageEnemiesOnce _outhits 3e+01 (Game|GetInstigatorController (Game|GetInstigator _returnvalue_3)) _returnvalue_3 (Game|GetInstigator _returnvalue_3))
          (Actor|DestroyActor))))))

(event EventBeginPlay
  (|CallParentFunction))

(event Collision|EventActorBeginOverlap
  (params (OtherActor :type Actor%20Object%20Reference)))

(event EventTick
  (params (DeltaSeconds :type Float%20%28single-precision%29)))

(fn ConstructionScript
  (|CallParentFunction))