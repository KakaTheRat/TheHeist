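; Enemy-empowering spell ability that buffs up to MaxBuffed other enemies around its owner.
; ExecuteAbility starts a looping timer, presumably driving RefreshBuffs, which sphere-overlaps for enemies, debuffs those out of range and randomly fills free slots.
; Buffs multiply scale, walk speed and current health; debuffs divide them, though the health factors are not exact inverses.
; Random picks are re-evaluated per call, so tracked and buffed actors can differ.
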(event EventBeginPlay
  (|CallParentFunction) ; This node is disabled and will not be called.\nDrag off pins to build functionality.
)

(event Collision|EventActorBeginOverlap
  (params (OtherActor :type Actor%20Object%20Reference))
  (|CallParentFunction OtherActor) ; This node is disabled and will not be called.\nDrag off pins to build functionality.
)

(event EventTick
  (params (DeltaSeconds :type Float%20%28single-precision%29))
  (|CallParentFunction DeltaSeconds) ; This node is disabled and will not be called.\nDrag off pins to build functionality.
)

(event EventExecuteAbility
  (Utilities|FlowControl|Delay 0.2)
  (Utilities|Time|SetTimerbyEvent (EventDispatchers|CreateEvent :!event RefreshBuffs) 3.0 true))

(fn ConstructionScript
  (|CallParentFunction))

(fn RefreshBuffs
  (bind _outactors (Collision|SphereOverlapActors (Transformation|GetActorLocation (Components|GetOwner)) 1e+04 (Utilities|Array|MakeArray "ObjectTypeQuery7") "/Game/SurvivorsTemplate/Blueprints/Enemies/BP_Base_Enemy.BP_Base_Enemy_C" (Utilities|Array|MakeArray (Components|GetOwner))))
  (bind _output_get (LocalVariables|SetCurrentOverlappedActors _outactors))
  (for _array_element (Variables|Default|GetBuffedLastTimer)
    (if (Utilities|Array|ContainsItem _output_get _array_element)
      (Utilities|Array|RemoveItem (LocalVariables|GetCurrentOverlappedActors) _array_element)
      (else
        (CallFunction|Debuff _array_element)
        (Utilities|Array|RemoveItem (Variables|Default|GetBuffedLastTimer) _array_element))))
  (Utilities|FlowControl|ForLoopwithBreak 0 (- (Variables|Default|GetMaxBuffed) (Utilities|Array|Length (Variables|Default|GetBuffedLastTimer))) :!label _label
    (:LoopBody
      (Utilities|Array|AddUnique (Variables|Default|GetBuffedLastTimer) (.OutItem (Utilities|Array|Random (LocalVariables|GetCurrentOverlappedActors))))
      (CallFunction|Buff (.OutItem (Utilities|Array|Random (LocalVariables|GetCurrentOverlappedActors))))
      (Utilities|Array|RemoveItem (LocalVariables|GetCurrentOverlappedActors) (.OutItem (Utilities|Array|Random (LocalVariables|GetCurrentOverlappedActors))))
      (if (Utilities|Array|IsEmpty (LocalVariables|GetCurrentOverlappedActors))
        (goto _label Break)))))

(fn Debuff
  (params (ActorToDebuff :type Actor%20Object%20Reference))
  (CallFunction|Buff/DebuffCalculation ActorToDebuff false))

(fn Buff
  (params (ActorToBuff :type Actor%20Object%20Reference))
  (CallFunction|Buff/DebuffCalculation ActorToBuff true))

(fn Buff/DebuffCalculation
  (params (TargetActor :type Actor%20Object%20Reference) (Buff :type Boolean))
  (bind _returnvalue (Actor|GetComponentbyClass TargetActor "/Script/Engine.CharacterMovementComponent"))
  (bind _returnvalue_2 (Actor|GetComponentbyClass TargetActor "/Game/SurvivorsTemplate/Blueprints/Components/BPC_Health.BPC_Health_C"))
  (bind _returnvalue_3 (Actor|GetComponentbyClass TargetActor "/Script/Engine.CharacterMovementComponent"))
  (bind _returnvalue_4 (Actor|GetComponentbyClass TargetActor "/Game/SurvivorsTemplate/Blueprints/Components/BPC_Health.BPC_Health_C"))
  (LocalVariables|GetTargetActor
    (:then
      (if Buff
        (Transformation|SetActorScale3D TargetActor (* (Transformation|GetActorScale3D TargetActor) 2.0))
        (Variables|/Script/Engine.CharacterMovementComponent|SetMaxWalkSpeed _returnvalue_3 (* (Class|MovementComponent|GetMaxSpeed _returnvalue_3) 2.0))
        (Variables|/Game/SurvivorsTemplate/Blueprints/Components/BPC_Health.BPC_Health_C|SetCurrentHealth _returnvalue_4 (* (Variables|/Game/SurvivorsTemplate/Blueprints/Components/BPC_Health.BPC_Health_C|GetCurrentHealth _returnvalue_4) 1e+05))
        (else
          (Transformation|SetActorScale3D TargetActor (* (Transformation|GetActorScale3D TargetActor) 0.5))
          (Variables|/Script/Engine.CharacterMovementComponent|SetMaxWalkSpeed _returnvalue (* (Class|MovementComponent|GetMaxSpeed _returnvalue) 0.5))
          (Variables|/Game/SurvivorsTemplate/Blueprints/Components/BPC_Health.BPC_Health_C|SetCurrentHealth _returnvalue_2 (* (Variables|/Game/SurvivorsTemplate/Blueprints/Components/BPC_Health.BPC_Health_C|GetCurrentHealth _returnvalue_2) 1e-06)))))
    (:else)))