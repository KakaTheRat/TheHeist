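; Spell ability that teleports its caster away, to a point picked by the EQS_FindFurthestPoint query.
; ExecuteAbility runs the single-result query with the caster as querier and binds the TP event to its completion.
; On success, TP moves the caster without sweep and spawns Niagara smoke at both origin and destination.
; The ability ends whether or not a location is found; SpawnEnnemies is an empty stub.
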(event Custom|TP
  (params (QueryInstance :type Env%20Query%20Instance%20Blueprint%20Wrapper%20Object%20Reference) (QueryStatus :type EEnvQueryStatus%20Enum :default "Processing"))
  (bind _caster (Variables|Default|GetCaster))
  (bind _caster_2 (Variables|Default|GetCaster))
  (bind (_resultlocations _returnvalue) (AI|EQS|GetQueryResultsasLocations QueryInstance))
  (if _returnvalue
    (Niagara|SpawnSystematLocation _caster "/Game/Fantastic_Dungeon_Pack/effects/PS_FX_smoke_dungeon_Niagara1.PS_FX_smoke_dungeon_Niagara1" (Transformation|GetActorLocation _caster))
    (Transformation|SetActorLocation _caster_2 (Utilities|Array|Get(acopy) _resultlocations) false false)
    (Niagara|SpawnSystematLocation _caster_2 "/Game/Fantastic_Dungeon_Pack/effects/PS_FX_smoke_dungeon_Niagara1.PS_FX_smoke_dungeon_Niagara1" (Utilities|Array|Get(acopy) _resultlocations))
    (CallFunction|EndAbility)
    (else
      (CallFunction|EndAbility))))

(event EventExecuteAbility
  (bind _returnvalue (AI|EQS|RunEQSQuery (Variables|Default|GetCaster) "/Game/SurvivorsTemplate/Blueprints/AI/EQS_FindFurthestPoint.EQS_FindFurthestPoint" (Variables|Default|GetCaster) "SingleResult"))
  (EventDispatchers|BindEventtoOnQueryFinishedEvent _returnvalue (EventDispatchers|CreateEvent :!event Custom|TP)))

(fn SpawnEnnemies)