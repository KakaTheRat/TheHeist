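; Lightning Strike spell ability that sets off a short burst of repeated lightning explosions at the player's position.
; On execute, a looping timer asks the ability component to spawn a BP_LightningExplosion just below player pawn 0's current location, so strikes follow the player.
; Each explosion is initialized with fixed radius, damage, VFX and sound.
; After seven strikes it clears the timer and ends the ability.
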(event Custom|CustomEvent
  (bind _caster (Variables|Default|GetCaster))
  (if (< (Variables|Default|GetIterations) 7)
    (bind _spawnedactor (Default|SpawnRequest (Variables|Default|GetAbilityComp) "/Game/SurvivorsTemplate/Blueprints/Abilities/BP_LightningExplosion.BP_LightningExplosion_C" (Math|Conversions|ToTransform(Vector) (+ (Transformation|GetActorLocation (Game|Player|GetPlayerPawn _caster)) "0.000000,0.000000,-100.000000")) (Variables|/Script/Engine.Actor|GetInstigator (Variables|Default|GetCaster))))
    (bind _asbp_lightning_explosion (Utilities|Casting|CastToBP_LightningExplosion _spawnedactor))
    (Default|Init _asbp_lightning_explosion 1e+02 5.0 "/Game/SurvivorsTemplate/Demo/Effects/FX_Mobile/Lightning/P_LineToPoint_Blast_Lightning_00.P_LineToPoint_Blast_Lightning_00" "/Game/2-Art/SFX/Audio/SurvivorRoguelike/Sounds/Abilities/Cue_lightning.Cue_lightning")
    (Math|Integer|IncrementInt (Variables|Default|GetIterations))
    (else
      (Utilities|Time|ClearandInvalidateTimerbyHandle _caster (Variables|Default|GetTimerHandle))
      (CallFunction|EndAbility))))

(event EventExecuteAbility
  (bind _returnvalue (Utilities|Time|SetTimerbyEvent (delegate Custom|CustomEvent) 0.3 true))
  (Variables|Default|SetTimerHandle _returnvalue))