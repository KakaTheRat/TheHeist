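; BP_AbilityShoot is a spell ability that makes its caster fire projectiles continuously.
; ExecuteAbility starts a short looping timer that calls Shoot, with no stop logic in this graph.
; Each shot requests a BP_Fireball_Projectile through AbilityComp just ahead of the caster along the control yaw, then initializes its radius, damage and ice impact VFX.
; It then sets the caster's rotation to the control rotation with a fixed yaw offset.
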(event Custom|Shoot
  (bind _caster (Variables|Default|GetCaster))
  (bind _caster_2 (Variables|Default|GetCaster))
  (bind _instigator (Variables|/Script/Engine.Actor|GetInstigator _caster_2))
  (bind _returnvalue (Pawn|GetControlRotation _instigator :!class /Script/Engine.Pawn))
  (bind _spawnedactor (Default|SpawnRequest (Variables|Default|GetAbilityComp) "/Game/SurvivorsTemplate/Blueprints/Abilities/BP_Fireball_Projectile.BP_Fireball_Projectile_C" (Math|Transform|MakeTransform (+ (Transformation|GetActorLocation _caster) (Transformation|GetActorForwardVector _caster)) (Math|Rotator|MakeRotator 0.0 0.0 (.Yaw (Math|Rotator|BreakRotator (Pawn|GetControlRotation (Variables|/Script/Engine.Actor|GetInstigator (Variables|Default|GetCaster)) :!class /Script/Engine.Pawn)))) "1.000000,1.000000,1.000000") (Variables|/Script/Engine.Actor|GetInstigator (Variables|Default|GetCaster))))
  (bind _asbp_fireball_projectile (Utilities|Casting|CastToBP_Fireball_Projectile _spawnedactor))
  (Default|Init _asbp_fireball_projectile 1e+01 1e+01 "/Game/SurvivorsTemplate/Demo/Effects/FX_Combat_Ice/Impact/P_Impact_Ice.P_Impact_Ice" 0 "0, 0, 0")
  (Transformation|SetActorRotation (Variables|Default|GetCaster) (Math|Rotator|MakeRotator (.roll _returnvalue) (.pitch _returnvalue) (+ (.yaw _returnvalue) 15.0))))

(event EventExecuteAbility
  (Utilities|Time|SetTimerbyEvent (delegate Custom|Shoot) 0.1 true))