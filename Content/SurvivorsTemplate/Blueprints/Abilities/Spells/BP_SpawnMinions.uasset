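; Spell ability that spawns BP_Base_Enemy minions, one per successful execution, while its Spawned list holds fewer than ten.
; ExecuteAbility runs an EQS spawn-point query around the player pawn and binds an event to its completion.
; SpawnPositionFound picks a random result, spawns the enemy slightly raised with BP_Soul as its soul, records it and ends the ability.
; The SpawnEnnemies function it calls is empty.
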(event Custom|SpawnPositionFound
  (params (QueryInstance :type Env%20Query%20Instance%20Blueprint%20Wrapper%20Object%20Reference) (QueryStatus :type EEnvQueryStatus%20Enum :default "Processing"))
  (bind (_resultlocations _returnvalue) (AI|EQS|GetQueryResultsasLocations QueryInstance))
  (if _returnvalue
    (bind _returnvalue_2 (Game|SpawnActorfromClass "/Game/SurvivorsTemplate/Blueprints/Enemies/BP_Base_Enemy.BP_Base_Enemy_C" (Math|Transform|MakeTransform (+ (.OutItem (Utilities|Array|Random _resultlocations)) "0,0,25.000000") "0, 0, 0" "1.000000,1.000000,1.000000") "AdjustIfPossibleButAlwaysSpawn" "SelectDefaultAtRuntime" 0 0 1e+01 15.0 "/Game/SurvivorsTemplate/Blueprints/GameplayActors/BP_Soul.BP_Soul_C" false false 0 1 0))
    (Utilities|Array|AddUnique (Variables|Default|GetSpawned) _returnvalue_2)
    (CallFunction|SpawnEnnemies)
    (CallFunction|EndAbility)))

(event EventBeginPlay
  (|CallParentFunction) ; This node is disabled and will not be called.\nDrag off pins to build functionality.
)

(event Collision|EventActorBeginOverlap
  (params (OtherActor :type Actor%20Object%20Reference))
  (|CallParentFunction OtherActor) ; This node is disabled and will not be called.\nDrag off pins to build functionality.
)

(event EventTick
  (params (DeltaSeconds :type Float%20%28single-precision%29))
  (|CallParentFunction DeltaSeconds) ; This node is disabled and will not be called.\nDrag off pins to build functionality.
)

(event EventExecuteAbility
  (if (< (Utilities|Array|Length (Variables|Default|GetSpawned)) 10)
    (bind _returnvalue (AI|EQS|RunEQSQuery "/Game/SurvivorsTemplate/Blueprints/AI/EQS_FindSpawnPoint_Modified.EQS_FindSpawnPoint_Modified" (Game|Player|GetPlayerPawn 0) "AllMatching"))
    (EventDispatchers|BindEventtoOnQueryFinishedEvent _returnvalue (EventDispatchers|CreateEvent :!event Custom|SpawnPositionFound))))

(fn ConstructionScript
  (|CallParentFunction))

(fn SpawnEnnemies)