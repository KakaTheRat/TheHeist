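; Bomb-throw ability that launches a projectile at the position of the first player's pawn.
; Execution plays the caster's throw animation and listens for its animation update events.
; The "Start" event spawns the projectile at a caster socket through the ability component, then initializes it with fixed damage and the pawn's location at that moment.
; When the animation is over, the ability unbinds from those events and ends.
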(event Custom|EventReceived
  (params (EventName :type Name) (IsOver :type Boolean))
  (if IsOver
    (EventDispatchers|UnbindallEventsfromAnimationUpdate (Variables|Default|GetCaster))
    (CallFunction|EndAbility)
    (elif (== EventName "Start")
      (bind _socketlocation (Class|ICharacterManager|GetSocketLocation(Message) (Variables|Default|GetCaster) "NewEnumerator0"))
      (bind _spawnedactor (Default|SpawnRequest (Variables|Default|GetAbilityComp) (Variables|Default|GetClass) _socketlocation (Variables|/Script/Engine.Actor|GetInstigator (Variables|Default|GetCaster))))
      (bind _asbp_base_projectile (Utilities|Casting|CastToBP_Base_Projectile _spawnedactor))
      (Default|Init _asbp_base_projectile 0.0 2e+01 0 0 (Transformation|GetActorLocation (Game|Player|GetPlayerPawn (Variables|Default|GetCaster)))))))

(event EventExecuteAbility
  (Class|ICharacterManager|PlayAnimation(Message) (Variables|Default|GetCaster) "(TagName=\"Ability.Throw\")")
  (EventDispatchers|BindEventtoAnimationUpdate (Variables|Default|GetCaster) (delegate Custom|EventReceived)))