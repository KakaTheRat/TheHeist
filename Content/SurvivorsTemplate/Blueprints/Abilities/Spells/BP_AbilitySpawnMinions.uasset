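; Enemy-spawning minion ability that adds one BP_Base_Enemy near its caster per execution while fewer than ten are tracked.
; An EQS query run from the caster finds candidate points, then its finish callback picks one at random and requests the spawn through the ability component, slightly raised.
; The new enemy is added to the Spawned list before the ability ends; SpawnEnnemies is an empty stub.
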(event Custom|SpawnPositionFound
  (params (QueryInstance :type Env%20Query%20Instance%20Blueprint%20Wrapper%20Object%20Reference) (QueryStatus :type EEnvQueryStatus%20Enum :default "Processing"))
  (bind (_resultlocations _returnvalue) (AI|EQS|GetQueryResultsasLocations QueryInstance))
  (if _returnvalue
    (Class|ICharacterManager|GetContext(Message) (Variables|Default|GetCaster))
    (bind _spawnedactor (Default|SpawnRequest (Variables|Default|GetAbilityComp) "/Game/SurvivorsTemplate/Blueprints/Enemies/BP_Base_Enemy.BP_Base_Enemy_C" (Math|Conversions|ToTransform(Vector) (+ (.OutItem (Utilities|Array|Random _resultlocations)) "0,0,25.000000")) (Variables|/Script/Engine.Actor|GetInstigator (Variables|Default|GetCaster))))
    (bind _asbp_base_enemy (Utilities|Casting|CastToBP_Base_Enemy _spawnedactor))
    (Utilities|Array|AddUnique (Variables|Default|GetSpawned) _asbp_base_enemy)
    (CallFunction|SpawnEnnemies)
    (CallFunction|EndAbility)))

(event EventExecuteAbility
  (if (< (Utilities|Array|Length (Variables|Default|GetSpawned)) 10)
    (bind _returnvalue (AI|EQS|RunEQSQuery (Variables|Default|GetCaster) "/Game/SurvivorsTemplate/Blueprints/AI/EQS_FindSpawnPoint_Modified.EQS_FindSpawnPoint_Modified" (Variables|Default|GetCaster) "AllMatching"))
    (EventDispatchers|BindEventtoOnQueryFinishedEvent _returnvalue (EventDispatchers|CreateEvent :!event Custom|SpawnPositionFound))))

(fn SpawnEnnemies)