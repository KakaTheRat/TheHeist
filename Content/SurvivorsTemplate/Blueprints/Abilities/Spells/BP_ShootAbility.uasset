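; BP_ShootAbility is a spell ability that makes its caster rapidly and repeatedly fire fireball projectiles.
; ExecuteAbility starts a short looping timer on the Shoot event, with no stop logic in this Blueprint.
; Each shot spawns BP_Fireball_Projectile just ahead of the caster at the instigator's control yaw, with an ice impact effect.
; It then sets the caster's rotation to that control rotation with a fixed yaw offset.
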(event Custom|Shoot
  (bind _caster (Variables|Default|GetCaster))
  (bind _caster_2 (Variables|Default|GetCaster))
  (bind _instigator (Variables|/Script/Engine.Actor|GetInstigator _caster_2))
  (bind _returnvalue (Pawn|GetControlRotation _instigator :!class /Script/Engine.Pawn))
  (Game|SpawnActorfromClass "/Game/SurvivorsTemplate/Blueprints/Abilities/BP_Fireball_Projectile.BP_Fireball_Projectile_C" (Math|Transform|MakeTransform (+ (Transformation|GetActorLocation _caster) (Transformation|GetActorForwardVector _caster)) (Math|Rotator|MakeRotator 0.0 0.0 (.Yaw (Math|Rotator|BreakRotator (Pawn|GetControlRotation (Variables|/Script/Engine.Actor|GetInstigator (Variables|Default|GetCaster)) :!class /Script/Engine.Pawn)))) "1.000000,1.000000,1.000000") "Undefined" "MultiplyWithRoot" 0 1e+01 "/Game/SurvivorsTemplate/Demo/Effects/FX_Combat_Ice/Impact/P_Impact_Ice.P_Impact_Ice" 1e+01 (Variables|/Script/Engine.Actor|GetInstigator (Variables|Default|GetCaster)))
  (Transformation|SetActorRotation (Variables|Default|GetCaster) (Math|Rotator|MakeRotator (.roll _returnvalue) (.pitch _returnvalue) (+ (.yaw _returnvalue) 15.0))))

(event EventBeginPlay
  (|CallParentFunction) ; This node is disabled and will not be called.\nDrag off pins to build functionality.
)

(event Collision|EventActorBeginOverlap
  (params (OtherActor :type Actor%20Object%20Reference))
  (|CallParentFunction OtherActor) ; This node is disabled and will not be called.\nDrag off pins to build functionality.
)

(event EventTick
  (params (DeltaSeconds :type Float%20%28single-precision%29))
  (|CallParentFunction DeltaSeconds) ; This node is disabled and will not be called.\nDrag off pins to build functionality.
)

(event EventExecuteAbility
  (Utilities|Time|SetTimerbyEvent (delegate Custom|Shoot) 0.1 true))

(fn ConstructionScript
  (|CallParentFunction))