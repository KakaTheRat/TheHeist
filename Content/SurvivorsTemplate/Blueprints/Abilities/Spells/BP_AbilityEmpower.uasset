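; Enemy-empowering spell ability that, as designed, buffs random nearby enemies around its owner, scaling up their size, speed and current health.
; ExecuteAbility starts a looping timer after a short delay, but RefreshBuffs is empty and its logic is disconnected.
; That unused logic sphere-overlaps enemies, debuffs those out of range and refills up to MaxBuffed.
; Debuff halves size and speed, but its health multiplier does not exactly reverse Buff's.
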(event EventExecuteAbility
  (Utilities|FlowControl|Delay (Variables|Default|GetCaster))
  (Utilities|Time|SetTimerbyEvent (EventDispatchers|CreateEvent :!event RefreshBuffs) 3.0 true))

(fn Debuff
  (params (ActorToDebuff :type Actor%20Object%20Reference))
  (CallFunction|Buff/DebuffCalculation ActorToDebuff false))

(fn Buff
  (params (ActorToBuff :type Actor%20Object%20Reference))
  (CallFunction|Buff/DebuffCalculation ActorToBuff true))

(fn Buff/DebuffCalculation
  (params (TargetActor :type Actor%20Object%20Reference) (Buff :type Boolean))
  (bind _returnvalue (Actor|GetComponentbyClass TargetActor "/Script/Engine.CharacterMovementComponent"))
  (bind _returnvalue_2 (Actor|GetComponentbyClass TargetActor "/Game/SurvivorsTemplate/Blueprints/Components/BPC_Health.BPC_Health_C"))
  (bind _returnvalue_3 (Actor|GetComponentbyClass TargetActor "/Script/Engine.CharacterMovementComponent"))
  (bind _returnvalue_4 (Actor|GetComponentbyClass TargetActor "/Game/SurvivorsTemplate/Blueprints/Components/BPC_Health.BPC_Health_C"))
  (LocalVariables|GetTargetActor
    (:then
      (if Buff
        (Transformation|SetActorScale3D TargetActor (* (Transformation|GetActorScale3D TargetActor) 2.0))
        (Variables|/Script/Engine.CharacterMovementComponent|SetMaxWalkSpeed _returnvalue_3 (* (Class|MovementComponent|GetMaxSpeed _returnvalue_3) 2.0))
        (Variables|/Game/SurvivorsTemplate/Blueprints/Components/BPC_Health.BPC_Health_C|SetCurrentHealth _returnvalue_4 (* (Variables|/Game/SurvivorsTemplate/Blueprints/Components/BPC_Health.BPC_Health_C|GetCurrentHealth _returnvalue_4) 1e+05))
        (else
          (Transformation|SetActorScale3D TargetActor (* (Transformation|GetActorScale3D TargetActor) 0.5))
          (Variables|/Script/Engine.CharacterMovementComponent|SetMaxWalkSpeed _returnvalue (* (Class|MovementComponent|GetMaxSpeed _returnvalue) 0.5))
          (Variables|/Game/SurvivorsTemplate/Blueprints/Components/BPC_Health.BPC_Health_C|SetCurrentHealth _returnvalue_2 (* (Variables|/Game/SurvivorsTemplate/Blueprints/Components/BPC_Health.BPC_Health_C|GetCurrentHealth _returnvalue_2) 1e-06)))))
    (:else)))

(fn RefreshBuffs)