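; Lightning strike spell ability that unleashes a short series of lightning explosions at the player's location.
; On execute, a looping timer spawns BP_LightningExplosion actors just below the player pawn, passing damage, lightning VFX and sound, with the caster's instigator.
; An iteration counter caps the number of strikes, then clears the timer and ends the ability.
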(event Custom|CustomEvent
  (if (< (Variables|Default|GetIterations) 7)
    (Game|SpawnActorfromClass "/Game/SurvivorsTemplate/Blueprints/Abilities/BP_LightningExplosion.BP_LightningExplosion_C" (Math|Transform|MakeTransform (+ (Transformation|GetActorLocation (Game|Player|GetPlayerPawn 0)) "0.000000,0.000000,-100.000000") "0, 0, 0" "1.000000,1.000000,1.000000") "Undefined" "MultiplyWithRoot" 0 1e+02 "None" 5.0 "/Game/SurvivorsTemplate/Demo/Effects/FX_Mobile/Lightning/P_LineToPoint_Blast_Lightning_00.P_LineToPoint_Blast_Lightning_00" "/Game/SurvivorsTemplate/Demo/Sounds/Abilities/Cue_lightning.Cue_lightning" (Game|GetInstigator (Variables|Default|GetCaster)))
    (Math|Integer|IncrementInt (Variables|Default|GetIterations))
    (else
      (Utilities|Time|ClearandInvalidateTimerbyHandle (Variables|Default|GetTimerHandle))
      (CallFunction|EndAbility))))

(event EventBeginPlay
  (|CallParentFunction) ; This node is disabled and will not be called.\nDrag off pins to build functionality.
)

(event Collision|EventActorBeginOverlap
  (params (OtherActor :type Actor%20Object%20Reference))
  (|CallParentFunction OtherActor) ; This node is disabled and will not be called.\nDrag off pins to build functionality.
)

(event EventTick
  (params (DeltaSeconds :type Float%20%28single-precision%29))
  (|CallParentFunction DeltaSeconds) ; This node is disabled and will not be called.\nDrag off pins to build functionality.
)

(event EventExecuteAbility
  (bind _returnvalue (Utilities|Time|SetTimerbyEvent (delegate Custom|CustomEvent) 0.3 true))
  (Variables|Default|SetTimerHandle _returnvalue))

(fn ConstructionScript
  (|CallParentFunction))