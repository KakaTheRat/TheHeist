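; BP_Stone is a stone ability actor that shatters on impact, with a whoosh sound that reacts to its distance from the player.
; It records its starting distance to the player pawn on BeginPlay.
; Each tick it remaps the current distance to whoosh volume and pitch, using the starting distance for the volume range.
; On hit it calls the parent logic, destroys its mesh, stops the whoosh and spawns a random number of rock fragments.
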(event EventBeginPlay
  (|CallParentFunction)
  (Variables|Default|SetStartLocationDistance (Transformation|GetDistanceTo (Game|Player|GetPlayerPawn 0))))

(event Collision|EventActorBeginOverlap
  (params (OtherActor :type Actor%20Object%20Reference))
  (|CallParentFunction OtherActor) ; This node is disabled and will not be called.\nDrag off pins to build functionality.
)

(event EventTick
  (params (DeltaSeconds :type Float%20%28single-precision%29))
  (|CallParentFunction DeltaSeconds) ; This node is disabled and will not be called.\nDrag off pins to build functionality.
)

(event EventHit
  (params (MyComp :type Primitive%20Component%20Object%20Reference) (Other :type Actor%20Object%20Reference) (OtherComp :type Primitive%20Component%20Object%20Reference) (bSelfMoved :type Boolean) (HitLocation :type Vector :default "0, 0, 0") (HitNormal :type Vector :default "0, 0, 0") (NormalImpulse :type Vector :default "0, 0, 0") (Hit :type Hit%20Result%20Structure%20%28by%20ref%29))
  (|CallParentFunction MyComp Other OtherComp bSelfMoved HitLocation HitNormal NormalImpulse Hit)
  (Components|DestroyComponent (Variables|Character|GetMesh))
  (Audio|Components|Audio|Stop (Variables|Default|GetWhoosh))
  (for _index (range 0 (Math|Random|RandomIntegerinRange 5 10))
    (Game|SpawnActorfromClass "/Game/SurvivorsTemplate/Blueprints/Abilities/BP_RockFragments.BP_RockFragments_C" (Math|Conversions|ToTransform(Vector) HitLocation) "Undefined" "MultiplyWithRoot" 0 0)))

(event EventTick
  (params (DeltaSeconds :type Float%20%28single-precision%29))
  (bind _returnvalue (Game|Player|GetPlayerPawn 0))
  (bind _whoosh (Variables|Default|GetWhoosh))
  (bind _returnvalue_2 (Transformation|GetDistanceTo _returnvalue))
  (Audio|Components|Audio|SetVolumeMultiplier _whoosh (Math|Float|MapRangeClamped _returnvalue_2 (Variables|Default|GetStartLocationDistance) 1e+03 0.0 2.0) :!class /Script/Engine.AudioComponent)
  (Audio|Components|Audio|SetPitchMultiplier _whoosh (Math|Float|MapRangeClamped _returnvalue_2 5e+03 1e+02 0.3 3.0)))

(fn ConstructionScript
  (|CallParentFunction))