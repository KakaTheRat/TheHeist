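; BP_Slave is a captive NPC that stays immobile until it is freed.
; Its Save event notifies the game manager's message object with a quest counter event carrying the slave's class and an amount, then sets IsFreed.
; The CanMove override allows movement only when the parent check passes and IsFreed is set.
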(event Custom|Save
  (bind _gamemanager (Class|IGameInstance|GetGameManager(Message) (Game|GetGameInstance)))
  (Default|NotifyEvent _gamemanager "(TagName=\"Quest.Event.Counter.Activated\")" self (Utilities|Struct|MakeST_EventPayload (Utilities|GetClass self) 1))
  (Variables|Default|SetIsFreed true))

(event EventBeginPlay
  (|CallParentFunction))

(event Collision|EventActorBeginOverlap
  (params (OtherActor :type Actor%20Object%20Reference))
  (|CallParentFunction OtherActor) ; This node is disabled and will not be called.\nDrag off pins to build functionality.
)

(event EventTick
  (params (DeltaSeconds :type Float%20%28single-precision%29))
  (|CallParentFunction DeltaSeconds) ; This node is disabled and will not be called.\nDrag off pins to build functionality.
)

(fn ConstructionScript
  (|CallParentFunction))

(fn CanMove?
  (bind _canmove_ (|CallParentFunction))
  (return (and _canmove_ (Variables|Default|GetIsFreed))))