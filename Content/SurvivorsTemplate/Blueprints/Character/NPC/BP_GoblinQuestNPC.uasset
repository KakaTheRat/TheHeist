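; Goblin quest NPC that the player interacts with to start and end the quest defined in its QuestData.
; Game instance quest state drives its prompt (Talk or End) and interactability, allowed before the quest exists or once any objective is done.
; Interact starts the quest through the player pawn's BPC_QuestManager, or sends a tagged completion event to the game manager if it already exists.
; EndQuest is left empty.
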(event EventBeginPlay
  (|CallParentFunction) ; This node is disabled and will not be called.\nDrag off pins to build functionality.
)

(event Collision|EventActorBeginOverlap
  (params (OtherActor :type Actor%20Object%20Reference))
  (|CallParentFunction OtherActor) ; This node is disabled and will not be called.\nDrag off pins to build functionality.
)

(event EventTick
  (params (DeltaSeconds :type Float%20%28single-precision%29))
  (|CallParentFunction DeltaSeconds) ; This node is disabled and will not be called.\nDrag off pins to build functionality.
)

(event EventInteract
  (params (Instigator :type Actor%20Object%20Reference))
  (bind _questfound (Class|IGameInstance|GetQuestState(Message) (Game|GetGameInstance) (Variables|/Game/SurvivorsTemplate/Blueprints/Map/Quest/Data/PDA_Quest_Base.PDA_Quest_Base_C|GetQuestID (Variables|Default|GetQuestData))))
  (if (not _questfound)
    (Default|StartQuest (Actor|GetComponentbyClass (Game|Player|GetPlayerPawn 0) "/Game/SurvivorsTemplate/Blueprints/Components/BPC_QuestManager.BPC_QuestManager_C") (Variables|Default|GetQuestData) self)
    (else
      (bind _gamemanager (Class|IGameInstance|GetGameManager(Message) (Game|GetGameInstance)))
      (Default|NotifyEvent _gamemanager "(TagName=\"Quest.Event.Classic.Completed\")" self))))

(event EventEndQuest
  (params (IsSuccess :type Boolean)))

(fn ConstructionScript
  (|CallParentFunction))

(fn GetInteractionText
  (bind _questfound (Class|IGameInstance|GetQuestState(Message) (Game|GetGameInstance) (Variables|/Game/SurvivorsTemplate/Blueprints/Map/Quest/Data/PDA_Quest_Base.PDA_Quest_Base_C|GetQuestID (Variables|Default|GetQuestData))))
  (if (not _questfound)
    (return "Talk")
    (else
      (return "End"))))

(fn IsInteractable
  (bind (_queststate _questfound) (Class|IGameInstance|GetQuestState(Message) (Game|GetGameInstance) (Variables|/Game/SurvivorsTemplate/Blueprints/Map/Quest/Data/PDA_Quest_Base.PDA_Quest_Base_C|GetQuestID (Variables|Default|GetQuestData))))
  (return (or (> (Utilities|Array|Length (Utilities|Struct|BreakST_QuestState _queststate)) 0) (not _questfound))))