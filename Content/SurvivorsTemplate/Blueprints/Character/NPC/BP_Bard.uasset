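; BP_Bard is an interactable bard NPC that offers a "KILL ?" prompt and drops into a ragdoll when interacted with.
; It always reports itself as interactable.
; Interact enables physics simulation and collision on the mesh and disables capsule collision, while setting IsDead to false despite the kill prompt.
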(event EventBeginPlay
  (|CallParentFunction) ; This node is disabled and will not be called.\nDrag off pins to build functionality.
)

(event Collision|EventActorBeginOverlap
  (params (OtherActor :type Actor%20Object%20Reference)))

(event EventTick
  (params (DeltaSeconds :type Float%20%28single-precision%29)))

(event EventInteract
  (params (Instigator :type Actor%20Object%20Reference))
  (bind _mesh (Variables|Character|GetMesh))
  (Variables|Default|SetIsDead false)
  (Physics|SetSimulatePhysics _mesh true)
  (Collision|SetCollisionEnabled _mesh "QueryAndPhysics")
  (Collision|SetCollisionEnabled (Variables|Default|GetCapsuleComponent) "NoCollision"))

(fn ConstructionScript
  (|CallParentFunction))

(fn IsInteractable
  (return true))

(fn GetInteractionText
  (return "KILL ?"))