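; Blueprint interface for characters in the Survivors template, letting other systems query and command them through interface calls.
; Queries expose alive state, faction, context, the character, ability component and sphere, and socket locations.
; Commands cover healing, killing, passive stat multipliers, pausing, class updates, health widget setup, dissolve effects, attack toggling and tag-based animation playback.
; It declares signatures only, so implementers supply all behavior.
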(fn IsAlive
  (return false))

(fn RestoreHealth
  (params (Amount :type Float%20%28double-precision%29)))

(fn GetAbilitySphere
  (return 0))

(fn GetCharacter
  (return 0))

(fn AdjustPassive
  (params (Stat :type E_PassiveAbilities%20Enum :default "NewEnumerator0") (MultiplicationAmount :type Float%20%28double-precision%29)))

(fn Paused
  (params (Pause :type Boolean) (Override :type Boolean)))

(fn GetAbilityComponent
  (return 0))

(fn UpdateClassName)

(fn UpdateCharacterClass
  (params (Character :type ST%20Available%20Characters%20Structure)))

(fn SetupHealthWidget)

(fn GetFaction
  (return "None"))

(fn Disolve
  (params (Invert :type Boolean)))

(fn Kill)

(fn GetContext
  (return ""))

(fn AttackEnabled
  (params (IsEnabled :type Boolean) (SocketName :type Array%20of%20Names)))

(fn PlayAnimation
  (params (AnimationTag :type Gameplay%20Tag%20Structure)))

(fn GetSocketLocation
  (params (SkeletalPart :type E_SkeletalParts%20Enum :default "NewEnumerator0"))
  (return ""))