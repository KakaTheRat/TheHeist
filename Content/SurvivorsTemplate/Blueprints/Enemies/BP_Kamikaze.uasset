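; Suicide-bomber enemy for the survivors game that explodes shortly after its attack collision is overlapped.
; The overlap triggers the inherited attack, pauses the enemy and grows a warning sphere through a timeline.
; A second timeline flashes the sphere's dynamic material at an accelerating rate using a sine of squared time.
; It then sphere-traces to damage the player, plays explosion sound and Niagara effects, and returns itself to the actor pool.
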(event OnComponentBeginOverlap(AttackCollisionSphere)
  (params (OverlappedComponent :type Primitive%20Component%20Object%20Reference) (OtherActor :type Actor%20Object%20Reference) (OtherComp :type Primitive%20Component%20Object%20Reference) (OtherBodyIndex :type Integer) (bFromSweep :type Boolean) (SweepResult :type Hit%20Result%20Structure%20%28by%20ref%29))
  (bind _returnvalue (Transformation|GetActorLocation))
  (CallFunction|MCEnemyAttack)
  (CallFunction|Pause)
  (Rendering|SetVisibility (Variables|Default|GetSphere) true false)
  (Collision|SetCollisionEnabled (Variables|Default|GetSphere) "QueryOnly")
  (bind _newtrack_0 (Timeline|ScaleSphere Play)
    (:Update
      (Transformation|SetWorldScale3D (Variables|Default|GetSphere) (* _newtrack_0 (Variables|Default|GetNew%20Scale))))
    (:Finished
      (bind _newtrack_0_2 (Timeline|LoopVisibilitySphere PlayFromStart)
        (:Update
          (Rendering|Material|SetVectorParameterValue (Variables|Default|GetMaterial) "Color" (Math|Color|Lerp(LinearColor) "(R=1.000000,G=1.000000,B=1.000000,A=1.000000)" "(R=1.000000,G=0.093059,B=0.027321,A=1.000000)" (+ (* (Math|Trig|Sin(Radians) (* (* _newtrack_0_2 _newtrack_0_2) 4e+01)) 0.5) 0.5)) :!class /Script/Engine.MaterialInstanceDynamic))
        (:Finished
          (Audio|PlaySoundatLocation "/Game/SurvivorsTemplate/Demo/Sounds/Explosion/EndExplosionCut.EndExplosionCut" (Transformation|GetActorLocation) "0, 0, 0" 1.0 1.0 0.0 0 0 0 0)
          (bind _outhit (Collision|SphereTraceForObjects _returnvalue _returnvalue 325.0 (Utilities|Array|MakeArray "ObjectTypeQuery10") false (Utilities|Array|MakeArray self) "None" true "(R=1.000000,G=0.000000,B=0.000000,A=1.000000)" "(R=0.000000,G=1.000000,B=0.000000,A=1.000000)" 1.0))
          (if (.bBlockingHit (Collision|BreakHitResult _outhit))
            (CallFunction|DamagePlayer))
          (Niagara|SpawnSystematLocation "/Game/2-Art/VFX/Niagara/NS_BombExplosion.NS_BombExplosion" (Transformation|GetWorldLocation (Variables|Character|GetMesh)))
          (Class|UltraPoolBlueprintLibrary|UltraPoolReturnbyActor self))))))

(event EventBeginPlay
  (bind _sphere (Variables|Default|GetSphere))
  (|CallParentFunction)
  (Variables|Default|SetAttackAnimation "/Game/2-Art/Animations/Animation/Movements/Explosion1_Montage.Explosion1_Montage")
  (Variables|Default|SetAttackSound "/Game/SurvivorsTemplate/Demo/Sounds/Explosion/ExplosionSoundCut.ExplosionSoundCut")
  (Rendering|SetVisibility (Variables|Default|GetSphere) false false)
  (bind _returnvalue (Rendering|Material|CreateDynamicMaterialInstance _sphere 0 (Rendering|Material|GetMaterial _sphere 0) "None" :!class /Script/Engine.PrimitiveComponent))
  (Variables|Default|SetMaterial _returnvalue))

(event Collision|EventActorBeginOverlap
  (params (OtherActor :type Actor%20Object%20Reference)))

(event EventTick
  (params (DeltaSeconds :type Float%20%28single-precision%29)))

(fn ConstructionScript
  (|CallParentFunction))

(fn DamagetoPlayer)