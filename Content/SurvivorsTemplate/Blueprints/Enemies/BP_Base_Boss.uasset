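; Base boss enemy Blueprint that adds a screen-space health bar and a telegraphed dash attack.
; Each Tick, it asks the enemy abilities component to choose a random ability whenever CanUseAbility returns false.
; Dash spawns an arrow decal below the boss aimed at the player, stretches it through a timeline, then launches the boss along its current forward vector.
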(event Custom|Dash
  (bind _returnvalue (Transformation|GetActorLocation))
  (bind _returnvalue_2 (+ _returnvalue "0.000000,0.000000,-100.000000"))
  (bind _returnvalue_3 (Rendering|Decal|SpawnDecalatLocation "/Game/ArrowIndicator.ArrowIndicator" "100.000000,100.000000,0.000000" _returnvalue_2 (Math|Rotator|MakeRotator 0.0 -9e+01 (.yaw (Math|Rotator|FindLookatRotation _returnvalue_2 (+ (Transformation|GetActorLocation (Game|Player|GetPlayerPawn 0)) "0.000000,0.000000,-100.000000")))) 1e+01))
  (Variables|Default|SetNewVar 0.0)
  (bind _newtrack_0 (Timeline|Timeline PlayFromStart)
    (:Update
      (Transformation|SetWorldScale3D _returnvalue_3 (Math|Vector|MakeVector 1.0 1.0 (+ (* _newtrack_0 1.0) (Variables|Default|GetNewVar))))
      (Variables|Default|SetNewVar (+ (* _newtrack_0 1.0) (Variables|Default|GetNewVar))))
    (:Finished
      (Character|LaunchCharacter (* (Transformation|GetActorForwardVector) 1e+04) true true))))

(event EventBeginPlay
  (|CallParentFunction)
  (Utilities|FlowControl|Delay 0.0)
  (Default|AddScreenSpaceBar (Variables|Default|GetBPC_Health)))

(event Collision|EventActorBeginOverlap
  (params (OtherActor :type Actor%20Object%20Reference)))

(event EventTick
  (params (DeltaSeconds :type Float%20%28single-precision%29))
  (bind _isbusy (Default|CanUseAbility (Variables|Default|GetBPC_EnemyAbilities)))
  (if (not _isbusy)
    (Default|ChoseRandomAbility (Variables|Default|GetBPC_EnemyAbilities))))

(fn ConstructionScript
  (|CallParentFunction))