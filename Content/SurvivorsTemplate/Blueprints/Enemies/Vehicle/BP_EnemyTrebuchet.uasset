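; Enemy trebuchet that keeps the player within a distance band and hurls explosive stones at them.
; While idle, Tick moves it forward or back to stay in range, slowly turns it toward the player, and shoots once aligned.
; Shooting physically simulates the beam with an impulse and attaches a spawned BP_Stone to it.
; A looping timer polls beam pitch to release and launch the stone, then a delayed reset re-enables shooting.
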(event Custom|Reset
  (Utilities|FlowControl|Delay 3.0)
  (Variables|Default|SetIsShooting false))

(event EventBeginPlay)

(event Collision|EventActorBeginOverlap
  (params (OtherActor :type Actor%20Object%20Reference)))

(event EventTick
  (params (DeltaSeconds :type Float%20%28single-precision%29))
  (if (not (Variables|Default|GetIsShooting))
    (Variables|Default|SetReadyToShoot true)
    (if (< (Transformation|GetDistanceTo (Game|Player|GetPlayerPawn 0)) 1e+03)
      (Variables|Default|SetReadyToShoot false)
      (CallFunction|Reposition false)
      (elif (> (Transformation|GetDistanceTo (Game|Player|GetPlayerPawn 0)) 2e+04)
        (Variables|Default|SetReadyToShoot false)
        (CallFunction|Reposition true)))
    (if (> (Math|Vector|DotProduct (Math|Vector|Normalize (- (Transformation|GetActorLocation (Game|Player|GetPlayerPawn 0)) (Transformation|GetActorLocation))) (Transformation|GetActorForwardVector)) 0.9)
      (if (Variables|Default|GetReadyToShoot)
        (CallFunction|Shoot))
      (else
        (Transformation|SetActorRotation (Math|Interpolation|RInterpTo (Transformation|GetActorRotation) (Math|Rotator|FindLookatRotation (Transformation|GetActorLocation) (Transformation|GetActorLocation (Game|Player|GetPlayerPawn 0))) (Utilities|Time|GetWorldDeltaSeconds) 0.3) true)))))

(fn ConstructionScript)

(fn Reposition
  (params (Forward :type Boolean))
  (if Forward
    (LocalVariables|SetSpeed 1e+02)
    (else
      (LocalVariables|SetSpeed -1e+02)))
  (Transformation|AddActorWorldOffset (* (* (Transformation|GetActorForwardVector) (LocalVariables|GetSpeed)) (Utilities|Time|GetWorldDeltaSeconds)) true true))

(fn Shoot
  (bind _skeletalmesh (Variables|Default|GetSkeletalMesh))
  (Variables|Default|SetIsShooting true)
  (Class|SkeletalMeshComponent|SetAllBodiesBelowSimulatePhysics _skeletalmesh (Utilities|Name|MakeLiteralName "SM_Veh_Trebuchet_01_Beam_01") true true)
  (Class|SkeletalMeshComponent|AddImpulsetoAllBodiesBelow _skeletalmesh "0.000000,0.000000,1500.000000" "SM_Veh_Trebuchet_01_Beam_01" true true)
  (bind _returnvalue (Game|SpawnActorfromClass "/Game/SurvivorsTemplate/Blueprints/Abilities/BP_Stone.BP_Stone_C" (Math|Conversions|ToTransform(Vector) (Transformation|GetSocketLocation (Variables|Default|GetSkeletalMesh) "Boulder")) "Undefined" "MultiplyWithRoot" 0 "/Game/SurvivorsTemplate/Demo/Effects/FX_Monsters/FX_Monster_Gruntling/Bomber/P_FireBombExplosion.P_FireBombExplosion" 1e+01 (Transformation|GetActorLocation (Game|Player|GetPlayerPawn 0)) false (Game|GetInstigator)))
  (bind _output_get (Variables|Default|SetCurrentProjectile _returnvalue))
  (Transformation|AttachComponentToComponent _output_get (Variables|Default|GetSkeletalMesh) "Boulder" "SnapToTarget" "SnapToTarget" "SnapToTarget" true)
  (bind _returnvalue_2 (Utilities|Time|SetTimerbyEvent (EventDispatchers|CreateEvent :!event LaunchProjectile) 0.1 true))
  (Variables|Default|SetNewVar _returnvalue_2))

(fn LaunchProjectile
  (if (< (.pitch (.Rotation (Math|Transform|BreakTransform (Transformation|GetBoneTransform (Variables|Default|GetSkeletalMesh) "SM_Veh_Trebuchet_01_Beam_01" "RTS_World")))) -4e+01)
    (Transformation|DetachFromComponent (Variables|/Game/SurvivorsTemplate/Blueprints/Abilities/BP_Base_Projectile.BP_Base_Projectile_C|GetMesh (Variables|Default|GetCurrentProjectile)) "KeepWorld" "KeepWorld" "KeepWorld" true)
    (Default|Launch (Variables|Default|GetCurrentProjectile))
    (Utilities|Time|ClearandInvalidateTimerbyHandle (Variables|Default|GetNewVar))
    (CallFunction|Reset)))