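; BP_Cannon is an enemy cannon that fires missiles at the player while a character is within its trigger sphere.
; A BP_Base_Character entering the sphere starts a looping five-second timer, apparently driving Shoot, and leaving pauses it.
; Shoot spawns an auto-launching BP_MIssile at the chimney mesh's Output socket, targeting player pawn 0.
; Debug strings print on entry and on each shot.
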(event OnComponentBeginOverlap(Sphere)
  (params (OverlappedComponent :type Primitive%20Component%20Object%20Reference) (OtherActor :type Actor%20Object%20Reference) (OtherComp :type Primitive%20Component%20Object%20Reference) (OtherBodyIndex :type Integer) (bFromSweep :type Boolean) (SweepResult :type Hit%20Result%20Structure%20%28by%20ref%29))
  (Utilities|Casting|CastToBP_Base_Character OtherActor)
  (Development|PrintString "Hello")
  (bind _returnvalue (Utilities|Time|SetTimerbyEvent (EventDispatchers|CreateEvent :!event Shoot) 5.0 true))
  (Variables|Default|SetTimerShoot _returnvalue))

(event OnComponentEndOverlap(Sphere)
  (params (OverlappedComponent :type Primitive%20Component%20Object%20Reference) (OtherActor :type Actor%20Object%20Reference) (OtherComp :type Primitive%20Component%20Object%20Reference) (OtherBodyIndex :type Integer))
  (Utilities|Casting|CastToBP_Base_Character OtherActor)
  (Utilities|Time|PauseTimerbyHandle (Variables|Default|GetTimerShoot)))

(event EventBeginPlay)

(event Collision|EventActorBeginOverlap
  (params (OtherActor :type Actor%20Object%20Reference)))

(event EventTick
  (params (DeltaSeconds :type Float%20%28single-precision%29)))

(fn ConstructionScript)

(fn Shoot
  (bind _sm_bld_chimney_02 (Variables|Default|GetSM_Bld_Chimney_02))
  (bind _returnvalue (Transformation|GetSocketTransform _sm_bld_chimney_02 "Output" "RTS_World"))
  (bind (_location _rotation) (Math|Transform|BreakTransform _returnvalue))
  (Game|SpawnActorfromClass "/Game/SurvivorsTemplate/Blueprints/Abilities/BP_MIssile.BP_MIssile_C" (Math|Transform|MakeTransform _location _rotation "1.000000,1.000000,1.000000") "Undefined" "MultiplyWithRoot" 0 1e+02 "0.000000,0.000000,0.000000" true "NewEnumerator2" (Game|Player|GetPlayerPawn 0) (Game|GetInstigator))
  (Development|PrintString "zqdqzd"))