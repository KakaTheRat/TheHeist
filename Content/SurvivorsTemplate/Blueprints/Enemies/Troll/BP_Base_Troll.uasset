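; Base troll enemy for the Survivors template that performs a melee montage attack when its attack range sphere is overlapped.
; The attack halts movement during the montage, restores walking on completion, then repeats after a short delay while a target remains.
; Two hit spheres apply damage on overlap.
; AttackEnabled toggles collision on only one of them, Sphere, leaving Sphere1 untouched.
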(event OnComponentBeginOverlap(AttackCollisionSphere)
  (params (OverlappedComponent :type Primitive%20Component%20Object%20Reference) (OtherActor :type Actor%20Object%20Reference) (OtherComp :type Primitive%20Component%20Object%20Reference) (OtherBodyIndex :type Integer) (bFromSweep :type Boolean) (SweepResult :type Hit%20Result%20Structure%20%28by%20ref%29))
  (Variables|Default|SetHasTarget true)
  (CallFunction|MCEnemyAttack))

(event OnComponentBeginOverlap(Sphere)
  (params (OverlappedComponent :type Primitive%20Component%20Object%20Reference) (OtherActor :type Actor%20Object%20Reference) (OtherComp :type Primitive%20Component%20Object%20Reference) (OtherBodyIndex :type Integer) (bFromSweep :type Boolean) (SweepResult :type Hit%20Result%20Structure%20%28by%20ref%29))
  (Game|Damage|ApplyDamage OtherActor (Variables|Default|GetDamage) (Game|GetInstigatorController (Variables|Default|GetInstigator)) self))

(event OnComponentEndOverlap(AttackCollisionSphere)
  (params (OverlappedComponent :type Primitive%20Component%20Object%20Reference) (OtherActor :type Actor%20Object%20Reference) (OtherComp :type Primitive%20Component%20Object%20Reference) (OtherBodyIndex :type Integer))
  (if (Utilities|Array|IsEmpty (Collision|GetOverlappingActors (Variables|Default|GetAttackCollisionSphere) "/Game/SurvivorsTemplate/Blueprints/Character/BP_Base_Character.BP_Base_Character_C" :!class /Script/Engine.PrimitiveComponent))
    (Variables|Default|SetHasTarget false)))

(event OnComponentBeginOverlap(Sphere1)
  (params (OverlappedComponent :type Primitive%20Component%20Object%20Reference) (OtherActor :type Actor%20Object%20Reference) (OtherComp :type Primitive%20Component%20Object%20Reference) (OtherBodyIndex :type Integer) (bFromSweep :type Boolean) (SweepResult :type Hit%20Result%20Structure%20%28by%20ref%29))
  (Game|Damage|ApplyDamage OtherActor (Variables|Default|GetDamage) (Game|GetInstigatorController (Variables|Default|GetInstigator)) self))

(event EventBeginPlay
  (|CallParentFunction))

(event Collision|EventActorBeginOverlap
  (params (OtherActor :type Actor%20Object%20Reference)))

(event EventTick
  (params (DeltaSeconds :type Float%20%28single-precision%29)))

(event EventAttackEnabled
  (params (IsEnabled :type Boolean) (SocketName :type Array%20of%20Names))
  (if IsEnabled
    (Collision|SetCollisionEnabled (Variables|Default|GetSphere) "QueryAndPhysics")
    (else
      (Collision|SetCollisionEnabled (Variables|Default|GetSphere) "NoCollision"))))

(event EventMCEnemyAttack
  (if (Variables|Default|GetHasTarget)
    (if (not (Variables|Default|GetIsAttacking))
      (Variables|Default|SetIsAttacking true)
      (Pawn|Components|CharacterMovement|DisableMovement (Variables|Character|GetCharacterMovement))
      (Animation|Montage|PlayMontage (Variables|Character|GetMesh) (Variables|Default|GetAttackAnimation)
        (:OnCompleted
          (Pawn|Components|CharacterMovement|SetMovementMode (Variables|Character|GetCharacterMovement) "MOVE_Walking" 0)
          (Utilities|FlowControl|Delay 2.0)
          (Variables|Default|SetIsAttacking false)
          (CallFunction|MCEnemyAttack))))))

(fn ConstructionScript
  (|CallParentFunction))