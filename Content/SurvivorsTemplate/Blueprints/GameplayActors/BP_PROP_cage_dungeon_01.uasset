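; Interactable dungeon cage prop whose door swings open once when the player interacts with it.
; BeginPlay caches the door's initial rotation, and Open plays a timeline that lerps its yaw to a fixed open angle.
; When the timeline finishes, it calls Save on each actor in the Slaves array.
; The "Open" interaction is available only until the cage has been opened.
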(event EventBeginPlay
  (Variables|Default|SetDoorRInitialPosition (Variables|/Script/Engine.SceneComponent|GetRelativeRotation (Variables|Default|GetSM_PROP_cage_door_01_dungeon))))

(event Collision|EventActorBeginOverlap
  (params (OtherActor :type Actor%20Object%20Reference)))

(event EventTick
  (params (DeltaSeconds :type Float%20%28single-precision%29)))

(event EventOpen
  (bind _doorrinitialposition (Variables|Default|GetDoorRInitialPosition))
  (Variables|Default|SetIsOpen true)
  (bind _newtrack_0 (Timeline|Timeline_0 Play)
    (:Update
      (Transformation|SetRelativeRotation (Variables|Default|GetSM_PROP_cage_door_01_dungeon) (Math|Rotator|Lerp(Rotator) (Variables|Default|GetDoorRInitialPosition) (Math|Rotator|MakeRotator (.roll _doorrinitialposition) (.pitch _doorrinitialposition) -8e+01) _newtrack_0 true) false false))
    (:Finished
      (for _array_element (Variables|Default|GetSlaves)
        (Default|Save _array_element)))))

(event EventInteract
  (params (Instigator :type Actor%20Object%20Reference))
  (CallFunction|Open))

(fn ConstructionScript)

(fn GetInteractionText
  (return "Open"))

(fn IsInteractable
  (return (not (Variables|Default|GetIsOpen))))