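; Speed pad that temporarily boosts the walk speed of a BP_Base_Character entering its box.
; Overlap plays a sound, sets the new speed, shakes the camera and runs a timeline driving player FOV, restoring the old speed when it finishes.
; While the player is nearby, Tick uses local-space dot products to show only the Niagara effect on the side facing them, throttled by a reset timer; all four hide out of range.
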(event OnComponentBeginOverlap(Box)
  (params (OverlappedComponent :type Primitive%20Component%20Object%20Reference) (OtherActor :type Actor%20Object%20Reference) (OtherComp :type Primitive%20Component%20Object%20Reference) (OtherBodyIndex :type Integer) (bFromSweep :type Boolean) (SweepResult :type Hit%20Result%20Structure%20%28by%20ref%29))
  (bind _player (Variables|Default|GetPlayer))
  (bind _camera (Variables|/Game/SurvivorsTemplate/Blueprints/Character/BP_Base_Character.BP_Base_Character_C|GetCamera _player))
  (Variables|Default|SetIsBoostActive true)
  (Audio|PlaySoundatLocation "/Game/2-Art/SFX/Audio/SurvivorRoguelike/Sounds/Pad/Cue_SpeedPad.Cue_SpeedPad" (Transformation|GetActorLocation) "0, 0, 0" 1.0 1.0 0.0 0 0 0 0)
  (bind _asbp_base_character (Utilities|Casting|CastToBP_Base_Character OtherActor))
  (Variables|Default|SetOldSpeed (Class|MovementComponent|GetMaxSpeed (Variables|/Script/Engine.Character|GetCharacterMovement _asbp_base_character)))
  (Variables|/Script/Engine.CharacterMovementComponent|SetMaxWalkSpeed (Variables|/Script/Engine.Character|GetCharacterMovement _asbp_base_character) (Variables|Default|GetNewSpeed))
  (Game|Feedback|ClientStartCameraShake (Game|GetPlayerController 0) "/Game/SurvivorsTemplate/Blueprints/Character/BP_CameraShakeSpeedBoost.BP_CameraShakeSpeedBoost_C" 1.0 "CameraLocal" "0, 0, 0")
  (Variables|Default|SetOldFOV (Variables|/Script/Engine.CameraComponent|GetFieldOfView _camera))
  (Camera|SetFieldOfView _camera 105.0)
  (bind _newtrack_0 (Timeline|FloatTrack PlayFromStart)
    (:Update
      (Camera|SetFieldOfView _camera _newtrack_0))
    (:Finished
      (Variables|/Script/Engine.CharacterMovementComponent|SetMaxWalkSpeed (Variables|/Script/Engine.Character|GetCharacterMovement _asbp_base_character) (Variables|Default|GetOldSpeed)))))

(event Custom|ResetBool
  (Utilities|Time|SetTimerbyEvent (delegate Custom|Event_ResetBool) 0.5))

(event Custom|Event_ResetBool
  (Variables|Default|SetTake false))

(event EventBeginPlay
  (bind _asbp_base_character (Utilities|Casting|CastToBP_Base_Character (Game|GetPlayerCharacter 0)))
  (Variables|Default|SetPlayer _asbp_base_character))

(event EventTick
  (params (DeltaSeconds :type Float%20%28single-precision%29))
  (bind _returnvalue (Transformation|GetActorLocation))
  (bind _self self)
  (bind _player (Variables|Default|GetPlayer))
  (bind _returnvalue_2 (Transformation|GetActorTransform _self))
  (bind _returnvalue_3 (Transformation|GetActorLocation _player))
  (bind _returnvalue_4 (- _returnvalue_3 _returnvalue))
  (bind _returnvalue_5 (Math|Transform|InverseTransformDirection _returnvalue_2 _returnvalue_4))
  (bind _returnvalue_6 (Math|Vector|Normalize _returnvalue_5))
  (Variables|Default|SetDelta%20Seconds DeltaSeconds)
  (if (< (Transformation|GetDistanceTo (Variables|Default|GetPlayer)) 1e+03)
    (if (not (Variables|Default|GetTake))
      (Variables|Default|SetFaceA (Math|Vector|DotProduct _returnvalue_6 "1.000000,0.000000,0.000000"))
      (Variables|Default|SetFaceB (Math|Vector|DotProduct _returnvalue_6 "-1.000000,0.000000,0.000000"))
      (Variables|Default|SetFaceC (Math|Vector|DotProduct _returnvalue_6 "0.000000,1.000000,0.000000"))
      (Variables|Default|SetFaceD (Math|Vector|DotProduct _returnvalue_6 "0.000000,-1.000000,0.000000"))
      (Variables|Default|SetMaxValue (Math|Float|Max(Float) (Variables|Default|GetFaceA) (Variables|Default|GetFaceB) (Variables|Default|GetFaceC) (Variables|Default|GetFaceD)))
      (if (== (Variables|Default|GetFaceA) (Variables|Default|GetMaxValue))
        (Rendering|SetVisibility (Variables|Default|GetNiagara_Face_A) true false)
        (Rendering|SetVisibility (Variables|Default|GetNiagara_Face_B) false false)
        (Rendering|SetVisibility (Variables|Default|GetNiagara_Face_C) false false)
        (Rendering|SetVisibility (Variables|Default|GetNiagara_Face_D) false false)
        (Variables|Default|SetTake true :!label _label)
        (CallFunction|ResetBool)
        (elif (== (Variables|Default|GetFaceB) (Variables|Default|GetMaxValue))
          (Rendering|SetVisibility (Variables|Default|GetNiagara_Face_A) false false)
          (Rendering|SetVisibility (Variables|Default|GetNiagara_Face_B) true false)
          (Rendering|SetVisibility (Variables|Default|GetNiagara_Face_C) false false)
          (Rendering|SetVisibility (Variables|Default|GetNiagara_Face_D) false false)
          (goto _label)
          (elif (== (Variables|Default|GetFaceC) (Variables|Default|GetMaxValue))
            (Rendering|SetVisibility (Variables|Default|GetNiagara_Face_A) false false)
            (Rendering|SetVisibility (Variables|Default|GetNiagara_Face_B) false false)
            (Rendering|SetVisibility (Variables|Default|GetNiagara_Face_C) true false)
            (Rendering|SetVisibility (Variables|Default|GetNiagara_Face_D) false false)
            (goto _label)
            (elif (== (Variables|Default|GetFaceD) (Variables|Default|GetMaxValue))
              (Rendering|SetVisibility (Variables|Default|GetNiagara_Face_A) false false)
              (Rendering|SetVisibility (Variables|Default|GetNiagara_Face_B) false false)
              (Rendering|SetVisibility (Variables|Default|GetNiagara_Face_C) false false)
              (Rendering|SetVisibility (Variables|Default|GetNiagara_Face_D) true false)
              (goto _label))))))
    (else
      (Rendering|SetVisibility (Variables|Default|GetNiagara_Face_A) false false)
      (Rendering|SetVisibility (Variables|Default|GetNiagara_Face_B) false false)
      (Rendering|SetVisibility (Variables|Default|GetNiagara_Face_C) false false)
      (Rendering|SetVisibility (Variables|Default|GetNiagara_Face_D) false false))))

(fn ConstructionScript)