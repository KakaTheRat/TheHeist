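; BP_Convoy is an interactable, Player-faction character that serves as the escort target of a quest.
; Interacting starts the quest through the player's BPC_QuestManager, then StartQuest registers it as an enemy target, shows a health bar and runs an EQS query.
; It AI-moves to a random query result, notifying quest completion on arrival or failure on death via game manager messages.
; EndQuest stops movement, removes the bar and unregisters it.
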(event Custom|CustomEvent
  (params (QueryInstance :type Env%20Query%20Instance%20Blueprint%20Wrapper%20Object%20Reference) (QueryStatus :type EEnvQueryStatus%20Enum :default "Processing"))
  (bind _resultlocations (AI|EQS|GetQueryResultsasLocations QueryInstance))
  (AI|AIMoveTo self (.OutItem (Utilities|Array|Random _resultlocations)) 0 5.0 false
    (:OnSuccess
      (bind _gamemanager (Class|IGameInstance|GetGameManager(Message) (Game|GetGameInstance)))
      (Default|NotifyEvent _gamemanager "(TagName=\"Quest.Event.Classic.Completed\")" self))))

(event Custom|CustomEvent_0
  (params (Owner :type Actor%20Object%20Reference))
  (bind _gamemanager (Class|IGameInstance|GetGameManager(Message) (Game|GetGameInstance)))
  (Default|NotifyEvent _gamemanager "(TagName=\"Quest.Event.Classic.Failed\")" self))

(event Game|Damage|EventAnyDamage
  (params (Damage :type Float%20%28single-precision%29) (DamageType :type Damage%20Type%20Object%20Reference) (InstigatedBy :type Controller%20Object%20Reference) (DamageCauser :type Actor%20Object%20Reference))
  (Default|ModifyHealth (Variables|Default|GetBPC_Health) (* Damage -1.0)))

(event EventStartQuest
  (bind _bpc_health (Variables|Default|GetBPC_Health))
  (Variables|Default|SetCanInteract false)
  (bind _returnvalue (AI|EQS|RunEQSQuery "/Game/SurvivorsTemplate/Blueprints/AI/EQS_RandomPointInRange.EQS_RandomPointInRange" self "AllMatching"))
  (EventDispatchers|BindEventtoOnQueryFinishedEvent _returnvalue (delegate Custom|CustomEvent))
  (bind _returnvalue_2 (Actor|GetActorOfClass "/Game/SurvivorsTemplate/Blueprints/System/BP_Game_Manager.BP_Game_Manager_C"))
  (Default|AddEnemiesTarget _returnvalue_2 self)
  (Utilities|FlowControl|Delay 0.2)
  (Variables|Default|SetCurrentHP (Variables|Default|GetBaseHP))
  (Default|AddScreenSpaceBar _bpc_health)
  (EventDispatchers|BindEventtoOnDead _bpc_health (delegate Custom|CustomEvent_0)))

(event EventTick
  (params (DeltaSeconds :type Float%20%28single-precision%29)))

(event EventEndQuest
  (params (IsSuccess :type Boolean))
  (Components|Movement|StopMovementImmediately (Variables|Character|GetCharacterMovement))
  (Default|RemoveScreenSpaceBar (Variables|Default|GetBPC_Health))
  (bind _returnvalue (Actor|GetActorOfClass "/Game/SurvivorsTemplate/Blueprints/System/BP_Game_Manager.BP_Game_Manager_C"))
  (Default|RemoveEnemiesTarget _returnvalue self))

(event EventInteract
  (params (Instigator :type Actor%20Object%20Reference))
  (Default|StartQuest (Actor|GetComponentbyClass (Game|Player|GetPlayerPawn 0) "/Game/SurvivorsTemplate/Blueprints/Components/BPC_QuestManager.BPC_QuestManager_C") (Variables|Default|GetQuestData) self))

(fn ConstructionScript)

(fn GetAbilityComponent
  (return 0))

(fn GetAbilitySphere
  (return 0))

(fn GetCharacter
  (return 0))

(fn GetContext
  (return ""))

(fn GetFaction
  (return "Player"))

(fn GetInteractionText
  (return "Escort"))

(fn GetSocketLocation
  (params (SkeletalPart :type E_SkeletalParts%20Enum :default "NewEnumerator2"))
  (return ""))

(fn IsAlive
  (return true))

(fn IsInteractable
  (return (Variables|Default|GetCanInteract)))