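; BP_Bard_AIController is the AI controller for the Bard NPC, keeping it loosely following the player at a distance.
; It caches the controlled pawn and player pawn 0 on BeginPlay.
; Each Tick, when the Bard is no longer within the follow distance, it issues AIMoveTo toward the player.
; The acceptance radius is smaller than that trigger distance, leaving a band where no new moves are issued.
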(event EventBeginPlay
  (Variables|Default|SetOwnerNpc (Pawn|GetControlledPawn))
  (Variables|Default|SetPlayer (Game|Player|GetPlayerPawn 0)))

(event EventTick
  (params (DeltaSeconds :type Float%20%28single-precision%29))
  (if (not (< (Transformation|GetDistanceTo (Variables|Default|GetOwnerNpc) (Variables|Default|GetPlayer)) 1.5e+03))
    (AI|AIMoveTo (Variables|Default|GetOwnerNpc) "0, 0, 0" (Variables|Default|GetPlayer) 1e+03 false)))

(fn ConstructionScript)