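; AI controller for NPCs that can follow the player in the Survivors template.
; On BeginPlay it runs the BT_NPC behavior tree, then seeds its blackboard from the controlled NPC_Base pawn's Data.
; It writes whether to follow, the following distance, and player pawn 0 as the following target, leaving the follow behavior itself to the tree.
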(event EventBeginPlay
  (AI|RunBehaviorTree "/Game/SurvivorsTemplate/Blueprints/AI/BT_NPC.BT_NPC")
  (CallFunction|Init))

(fn ConstructionScript)

(fn Init
  (bind _asnpc_base (Utilities|Casting|CastToNPC_Base (Pawn|GetControlledPawn)))
  (LocalVariables|SetData (Variables|/Game/SurvivorsTemplate/Blueprints/Character/NPC/NPC_Base.NPC_Base_C|GetData _asnpc_base))
  (AI|Components|Blackboard|SetValueasBool (AI|GetBlackboard 0) (Utilities|Name|MakeLiteralName "FollowPlayer") (Variables|/Game/SurvivorsTemplate/Blueprints/Structs/Character/PDA_NPCDatas.PDA_NPCDatas_C|GetIsFollowingPlayer (Variables|/Game/SurvivorsTemplate/Blueprints/Character/NPC/NPC_Base.NPC_Base_C|GetData _asnpc_base)))
  (AI|Components|Blackboard|SetValueasFloat (AI|GetBlackboard 0) (Utilities|Name|MakeLiteralName "FollowDistance") (Variables|/Game/SurvivorsTemplate/Blueprints/Structs/Character/PDA_NPCDatas.PDA_NPCDatas_C|GetFollowingDistance (LocalVariables|GetData)))
  (AI|Components|Blackboard|SetValueasObject (AI|GetBlackboard 0) (Utilities|Name|MakeLiteralName "FollowingTarget") (Game|Player|GetPlayerPawn 0)))