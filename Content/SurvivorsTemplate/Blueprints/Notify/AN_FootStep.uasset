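; Animation notify that plays a surface-dependent running footstep sound for the mesh's owning actor.
; On each notify it traces a short line on the Visibility channel from the actor's location along its downward axis to read the physical surface type.
; Grass, rock, wood, dirt, concrete and leather each play their own foley sound at the actor's location, not at a foot bone.
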(fn ReceivedNotify
  (params (MeshComp :type Skeletal%20Mesh%20Component%20Object%20Reference) (Animation :type Anim%20Sequence%20Base%20Object%20Reference) (EventReference :type Anim%20Notify%20Event%20Reference%20Structure%20%28by%20ref%29))
  (bind _returnvalue (Components|GetOwner MeshComp))
  (bind _returnvalue_2 (Transformation|GetActorLocation _returnvalue))
  (bind _outhit (Collision|LineTraceByChannel _returnvalue_2 (+ _returnvalue_2 (* (Transformation|GetActorUpVector _returnvalue) -1e+02)) "TraceTypeQuery1" false 0 "None"))
  (switch Utilities|FlowControl|Switch|SwitchonEPhysicalSurface (Collision|GetSurfaceType _outhit)
    (:SurfaceType1
      (Audio|PlaySoundatLocation "/Game/Audio/Foley/MetaSounds/MSS_FoleySound_RunGrass.MSS_FoleySound_RunGrass" _returnvalue_2 "0, 0, 0" 1.0 1.0 0.0 0 0 0 0)
      (return false))
    (:SurfaceType2
      (Audio|PlaySoundatLocation "/Game/Audio/Foley/MetaSounds/MSS_FoleySound_RunRock.MSS_FoleySound_RunRock" _returnvalue_2 "0, 0, 0" 1.0 1.0 0.0 0 0 0 0))
    (:SurfaceType3
      (Audio|PlaySoundatLocation "/Game/Audio/Foley/MetaSounds/MSS_FoleySound_RunWood.MSS_FoleySound_RunWood" _returnvalue_2 "0, 0, 0" 1.0 1.0 0.0 0 0 0 0))
    (:SurfaceType5
      (Audio|PlaySoundatLocation "/Game/Audio/Foley/MetaSounds/MSS_FoleySound_RunDirt.MSS_FoleySound_RunDirt" _returnvalue_2 "0, 0, 0" 1.0 1.0 0.0 0 0 0 0))
    (:SurfaceType6
      (Audio|PlaySoundatLocation "/Game/Audio/Foley/MetaSounds/MSS_FoleySound_RunConcrete.MSS_FoleySound_RunConcrete" _returnvalue_2 "0, 0, 0" 1.0 1.0 0.0 0 0 0 0))
    (:SurfaceType7
      (Audio|PlaySoundatLocation "/Game/Audio/Foley/MetaSounds/MSS_FoleySound_RunLeather.MSS_FoleySound_RunLeather" _returnvalue_2 "0, 0, 0" 1.0 1.0 0.0 0 0 0 0))))