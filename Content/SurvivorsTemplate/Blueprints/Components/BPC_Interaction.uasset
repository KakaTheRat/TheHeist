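; Interaction component that lets the player target and use I_Interaction actors under the camera view.
; A looping timer drives polling, with a camera-forward line trace feeding HandleTracingHit.
; New interactable hits show a text prompt widget and an outline overlay material on meshes, cleared only when the trace hits nothing or on interaction.
; InteractInput sends InteractMessage with the owner to the current target, then clears it.
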(event Custom|InteractInput
  (bind _currentinteractableactor (Variables|Default|GetCurrentInteractableActor)
    (:then
      (Class|IInteraction|Interact(Message) _currentinteractableactor (Components|GetOwner))
      (for _array_element (Actor|GetComponentsByClass (Variables|Default|GetCurrentInteractableActor) "/Script/Engine.StaticMeshComponent")
        (Rendering|Material|SetOverlayMaterial _array_element 0 :!class /Script/Engine.MeshComponent))
      (for _array_element_2 (Actor|GetComponentsByClass (Variables|Default|GetCurrentInteractableActor) "/Script/Engine.SkeletalMeshComponent")
        (Rendering|Material|SetOverlayMaterial _array_element_2 0 :!class /Script/Engine.MeshComponent))
      (Variables|Default|SetCurrentInteractableActor 0)
      (Widget|SetVisibility (Variables|Default|GetInteractionWidgetRef) "Hidden"))
    (:else)))

(event EventBeginPlay
  (bind _returnvalue (UserInterface|CreateWidget (Variables|Default|GetInteractionWidgetClass) (Game|GetPlayerController 0)))
  (bind _output_get (Variables|Default|SetInteractionWidgetRef _returnvalue))
  (UserInterface|Viewport|AddtoViewport _output_get 0)
  (Widget|SetVisibility (Variables|Default|GetInteractionWidgetRef) "Hidden")
  (Utilities|Time|SetTimerbyEvent (EventDispatchers|CreateEvent :!event PerformLineTrace) 0.1 true true))

(fn HandleTracingHit
  (params (Hit :type Boolean) (Actor :type Actor%20Object%20Reference))
  (if Hit
    (if (Utilities|DoesObjectImplementInterface Actor "/Game/SurvivorsTemplate/Blueprints/Interfaces/I_Interaction.I_Interaction_C")
      (bind _isinteractible (Class|IInteraction|IsInteractable(Message) Actor))
      (if _isinteractible
        (if (!= Actor (Variables|Default|GetCurrentInteractableActor))
          (Variables|Default|SetCurrentInteractableActor Actor)
          (bind _interactiontext (Class|IInteraction|GetInteractionText(Message) Actor))
          (Default|SetInformationText (Variables|Default|GetInteractionWidgetRef) _interactiontext)
          (Widget|SetVisibility (Variables|Default|GetInteractionWidgetRef) "Visible")
          (for _array_element (Actor|GetComponentsByClass (Variables|Default|GetCurrentInteractableActor) "/Script/Engine.StaticMeshComponent")
            (Rendering|Material|SetOverlayMaterial _array_element "/Game/2-Art/Textures/MI_Outliner.MI_Outliner" :!class /Script/Engine.MeshComponent))
          (for _array_element_2 (Actor|GetComponentsByClass (Variables|Default|GetCurrentInteractableActor) "/Script/Engine.SkeletalMeshComponent")
            (Rendering|Material|SetOverlayMaterial _array_element_2 "/Game/2-Art/Textures/MI_Outliner.MI_Outliner" :!class /Script/Engine.MeshComponent)))))
    (else
      (Utilities|IsValid (Variables|Default|GetCurrentInteractableActor)
        (:Is%20Valid
          (Widget|SetVisibility (Variables|Default|GetInteractionWidgetRef) "Hidden")
          (Default|SetInformationText (Variables|Default|GetInteractionWidgetRef))
          (for _array_element_3 (Actor|GetComponentsByClass (Variables|Default|GetCurrentInteractableActor) "/Script/Engine.StaticMeshComponent")
            (Rendering|Material|SetOverlayMaterial _array_element_3 0 :!class /Script/Engine.MeshComponent))
          (for _array_element_4 (Actor|GetComponentsByClass (Variables|Default|GetCurrentInteractableActor) "/Script/Engine.SkeletalMeshComponent")
            (Rendering|Material|SetOverlayMaterial _array_element_4 0 :!class /Script/Engine.MeshComponent))
          (Variables|Default|SetCurrentInteractableActor 0))))))

(fn PerformLineTrace
  (bind _returnvalue (Game|GetPlayerCameraManager 0))
  (bind _returnvalue_2 (Camera|GetCameraLocation _returnvalue))
  (bind _outhit (Collision|LineTraceByChannel _returnvalue_2 (+ _returnvalue_2 (* (Transformation|GetActorForwardVector _returnvalue) 1.5e+03)) "TraceTypeQuery2" false (Utilities|Array|MakeArray (Components|GetOwner)) "None"))
  (CallFunction|HandleTracingHit (.bBlockingHit (Collision|BreakHitResult _outhit)) (.HitActor (Collision|BreakHitResult _outhit))))