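; Quest manager component that runs one current quest and hands out its rewards, auto-starting the kill-enemies quest shortly after play begins.
; It constructs the quest object from the class in its data asset, initializes it with the game instance's message manager and registers it with the player controller.
; It listens for the quest's end and, on success only, sends each reward type to the player controller as a reward message.
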(event Custom|StartQuest
  (params (QuestData :type PDA%20Quest%20Base%20Object%20Reference) (QuestActor :type Actor%20Object%20Reference))
  (bind _returnvalue (Game|ConstructObjectfromClass (Variables|/Game/SurvivorsTemplate/Blueprints/Map/Quest/Data/PDA_Quest_Base.PDA_Quest_Base_C|GetQuestClass QuestData) QuestData))
  (bind _gamemanager (Class|IGameInstance|GetGameManager(Message) (Game|GetGameInstance)))
  (Default|Init _returnvalue _gamemanager)
  (bind _output_get (Variables|Default|SetCurrentQuest _returnvalue))
  (Class|IControllerManager|SetupQuest(Message) (Game|GetPlayerController 0) _output_get)
  (Default|StartQuest _output_get QuestActor)
  (EventDispatchers|BindEventtoEndQuest _output_get (delegate Custom|EndQuest)))

(event Custom|OnQuestCompleted
  (params (Quest :type BP%20Quest%20Object%20Reference))
  (for _array_element (Variables|/Game/SurvivorsTemplate/Blueprints/Map/Quest/Data/PDA_Quest_Base.PDA_Quest_Base_C|GetQuestReward (Variables|/Game/SurvivorsTemplate/Blueprints/Map/Quest/BP_Quest.BP_Quest_C|GetQuestData Quest))
    (Class|IControllerManager|OnReward(Message) (Game|GetPlayerController 0) (.Rewardtype (Utilities|Struct|BreakST_QuestRewardData _array_element)) "NewEnumerator0" "NewEnumerator0")))

(event Custom|EndQuest
  (params (IsSuccess :type Boolean) (Quest :type BP%20Quest%20Object%20Reference))
  (if IsSuccess
    (CallFunction|OnQuestCompleted Quest)))

(event EventBeginPlay
  (Utilities|FlowControl|Delay 2.0)
  (CallFunction|StartQuest "/Game/SurvivorsTemplate/Blueprints/Map/Quest/Data/DA_KillEnemies.DA_KillEnemies"))