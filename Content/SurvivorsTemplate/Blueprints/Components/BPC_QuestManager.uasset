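; Quest manager component for the Survivors template that starts, tracks and rewards one current quest, opening with the brazero activation quest shortly after BeginPlay.
; Quests requiring acceptance are held pending until the player controller reports the player's choice.
; Started quests become BP_QuestBase objects built from quest data and passed to the controller for setup.
; On successful completion, each reward entry is sent to the player controller.
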(event Custom|OnQuestCompleted
  (params (Quest :type BP%20Quest%20Base%20Object%20Reference))
  (for _array_element (Variables|/Game/SurvivorsTemplate/Blueprints/Map/Quest/Data/PDA_Quest_Base.PDA_Quest_Base_C|GetQuestReward (Variables|/Game/SurvivorsTemplate/Blueprints/Map/Quest/BP_QuestBase.BP_QuestBase_C|GetQuestData Quest))
    (Class|IControllerManager|OnReward(Message) (Game|GetPlayerController 0) (.Rewardtype (Utilities|Struct|BreakST_QuestRewardData _array_element)) "NewEnumerator0" "NewEnumerator0" (.Amount (Utilities|Struct|BreakST_QuestRewardData _array_element)))))

(event EventBeginPlay
  (Utilities|FlowControl|Delay 2.0)
  (CallFunction|StartQuest "/Game/SurvivorsTemplate/Blueprints/Map/Quest/Data/DA_ActivateBrazero.DA_ActivateBrazero"))

(fn StartQuest
  (params (QuestData :type PDA%20Quest%20Base%20Object%20Reference) (QuestActor :type Actor%20Object%20Reference))
  (bind _returnvalue (Game|GetPlayerController 0))
  (if (Variables|/Game/SurvivorsTemplate/Blueprints/Map/Quest/Data/PDA_Quest_Base.PDA_Quest_Base_C|GetMustBeAccepted QuestData)
    (Variables|Default|SetPendingQuestAccept true)
    (Class|IControllerManager|ShowQuestAcceptUI(Message) _returnvalue QuestData)
    (bind _asbp_gameplay_player_controller (Utilities|Casting|CastToBP_Gameplay_PlayerController _returnvalue))
    (Variables|Default|SetPendingQuestData QuestData)
    (Variables|Default|SetPendingQuestActor QuestActor)
    (EventDispatchers|BindEventtoQuestChoiceOver _asbp_gameplay_player_controller (EventDispatchers|CreateEvent :!event OnQuestChoiceOver))
    (else
      (bind _gamemanager (Class|IGameInstance|GetGameManager(Message) (Game|GetGameInstance)))
      (bind _returnvalue_2 (Game|ConstructObjectfromClass "/Game/SurvivorsTemplate/Blueprints/Map/Quest/BP_QuestBase.BP_QuestBase_C" _gamemanager QuestData QuestActor))
      (bind _output_get (LocalVariables|SetCurrentQuest _returnvalue_2))
      (Default|StartQuest _output_get)
      (Class|IControllerManager|SetupQuest(Message) (Game|GetPlayerController 0) (LocalVariables|GetCurrentQuest))
      (EventDispatchers|BindEventtoEndQuest (LocalVariables|GetCurrentQuest) (EventDispatchers|CreateEvent :!event OnQuestEnd)))))

(fn OnQuestEnd
  (params (IsSuccess :type Boolean) (Quest :type BP%20Quest%20Base%20Object%20Reference))
  (if IsSuccess
    (CallFunction|OnQuestCompleted Quest)))

(fn OnQuestChoiceOver
  (params (DoAccept :type Boolean))
  (if DoAccept
    (bind _gamemanager (Class|IGameInstance|GetGameManager(Message) (Game|GetGameInstance)))
    (bind _returnvalue (Game|ConstructObjectfromClass "/Game/SurvivorsTemplate/Blueprints/Map/Quest/BP_QuestBase.BP_QuestBase_C" _gamemanager (Variables|Default|GetPendingQuestData) (Variables|Default|GetPendingQuestActor)))
    (bind _output_get (LocalVariables|SetCurrentQuest _returnvalue))
    (Default|StartQuest _output_get)
    (Class|IControllerManager|SetupQuest(Message) (Game|GetPlayerController 0) (LocalVariables|GetCurrentQuest))
    (EventDispatchers|BindEventtoEndQuest (LocalVariables|GetCurrentQuest) (EventDispatchers|CreateEvent :!event OnQuestEnd))
    (Variables|Default|SetPendingQuestData 0)
    (Variables|Default|SetPendingQuestActor 0)
    (Variables|Default|SetPendingQuestAccept false)
    (else
      (Variables|Default|SetPendingQuestData 0)
      (Variables|Default|SetPendingQuestActor 0)
      (Variables|Default|SetPendingQuestAccept false))))