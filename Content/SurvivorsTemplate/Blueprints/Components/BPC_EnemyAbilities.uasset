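; Enemy ability component that picks a random off-cooldown ability from its list and runs it as an object constructed from the ability's class.
; Candidates are filtered by MinPhase and a per-ability timestamp map, seeded far in the past so all start ready.
; Execution sets IsBusy, which CanUseAbility returns uninverted; AbilityEnd clears it and stamps the cooldown.
; SpawnRequest spawns actors of a given class, transform and instigator.
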(event Custom|AbilityEnd
  (Utilities|Map|Add (Variables|Default|GetCooldownMap) (Variables|Default|GetNewVar) (Utilities|Time|GetGameTimeinSeconds))
  (Variables|Default|SetIsBusy false))

(event EventBeginPlay
  (for _array_element (Variables|Default|GetAbilitiesList)
    (Utilities|Map|Add (Variables|Default|GetCooldownMap) _array_element -1e+03)))

(event EventTick
  (params (DeltaSeconds :type Float%20%28single-precision%29)))

(fn ChoseRandomAbility
  (bind _availableabilities (CallFunction|GetAvailableAbilities -1))
  (if (> (Utilities|Array|Length _availableabilities) 0)
    (if (Utilities|IsValidClass (.AbilitiyClass (Utilities|Struct|BreakST_AbilityStruct (Utilities|Array|Get(acopy) _availableabilities (Math|Random|RandomIntegerinRange 0 (- (Utilities|Array|Length _availableabilities) 1))))))
      (Variables|Default|SetNewVar (Utilities|Array|Get(acopy) _availableabilities (Math|Random|RandomIntegerinRange 0 (- (Utilities|Array|Length _availableabilities) 1))))
      (bind _returnvalue (Game|ConstructObjectfromClass (.AbilitiyClass (Utilities|Struct|BreakST_AbilityStruct (Utilities|Array|Get(acopy) _availableabilities (Math|Random|RandomIntegerinRange 0 (- (Utilities|Array|Length _availableabilities) 1))))) (Components|GetOwner) self (.AbilityData (Utilities|Struct|BreakST_AbilityStruct (Utilities|Array|Get(acopy) _availableabilities (Math|Random|RandomIntegerinRange 0 (- (Utilities|Array|Length _availableabilities) 1)))))))
      (bind _output_get (Variables|Default|SetCurrentAbility _returnvalue))
      (Default|ExecuteAbility _output_get)
      (Variables|Default|SetIsBusy true))))

(fn GetAvailableAbilities
  (params (CurrentPhase :type Integer))
  ;[0.15 0.15 0.15 0.5] Returns available abilities
  (LocalVariables|Setm_CurrentPhase CurrentPhase)
  (for _array_element (Variables|Default|GetAbilitiesList)
    (if (>= (Variables|/Game/SurvivorsTemplate/Blueprints/Abilities/Data/PDA_Ability.PDA_Ability_C|GetMinPhase (.AbilityData (Utilities|Struct|BreakST_AbilityStruct _array_element))) (LocalVariables|Getm_CurrentPhase))
      (bind _isavailable (CallFunction|CheckCooldown _array_element))
      (if _isavailable
        (Utilities|Array|AddUnique (LocalVariables|GetAvailableAbilities) _array_element))))
  (return (LocalVariables|GetAvailableAbilities)))

(fn CheckCooldown
  (params (Ability :type ST%20Ability%20Struct%20Structure))
  ;[0.15 0.15 0.15 0.5] Calculates cooldown for a given ability struct
  (return (>= (- (Utilities|Time|GetGameTimeinSeconds) (.Value (Utilities|Map|Find (Variables|Default|GetCooldownMap) Ability))) (Variables|/Game/SurvivorsTemplate/Blueprints/Abilities/Data/PDA_Ability.PDA_Ability_C|GetCooldown (.AbilityData (Utilities|Struct|BreakST_AbilityStruct Ability))))))

(fn CanUseAbility
  (return (Variables|Default|GetIsBusy)))

(fn SpawnRequest
  (params (Class :type Actor%20Class%20Reference) (Transform :type Transform) (Instigator :type Pawn%20Object%20Reference))
  (bind (_location _rotation _scale) (Math|Transform|BreakTransform Transform))
  (bind _returnvalue (Game|SpawnActorfromClass Class (Math|Transform|MakeTransform _location _rotation _scale) "Undefined" "MultiplyWithRoot" 0 Instigator))
  (return _returnvalue))