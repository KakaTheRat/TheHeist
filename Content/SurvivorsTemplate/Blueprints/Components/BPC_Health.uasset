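; BPC_Health is an actor component that tracks an entity's health and handles its death.
; Init fills health to max, and ModifyHealth applies a clamped change, then broadcasts the normalized value and owner name through OnUpdate.
; At zero health it notifies the game manager with a tagged killed-entity event and payload, then fires OnDead.
; It can also ask the player controller to set up a screen-space health bar for its owner.
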(event Custom|AddScreenSpaceBar
  ;[0.15 0.15 0.15 0.5] Screen space health bar setup
  (Class|IControllerManager|SetupHealthBar(Message) (Game|GetPlayerController 0) (Components|GetOwner) (Utilities|String|StringToName (Utilities|GetDisplayName (Components|GetOwner))) (Variables|Default|GetCurrentHealth)))

(event Custom|ModifyHealth
  (params (Modification :type Float%20%28double-precision%29))
  ;[0.15 0.15 0.15 0.5] Life calculation
  (Variables|Default|SetCurrentHealth (Math|Float|Clamp(Float) (+ (Variables|Default|GetCurrentHealth) Modification) 0.0 (Variables|Default|GetMaxHealth)))
  (Default|CallOnUpdate (/ (Variables|Default|GetCurrentHealth) (Variables|Default|GetMaxHealth)) (Utilities|String|StringToName (Utilities|GetDisplayName (Components|GetOwner))))
  (if (<= (Variables|Default|GetCurrentHealth) 0.0)
    (bind _gamemanager (Class|IGameInstance|GetGameManager(Message) (Game|GetGameInstance)))
    (Default|NotifyEvent _gamemanager (Variables|Default|GetKilledEntityEventTag) (Components|GetOwner) (Utilities|Struct|MakeST_EventPayload "(TagName=\"\")" (Utilities|GetClass (Components|GetOwner)) 1))
    (Default|CallOnDead (Components|GetOwner))))

(event Custom|Init
  (Variables|Default|SetCurrentHealth (Variables|Default|GetMaxHealth)))