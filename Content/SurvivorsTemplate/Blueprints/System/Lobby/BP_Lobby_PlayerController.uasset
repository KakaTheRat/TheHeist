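; Lobby player controller that creates and maintains the lobby menu UI for its player.
; On BeginPlay, the local controller runs CleanUpUI, then creates or reuses the WB_LobbyMenu widget, adds it to the viewport and sets Game and UI input focused on it.
; OnPlayerJoin calls OC_UpdatePlayerTotal, which passes the GameState PlayerArray length to the widget as the player count.
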(event Custom|OC_UpdatePlayerTotal
  ;[1 1 1] Update Player Count
  (Default|UpdatePlayerTotal (Variables|Default|GetPlayerHud) (Utilities|Array|Length (Variables|/Script/Engine.GameStateBase|GetPlayerArray (Game|GetGameState)))))

(event EventBeginPlay
  ;[1 1 1] Prepare UI
  (|CallParentFunction)
  (if (Pawn|IsLocalPlayerController)
    (CallFunction|CleanUpUI)
    (CallFunction|CreateUI)))

(event EventOnPlayerJoin
  ;[1 1 1] Update Player Count
  (CallFunction|OCUpdatePlayerTotal))

(fn ConstructionScript
  (|CallParentFunction))

(fn CreateUI
  (bind _playerhud (Variables|Default|GetPlayerHud)
    (:then
      (if (not (UserInterface|Viewport|IsinViewport _playerhud))
        (UserInterface|Viewport|AddtoViewport (stale _output_get) 0 :!label _label)
        (Input|SetInputModeGameandUI self (Variables|Default|GetPlayerHud) "DoNotLock" false false)))
    (:else
      (bind _returnvalue (UserInterface|CreateWidget "/Game/SurvivorsTemplate/Widgets/WB_LobbyMenu.WB_LobbyMenu_C" self))
      (bind _output_get (Variables|Default|SetPlayerHud _returnvalue))
      (goto _label))))