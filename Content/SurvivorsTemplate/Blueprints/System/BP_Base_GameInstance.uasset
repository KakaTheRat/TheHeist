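; Base game instance for the Survivors template that holds shared game state: pausable actors, quest progress and a GameManager reference.
; Actors register in a unique list, and the Pause event sends each valid one a pause or resume message.
; Quest updates append completed objectives to structs in a name-keyed map, creating a default entry for unknown quests without recording that objective.
; Getters expose quest state and the game manager.
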(event EventAddPausable
  (params (ActorToPause :type Actor%20Object%20Reference))
  (Utilities|Array|AddUnique (Variables|Default|GetPausableActors) ActorToPause))

(event EventPause
  (params (ShouldPause :type Boolean))
  (for _array_element (Variables|Default|GetPausableActors)
    (Utilities|IsValid _array_element
      (:Is%20Valid
        (if ShouldPause
          (Class|IPausable|Pause(Message) _array_element)
          (else
            (Class|IPausable|Resume(Message) _array_element)))))))

(event EventUpdateQuestState
  (params (QuestName :type Name :default "None") (QuestObjective :type BP%20Quest%20Objective%20Base%20Object%20Reference))
  (CallFunction|UpdateQuest QuestName QuestObjective))

(fn UpdateQuest
  (params (QuestName :type Name) (QuestObjective :type BP%20Quest%20Objective%20Base%20Object%20Reference))
  (bind _quests (Variables|Default|GetQuests))
  (bind (_value _returnvalue) (Utilities|Map|Find _quests QuestName))
  ;[0.15 0.15 0.15 0.5] Update quest state
  (LocalVariables|SetCurrentQuestStruct _value)
  (if _returnvalue
    (Utilities|Array|Add (Utilities|Struct|BreakST_QuestState (LocalVariables|GetCurrentQuestStruct)) QuestObjective)
    (bind _structout (Utilities|Struct|SetmembersinST_QuestState (LocalVariables|GetCurrentQuestStruct) (Utilities|Struct|BreakST_QuestState (LocalVariables|GetCurrentQuestStruct))))
    (Utilities|Map|Add (Variables|Default|GetQuests) QuestName _structout)
    (else
      (Utilities|Map|Add :TargetMap (Variables|Default|GetQuests) :Key QuestName))))

(fn GetGameManager
  (return (Variables|Default|GetGameManager)))

(fn GetQuestState
  (params (QuestName :type Name :default "None"))
  (bind _quests (Variables|Default|GetQuests))
  (bind (_value _returnvalue) (Utilities|Map|Find _quests QuestName))
  ;[0.15 0.15 0.15 0.5] Get quest state
  (if _returnvalue
    (return _value true)
    (else
      (return "" false))))