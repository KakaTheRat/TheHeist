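; Capture-zone quest actor: the player entering its cylinder starts a timed quest through the player's BPC_QuestManager.
; StartQuest runs a looping timer that shrinks the cylinder toward MinSize over MaxTime.
; Leaving mid-capture shows a red vignette and starts a five-second countdown to a quest-failed event via the game manager message system.
; Re-entry hides the vignette without stopping that countdown; EndQuest stops shrinking and hides the decal.
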(event OnComponentBeginOverlap(Cylinder)
  (params (OverlappedComponent :type Primitive%20Component%20Object%20Reference) (OtherActor :type Actor%20Object%20Reference) (OtherComp :type Primitive%20Component%20Object%20Reference) (OtherBodyIndex :type Integer) (bFromSweep :type Boolean) (SweepResult :type Hit%20Result%20Structure%20%28by%20ref%29))
  (if (== OtherActor (Game|Player|GetPlayerPawn 0))
    (if (Variables|Default|GetCaptureOngoing)
      (if (Variables|Default|GetPlayerOutside)
        (Rendering|AddorUpdateBlendable (Actor|GetComponentbyClass (Game|Player|GetPlayerPawn 0) "/Script/Engine.PostProcessComponent") "/Game/SurvivorsTemplate/Blueprints/Abilities/RedVignette.RedVignette" 0.0 :!class /Script/Engine.PostProcessComponent))
      (else
        (CallFunction|StartCapture)))))

(event OnComponentEndOverlap(Cylinder)
  (params (OverlappedComponent :type Primitive%20Component%20Object%20Reference) (OtherActor :type Actor%20Object%20Reference) (OtherComp :type Primitive%20Component%20Object%20Reference) (OtherBodyIndex :type Integer))
  (if (and (== OtherActor (Game|Player|GetPlayerPawn 0)) (Variables|Default|GetCaptureOngoing))
    (Rendering|AddorUpdateBlendable (Actor|GetComponentbyClass (Game|Player|GetPlayerPawn 0) "/Script/Engine.PostProcessComponent") "/Game/SurvivorsTemplate/Blueprints/Abilities/RedVignette.RedVignette" 1.0 :!class /Script/Engine.PostProcessComponent)
    (Variables|Default|SetPlayerOutside true)
    (Class|IGameInstance|GetGameManager(Message) (Game|GetGameInstance))
    (Variables|Default|SetOutsidePlayerTimer 0.0)
    (Utilities|Time|SetTimerbyEvent (delegate Custom|CustomEvent) 0.1 true)))

(event Custom|StartCapture
  (Default|StartQuest (Actor|GetComponentbyClass (Game|Player|GetPlayerPawn 0) "/Game/SurvivorsTemplate/Blueprints/Components/BPC_QuestManager.BPC_QuestManager_C") "/Game/SurvivorsTemplate/Blueprints/Map/Quest/Data/DA_Timer.DA_Timer" self "(GameplayTags=)"))

(event Custom|Update
  (bind _returnvalue (Utilities|Time|GetGameTimeinSeconds))
  (bind _maxtime (Variables|Default|GetMaxTime))
  (bind _currenttime (Variables|Default|GetCurrentTime))
  (bind _returnvalue_2 (- _returnvalue _currenttime))
  (bind _returnvalue_3 (/ _returnvalue_2 _maxtime))
  (if (<= _returnvalue_3 1.0)
    (bind _output_get (Variables|Default|SetCurrentProgress _returnvalue_3))
    (Transformation|SetWorldScale3D (Variables|Default|GetCylinder) (* (Math|Float|Lerp 1.0 (Variables|Default|GetMinSize) _output_get) (Variables|Default|GetOriginalSize)))
    (else
      (Utilities|Time|ClearandInvalidateTimerbyHandle (Variables|Default|GetTimerHandle)))))

(event Custom|CustomEvent
  (bind _output_get (Variables|Default|SetOutsidePlayerTimer (+ (Variables|Default|GetOutsidePlayerTimer) 0.1)))
  (if (>= _output_get 5.0)
    (Rendering|AddorUpdateBlendable (Actor|GetComponentbyClass (Game|Player|GetPlayerPawn 0) "/Script/Engine.PostProcessComponent") "/Game/SurvivorsTemplate/Blueprints/Abilities/RedVignette.RedVignette" 0.0 :!class /Script/Engine.PostProcessComponent)
    (bind _gamemanager (Class|IGameInstance|GetGameManager(Message) (Game|GetGameInstance)))
    (Default|NotifyEvent _gamemanager "(TagName=\"Quest.Event.Classic.Failed\")" self)))

(event EventBeginPlay)

(event Collision|EventActorBeginOverlap
  (params (OtherActor :type Actor%20Object%20Reference)))

(event EventTick
  (params (DeltaSeconds :type Float%20%28single-precision%29)))

(event EventStartQuest
  (Variables|Default|SetCaptureOngoing true)
  (Variables|Default|SetCurrentTime (Utilities|Time|GetGameTimeinSeconds))
  (Variables|Default|SetOriginalSize (Transformation|GetWorldScale (Variables|Default|GetCylinder)))
  (bind _returnvalue (Utilities|Time|SetTimerbyEvent (delegate Custom|Update) 0.01 true))
  (Variables|Default|SetTimerHandle _returnvalue))

(event EventEndQuest
  (params (IsSuccess :type Boolean))
  (Utilities|Time|ClearandInvalidateTimerbyHandle (Variables|Default|GetTimerHandle))
  (Rendering|SetVisibility (Variables|Default|GetDecal) false false))

(fn ConstructionScript)