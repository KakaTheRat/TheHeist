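; Arena encounter zone that locks the player in to fight a wave of enemies.
; Player overlap starts it once: game-manager spawning stops, doors close, and after a delay LaunchWave totals the enemies, starts a quest and a looping spawn timer.
; Spawning adds one enemy per call at random spawn points, tracking per-class counts in a map.
; Death callbacks count down to zero, then notify quest completion, reopen doors, trigger rewards and start a sequence.
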(event OnComponentBeginOverlap(ArenaTrigger)
  (params (OverlappedComponent :type Primitive%20Component%20Object%20Reference) (OtherActor :type Actor%20Object%20Reference) (OtherComp :type Primitive%20Component%20Object%20Reference) (OtherBodyIndex :type Integer) (bFromSweep :type Boolean) (SweepResult :type Hit%20Result%20Structure%20%28by%20ref%29))
  (if (== OtherActor (Game|Player|GetPlayerPawn 0))
    (CallFunction|StartArena)
    (Default|CallArenaIdle false)))

(event Custom|StartArena
  (Utilities|FlowControl|DoOnce false
    (:Completed
      (bind _gamemanager (Class|IGameInstance|GetGameManager(Message) (Game|GetGameInstance)))
      (Class|IGameManager|StopSpawn(Message) _gamemanager)
      (CallFunction|InitializeEntries false)
      (Utilities|FlowControl|Delay 3.0)
      (CallFunction|LaunchWave))))

(event Custom|EndArena
  (CallFunction|InitializeEntries true)
  (for _array_element (Variables|Default|GetReward)
    (Class|ITrigger|Trigger(Message) _array_element))
  (bind _returnvalue (Actor|GetActorOfClass "/Game/SurvivorsTemplate/BP_SequenceManager.BP_SequenceManager_C"))
  (Default|StartSequence _returnvalue (Variables|Default|GetSequenceStruct)))

(event Custom|SpawnEnemy
  (bind _spawnpoints (Variables|Default|GetSpawnPoints))
  (bind _gamemanager (Variables|Default|GetGameManager))
  (bind _returnvalue (Utilities|Array|Length _spawnpoints))
  (bind _returnvalue_2 (- _returnvalue 1))
  (bind _returnvalue_3 (Math|Random|RandomIntegerinRange 0 _returnvalue_2))
  (bind _output (Utilities|Array|Get(acopy) _spawnpoints _returnvalue_3))
  (bind _returnvalue_4 (Transformation|GetActorTransform _output))
  (bind (_keypin _valuepin) (Utilities|Map|ForEachLoop(Map) (.EnemyClass (Utilities|Struct|BreakST_WaveData (Utilities|Array|Get(acopy) (Variables|/Game/SurvivorsTemplate/Blueprints/Map/Arena/Data/PDA_ArenaSetup.PDA_ArenaSetup_C|GetWaves (Variables|Default|GetArenaSetup)) (Variables|Default|GetCurrentWave)))) :!label _label)
    (:then
      (if (.ReturnValue (Utilities|Map|Find (Variables|Default|GetCurrentWaveState) _keypin))
        (if (not (>= (.Value (Utilities|Map|Find (Variables|Default|GetCurrentWaveState) _keypin)) _valuepin))
          (bind _returnvalue_5 (Game|SpawnActorfromClass :Class _keypin :SpawnTransform _returnvalue_4 :CollisionHandlingOverride "AlwaysSpawn" :TransformScaleMethod "MultiplyWithRoot" :Soul "/Game/SurvivorsTemplate/Blueprints/GameplayActors/BP_Soul.BP_Soul_C" :GM_Interface _gamemanager :Instigator 0))
          (EventDispatchers|BindEventtoOnDeath _returnvalue_5 (delegate Custom|ee))
          (Utilities|Map|Add (Variables|Default|GetCurrentWaveState) _keypin (+ (.Value (Utilities|Map|Find (Variables|Default|GetCurrentWaveState) _keypin)) 1))
          (goto _label BreakPin))
        (else
          (bind _returnvalue_6 (Game|SpawnActorfromClass _keypin _returnvalue_4 "AlwaysSpawn" "MultiplyWithRoot" 0 0 1e+01 15.0 "/Game/SurvivorsTemplate/Blueprints/GameplayActors/BP_Soul.BP_Soul_C" false false _gamemanager 1 "(TagName=\"Context.Spawn.Arena\")" 0))
          (EventDispatchers|BindEventtoOnDeath _returnvalue_6 (delegate Custom|DeadUnit))
          (Utilities|Map|Add (Variables|Default|GetCurrentWaveState) _keypin 1)
          (goto _label BreakPin))))))

(event Custom|ee
  (params (EnemyRef :type Actor%20Object%20Reference))
  (Math|Integer|DecrementInt (Variables|Default|GetEnnemisToBeat)
    (:%20%20
      (if (<= (Variables|Default|GetEnnemisToBeat) 0)
        (CallFunction|EndOfWave)))))

(event Custom|EndOfWave
  (bind _gamemanager (Class|IGameInstance|GetGameManager(Message) (Game|GetGameInstance)))
  (Default|NotifyEvent _gamemanager "(TagName=\"Quest.Event.Classic.Completed\")" self)
  (CallFunction|EndArena))

(event Custom|DeadUnit
  (params (EnemyRef :type Actor%20Object%20Reference))
  (Math|Integer|DecrementInt (Variables|Default|GetEnnemisToBeat)
    (:%20%20
      (if (<= (Variables|Default|GetEnnemisToBeat) 0)
        (CallFunction|EndOfWave)))))

(event EventBeginPlay)

(fn ConstructionScript)

(fn InitializeEntries
  (params (bShouldOpenArena :type Boolean))
  (if bShouldOpenArena
    (for _array_element (Variables|Default|GetDoors)
      (Class|IDoor|Open(Message) _array_element))
    (else
      (for _array_element_2 (Variables|Default|GetDoors)
        (Class|IDoor|Close(Message) _array_element_2)))))

(fn LaunchWave
  (bind _currentwave (Variables|Default|GetCurrentWave))
  (bind _arenasetup (Variables|Default|GetArenaSetup))
  (bind _waves (Variables|/Game/SurvivorsTemplate/Blueprints/Map/Arena/Data/PDA_ArenaSetup.PDA_ArenaSetup_C|GetWaves _arenasetup))
  (bind _output (Utilities|Array|Get(acopy) _waves _currentwave))
  (bind (_enemyclass _spawndelay) (Utilities|Struct|BreakST_WaveData _output))
  (Variables|Default|SetEnnemisToBeat 0)
  (bind _valuepin (Utilities|Map|ForEachLoop(Map) _enemyclass)
    (:then
      (Variables|Default|SetEnnemisToBeat (+ (Variables|Default|GetEnnemisToBeat) _valuepin)))
    (:CompletedPin
      (Utilities|Time|SetTimerbyEvent (EventDispatchers|CreateEvent :!event Custom|SpawnEnemy) _spawndelay true)
      (Default|StartQuest (Actor|GetComponentbyClass (Game|Player|GetPlayerPawn 0) "/Game/SurvivorsTemplate/Blueprints/Components/BPC_QuestManager.BPC_QuestManager_C") "/Game/SurvivorsTemplate/Blueprints/Map/Quest/Data/DA_GoblinSlayerEntranceArena.DA_GoblinSlayerEntranceArena" self))))

(fn Spawn
  (bind _spawnpoints (Variables|Default|GetSpawnPoints))
  (bind _gamemanager (Variables|Default|GetGameManager))
  (bind _returnvalue (Utilities|Array|Length _spawnpoints))
  (bind _returnvalue_2 (- _returnvalue 1))
  (bind _returnvalue_3 (Math|Random|RandomIntegerinRange 0 _returnvalue_2))
  (bind _output (Utilities|Array|Get(acopy) _spawnpoints _returnvalue_3))
  (bind _returnvalue_4 (Transformation|GetActorTransform _output))
  (bind (_keypin _valuepin) (Utilities|Map|ForEachLoop(Map) (.EnemyClass (Utilities|Struct|BreakST_WaveData (Utilities|Array|Get(acopy) (Variables|/Game/SurvivorsTemplate/Blueprints/Map/Arena/Data/PDA_ArenaSetup.PDA_ArenaSetup_C|GetWaves (Variables|Default|GetArenaSetup)) (Variables|Default|GetCurrentWave)))) :!label _label)
    (:then
      (LocalVariables|SetNewLocalVar _keypin)
      (LocalVariables|SetNewLocalVar_0 _valuepin)
      (if (.ReturnValue (Utilities|Map|Find (Variables|Default|GetCurrentWaveState) (LocalVariables|GetNewLocalVar)))
        (if (not (>= (.Value (Utilities|Map|Find (Variables|Default|GetCurrentWaveState) (LocalVariables|GetNewLocalVar))) (LocalVariables|GetNewLocalVar_0)))
          (Game|SpawnActorfromClass :Class (LocalVariables|GetNewLocalVar) :SpawnTransform _returnvalue_4 :CollisionHandlingOverride "AlwaysSpawn" :TransformScaleMethod "MultiplyWithRoot" :MaxHealth 1e+03 :Soul "/Game/SurvivorsTemplate/Blueprints/GameplayActors/BP_Soul.BP_Soul_C" :GM_Interface _gamemanager :Instigator 0)
          (Utilities|Map|Add (Variables|Default|GetCurrentWaveState) (LocalVariables|GetNewLocalVar) (+ (.Value (Utilities|Map|Find (Variables|Default|GetCurrentWaveState) (LocalVariables|GetNewLocalVar))) 1))
          (goto _label BreakPin))
        (else
          (bind _returnvalue_5 (Game|SpawnActorfromClass :Class (LocalVariables|GetNewLocalVar) :SpawnTransform _returnvalue_4 :CollisionHandlingOverride "AlwaysSpawn" :TransformScaleMethod "MultiplyWithRoot" :Soul "/Game/SurvivorsTemplate/Blueprints/GameplayActors/BP_Soul.BP_Soul_C" :GM_Interface _gamemanager :Instigator 0))
          (Utilities|Map|Add (Variables|Default|GetCurrentWaveState) (LocalVariables|GetNewLocalVar) 1)
          (goto _label BreakPin))))))