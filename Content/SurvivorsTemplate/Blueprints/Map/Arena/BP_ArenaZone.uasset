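; Arena zone that locks the player into an enemy wave with a fixed camera and reactive crowd audio.
; Entering the trigger closes doors, then LaunchWave totals enemies from ArenaSetup, starts a looping timer and starts the DA_Convoy quest.
; SpawnEnemy adds one enemy per call at random points up to per-class quotas, with death events counting down.
; At zero it notifies quest completion, restores the third-person camera and reopens doors.
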(event OnComponentBeginOverlap(ArenaTrigger)
  (params (OverlappedComponent :type Primitive%20Component%20Object%20Reference) (OtherActor :type Actor%20Object%20Reference) (OtherComp :type Primitive%20Component%20Object%20Reference) (OtherBodyIndex :type Integer) (bFromSweep :type Boolean) (SweepResult :type Hit%20Result%20Structure%20%28by%20ref%29))
  (bind _crowdreaction (Variables|Default|GetCrowdReaction))
  (bind _audio (Variables|Default|GetAudio))
  (if (== OtherActor (Game|Player|GetPlayerPawn 0))
    (CallFunction|StartArena)
    (Default|CallArenaIdle false)
    (Audio|Components|Audio|SetSound _crowdreaction "/Game/SurvivorsTemplate/FX/SFX/CrowdCheering.CrowdCheering")
    (Audio|Components|Audio|FadeIn _crowdreaction 2.0 3.0 0.0 "SCurve" :!class /Script/Engine.AudioComponent)
    (Utilities|FlowControl|Delay 0.0)
    (Audio|Components|Audio|Play _audio 0.0)
    (Audio|Components|Audio|AdjustVolume _audio 2.0 2.0 "SCurve" :!class /Script/Engine.AudioComponent)
    (Audio|Components|Audio|Play (Variables|Default|GetAudio1) 0.0)
    (Game|Player|SetViewTargetwithBlend (Game|GetPlayerController 0) (Variables|Default|GetNewVar_1) 2.0 "VTBlend_Linear" 0.0 false)
    (Default|SwitchMapping (Variables|Default|GetNewVar_0) "/Game/SoStylized/Demo/Pawn/Input/IMC_FixCamera.IMC_FixCamera")))

(event OnComponentBeginOverlap(Box)
  (params (OverlappedComponent :type Primitive%20Component%20Object%20Reference) (OtherActor :type Actor%20Object%20Reference) (OtherComp :type Primitive%20Component%20Object%20Reference) (OtherBodyIndex :type Integer) (bFromSweep :type Boolean) (SweepResult :type Hit%20Result%20Structure%20%28by%20ref%29))
  (Audio|Components|Audio|AdjustVolume (Variables|Default|GetAudio) 2.0 3.0 "SCurve" :!class /Script/Engine.AudioComponent))

(event OnComponentBeginOverlap(Box1)
  (params (OverlappedComponent :type Primitive%20Component%20Object%20Reference) (OtherActor :type Actor%20Object%20Reference) (OtherComp :type Primitive%20Component%20Object%20Reference) (OtherBodyIndex :type Integer) (bFromSweep :type Boolean) (SweepResult :type Hit%20Result%20Structure%20%28by%20ref%29))
  (Audio|Components|Audio|AdjustVolume (Variables|Default|GetAudio) 4.0 0.0 "SCurve" :!class /Script/Engine.AudioComponent)
  (Default|CallArenaIdle true))

(event Custom|StartArena
  (CallFunction|InitializeEntries false)
  (Utilities|FlowControl|Delay 3.0)
  (CallFunction|LaunchWave))

(event Custom|EndArena
  (Game|Player|SetViewTargetwithBlend (Game|GetPlayerController 0) (Game|GetPlayerCharacter 0) 2.0 "VTBlend_Linear" 0.0 false)
  (Utilities|FlowControl|Delay 2.0)
  (Default|SwitchMapping (Variables|Default|GetNewVar_0) "/Game/SoStylized/Demo/Pawn/Input/IMC_ThirdPersonChar.IMC_ThirdPersonChar")
  (CallFunction|InitializeEntries true))

(event Custom|SpawnEnemy
  (bind _spawnpoints (Variables|Default|GetSpawnPoints))
  (bind _newvar (Variables|Default|GetNewVar))
  (bind _returnvalue (Utilities|Array|Length _spawnpoints))
  (bind _returnvalue_2 (- _returnvalue 1))
  (bind _returnvalue_3 (Math|Random|RandomIntegerinRange 0 _returnvalue_2))
  (bind _output (Utilities|Array|Get(acopy) _spawnpoints _returnvalue_3))
  (bind _returnvalue_4 (Transformation|GetActorTransform _output))
  (bind (_keypin _valuepin) (Utilities|Map|ForEachLoop(Map) (.EnemyClass (Utilities|Struct|BreakST_WaveData (Utilities|Array|Get(acopy) (Variables|/Game/SurvivorsTemplate/Blueprints/Map/Arena/Data/PDA_ArenaSetup.PDA_ArenaSetup_C|GetWaves (Variables|Default|GetArenaSetup)) (Variables|Default|GetCurrentWave)))) :!label _label)
    (:then
      (if (.ReturnValue (Utilities|Map|Find (Variables|Default|GetCurrentWaveState) _keypin))
        (if (not (>= (.Value (Utilities|Map|Find (Variables|Default|GetCurrentWaveState) _keypin)) _valuepin))
          (bind _returnvalue_5 (Game|SpawnActorfromClass _keypin _returnvalue_4 "AlwaysSpawn" "MultiplyWithRoot" 0 0 1e+01 15.0 "/Game/SurvivorsTemplate/Blueprints/GameplayActors/BP_Soul.BP_Soul_C" false false _newvar 1 0))
          (EventDispatchers|BindEventtoOnDeath _returnvalue_5 (delegate Custom|ee))
          (Utilities|Map|Add (Variables|Default|GetCurrentWaveState) _keypin (+ (.Value (Utilities|Map|Find (Variables|Default|GetCurrentWaveState) _keypin)) 1))
          (goto _label BreakPin))
        (else
          (bind _returnvalue_6 (Game|SpawnActorfromClass _keypin _returnvalue_4 "AlwaysSpawn" "MultiplyWithRoot" 0 0 1e+01 15.0 "/Game/SurvivorsTemplate/Blueprints/GameplayActors/BP_Soul.BP_Soul_C" false false _newvar 1 0))
          (EventDispatchers|BindEventtoOnDeath _returnvalue_6 (delegate Custom|DeadUnit))
          (Utilities|Map|Add (Variables|Default|GetCurrentWaveState) _keypin 1)
          (goto _label BreakPin))))))

(event Custom|ee
  (Math|Integer|DecrementInt (Variables|Default|GetEnnemisToBeat)
    (:%20%20
      (if (<= (Variables|Default|GetEnnemisToBeat) 0)
        (CallFunction|EndOfWave)))))

(event Custom|DamageTaken
  (bind _crowdreaction (Variables|Default|GetCrowdReaction))
  (if (not (Audio|Components|Audio|IsPlaying _crowdreaction))
    (Audio|Components|Audio|SetSound _crowdreaction "/Game/SurvivorsTemplate/FX/SFX/GaspCrowd.GaspCrowd")
    (Audio|Components|Audio|Play (Variables|Default|GetCrowdReaction) 0.0)))

(event Custom|PlayerDead
  (bind _crowdreaction (Variables|Default|GetCrowdReaction))
  (Audio|Components|Audio|SetSound _crowdreaction "/Game/SurvivorsTemplate/FX/SFX/crowd-laughing-1.crowd-laughing-1")
  (Audio|Components|Audio|FadeIn _crowdreaction 2.0 2.0 0.0 "SCurve" :!class /Script/Engine.AudioComponent)
  (Audio|Components|Audio|FadeOut (Variables|Default|GetAudio) 2.0 0.0 "SCurve" :!class /Script/Engine.AudioComponent)
  (Audio|Components|Audio|FadeOut (Variables|Default|GetAudio1) 2.0 0.0 "SCurve" :!class /Script/Engine.AudioComponent))

(event Custom|EndOfWave
  (bind _gamemanager (Class|IGameInstance|GetGameManager(Message) (Game|GetGameInstance)))
  (Default|NotifyEvent _gamemanager "(TagName=\"Quest.Event.Classic.Completed\")" self)
  (CallFunction|EndArena))

(event Custom|DeadUnit
  (Math|Integer|DecrementInt (Variables|Default|GetEnnemisToBeat)
    (:%20%20
      (if (<= (Variables|Default|GetEnnemisToBeat) 0)
        (CallFunction|EndOfWave)))))

(event EventBeginPlay
  (Audio|Components|Audio|Play (Variables|Default|GetAudio) 0.0)
  (Utilities|FlowControl|Delay 0.0)
  (bind _returnvalue (Actor|GetActorOfClass "/Game/SurvivorsTemplate/Blueprints/Character/BP_Base_Character.BP_Base_Character_C"))
  (bind _output_get (Variables|Default|SetNewVar_0 _returnvalue))
  (Default|SwitchtoFPS _output_get)
  (EventDispatchers|BindEventtoOnDamageTaken _output_get (delegate Custom|DamageTaken))
  (EventDispatchers|BindEventtoOnDead _output_get (delegate Custom|PlayerDead)))

(fn ConstructionScript)

(fn InitializeEntries
  (params (bShouldOpenArena :type Boolean))
  (if bShouldOpenArena
    (for _array_element (Variables|Default|GetDoors)
      (Class|IDoor|Open(Message) _array_element))
    (else
      (for _array_element_2 (Variables|Default|GetDoors)
        (Class|IDoor|Close(Message) _array_element_2)))))

(fn LaunchWave
  (bind _currentwave (Variables|Default|GetCurrentWave))
  (bind _arenasetup (Variables|Default|GetArenaSetup))
  (bind _waves (Variables|/Game/SurvivorsTemplate/Blueprints/Map/Arena/Data/PDA_ArenaSetup.PDA_ArenaSetup_C|GetWaves _arenasetup))
  (bind _output (Utilities|Array|Get(acopy) _waves _currentwave))
  (bind (_enemyclass _spawndelay) (Utilities|Struct|BreakST_WaveData _output))
  (Variables|Default|SetEnnemisToBeat 0)
  (bind _valuepin (Utilities|Map|ForEachLoop(Map) _enemyclass)
    (:then
      (Variables|Default|SetEnnemisToBeat (+ (Variables|Default|GetEnnemisToBeat) _valuepin)))
    (:CompletedPin
      (Utilities|Time|SetTimerbyEvent (EventDispatchers|CreateEvent :!event Custom|SpawnEnemy) _spawndelay true)
      (Default|StartQuest (Actor|GetComponentbyClass (Game|Player|GetPlayerPawn 0) "/Game/SurvivorsTemplate/Blueprints/Components/BPC_QuestManager.BPC_QuestManager_C") "/Game/SurvivorsTemplate/Blueprints/Map/Quest/Data/DA_Convoy.DA_Convoy" self))))

(fn Spawn
  (bind _spawnpoints (Variables|Default|GetSpawnPoints))
  (bind _newvar (Variables|Default|GetNewVar))
  (bind _returnvalue (Utilities|Array|Length _spawnpoints))
  (bind _returnvalue_2 (- _returnvalue 1))
  (bind _returnvalue_3 (Math|Random|RandomIntegerinRange 0 _returnvalue_2))
  (bind _output (Utilities|Array|Get(acopy) _spawnpoints _returnvalue_3))
  (bind _returnvalue_4 (Transformation|GetActorTransform _output))
  (bind (_keypin _valuepin) (Utilities|Map|ForEachLoop(Map) (.EnemyClass (Utilities|Struct|BreakST_WaveData (Utilities|Array|Get(acopy) (Variables|/Game/SurvivorsTemplate/Blueprints/Map/Arena/Data/PDA_ArenaSetup.PDA_ArenaSetup_C|GetWaves (Variables|Default|GetArenaSetup)) (Variables|Default|GetCurrentWave)))) :!label _label)
    (:then
      (LocalVariables|SetNewLocalVar _keypin)
      (LocalVariables|SetNewLocalVar_0 _valuepin)
      (if (.ReturnValue (Utilities|Map|Find (Variables|Default|GetCurrentWaveState) (LocalVariables|GetNewLocalVar)))
        (if (not (>= (.Value (Utilities|Map|Find (Variables|Default|GetCurrentWaveState) (LocalVariables|GetNewLocalVar))) (LocalVariables|GetNewLocalVar_0)))
          (Game|SpawnActorfromClass (LocalVariables|GetNewLocalVar) _returnvalue_4 "AlwaysSpawn" "MultiplyWithRoot" 0 0 1e+01 1e+03 "/Game/SurvivorsTemplate/Blueprints/GameplayActors/BP_Soul.BP_Soul_C" false false _newvar 1 0)
          (Utilities|Map|Add (Variables|Default|GetCurrentWaveState) (LocalVariables|GetNewLocalVar) (+ (.Value (Utilities|Map|Find (Variables|Default|GetCurrentWaveState) (LocalVariables|GetNewLocalVar))) 1))
          (goto _label BreakPin))
        (else
          (bind _returnvalue_5 (Game|SpawnActorfromClass (LocalVariables|GetNewLocalVar) _returnvalue_4 "AlwaysSpawn" "MultiplyWithRoot" 0 0 1e+01 15.0 "/Game/SurvivorsTemplate/Blueprints/GameplayActors/BP_Soul.BP_Soul_C" false false _newvar 1 0))
          (Utilities|Map|Add (Variables|Default|GetCurrentWaveState) (LocalVariables|GetNewLocalVar) 1)
          (goto _label BreakPin))))))