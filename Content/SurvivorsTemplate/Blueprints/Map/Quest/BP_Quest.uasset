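; BP_Quest is a quest object that tracks the active, complete and failed states of a quest tied to a target actor.
; Init stores the GameManager, and StartQuest stores the target actor, marks the quest active and triggers its start message.
; Completing or failing sets the matching flag, unregisters the quest from the GameManager and triggers the actor's end message.
; Only completion also calls CallObjectiveEnd, reporting success for the first objective.
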(event Custom|StartQuest
  (params (QuestActor :type Actor%20Object%20Reference))
  (bind _output_get (Variables|Default|SetTargetActor QuestActor))
  (Variables|Default|SetIsActive true)
  (Class|IQuest|StartQuest(Message) _output_get))

(event Custom|CompleteQuest
  (Variables|Default|SetIsComplete true)
  (Default|UnregisterListener (Variables|Default|GetGameManager) self)
  (bind _targetactor (Variables|Default|GetTargetActor)
    (:then
      (Class|IQuest|EndQuest(Message) _targetactor))
    (:else
      _))
  (Default|CallObjectiveEnd true))

(event Custom|FailQuest
  (Variables|Default|SetIsFailed true)
  (Default|UnregisterListener (Variables|Default|GetGameManager) self)
  (bind _targetactor (Variables|Default|GetTargetActor)
    (:then
      (Class|IQuest|EndQuest(Message) _targetactor))
    (:else)))

(fn Init
  (params (GameManager :type BP%20Game%20Manager%20Object%20Reference))
  (Variables|Default|SetGameManager GameManager))