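; Base quest Blueprint for the Survivors template that runs the set of objectives defined in its QuestData.
; On start it constructs each objective with the target actor and its data, initializes it with the GameManager, starts it, then binds to its end event.
; Objectives are stored in a map keyed by class.
; A countdown ends the quest when all objectives finish, passing only the last one's success flag.
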(event Custom|StartQuest
  (bind _questdata (Variables|Default|GetQuestData))
  (bind _questobjectives (Variables|/Game/SurvivorsTemplate/Blueprints/Map/Quest/Data/PDA_Quest_Base.PDA_Quest_Base_C|GetQuestObjectives _questdata))
  (Variables|Default|SetObjectivesCount (Utilities|Array|Length _questobjectives))
  (for _array_element _questobjectives
    (bind _returnvalue (Game|ConstructObjectfromClass (Utilities|ResolveSoftReference (.Class (Utilities|Struct|BreakST_ObjectiveClassSetup _array_element))) (Variables|Default|GetTargetActor) (.ObjectivesData (Utilities|Struct|BreakST_ObjectiveClassSetup _array_element))))
    (Default|Init _returnvalue (Variables|Default|GetGameManager))
    (Default|StartQuest _returnvalue)
    (Utilities|Map|Add (Variables|Default|GetObjectivesRef) (Utilities|GetClass _returnvalue) _returnvalue)
    (EventDispatchers|BindEventtoObjectiveClassEnd _returnvalue (EventDispatchers|CreateEvent :!event Custom|OnObjectiveEnded))))

(event Custom|OnObjectiveEnded
  (params (IsSuccess :type Boolean))
  (bind _result (Math|Integer|DecrementInt (Variables|Default|GetObjectivesCount))
    (:%20%20
      (if (<= _result 0)
        (Default|CallEndQuest IsSuccess self)))))