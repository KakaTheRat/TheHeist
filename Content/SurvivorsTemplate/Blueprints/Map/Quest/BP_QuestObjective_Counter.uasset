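; Counter quest objective for the Survivors template that tracks how many times tagged events occur for a given actor class.
; Init builds a counter entry per quest objective from its event tags and the first class/target pair in its map.
; OnEventReceived increments unfinished counters matching tag and payload class, then calls ObjectiveUpdate with progress or successful completion.
; GetDatas returns a counter's current values through the parent's quest data event.
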(event EventOnEventReceived
  (params (EventTag :type Gameplay%20Tag%20Structure) (Instigator :type Actor%20Object%20Reference) (Payload :type ST%20Event%20Payload%20Structure))
  (for (_array_element _array_index) (Variables|Default|GetCounterData)
    (if (< (.CurrentAmount (Utilities|Struct|BreakST_CounterQuestStruct (.Counter (Utilities|Struct|BreakST_CounterOverallStruct _array_element)))) (.MaxAmount (Utilities|Struct|BreakST_CounterQuestStruct (.Counter (Utilities|Struct|BreakST_CounterOverallStruct _array_element)))))
      (Variables|Default|SetCurrentIndex _array_index)
      (if (GameplayTags|MatchesAnyTags EventTag (.Tags (Utilities|Struct|BreakST_CounterOverallStruct _array_element)) true)
        (if (== (.Class (Utilities|Struct|BreakST_CounterOverallStruct _array_element)) (.ActorClass (Utilities|Struct|BreakST_EventPayload Payload)))
          (bind _structout (Utilities|Struct|SetmembersinST_CounterOverallStruct _array_element (Utilities|Struct|MakeST_CounterQuestStruct (.MaxAmount (Utilities|Struct|BreakST_CounterQuestStruct (.Counter (Utilities|Struct|BreakST_CounterOverallStruct _array_element)))) (+ (.CurrentAmount (Utilities|Struct|BreakST_CounterQuestStruct (.Counter (Utilities|Struct|BreakST_CounterOverallStruct _array_element)))) 1))))
          (Utilities|Array|SetArrayElem (Variables|Default|GetCounterData) (Variables|Default|GetCurrentIndex) _structout)
          (if (<= (.MaxAmount (Utilities|Struct|BreakST_CounterQuestStruct (.Counter (Utilities|Struct|BreakST_CounterOverallStruct _array_element)))) (.CurrentAmount (Utilities|Struct|BreakST_CounterQuestStruct (.Counter (Utilities|Struct|BreakST_CounterOverallStruct _array_element)))))
            (CallFunction|ObjectiveUpdate true (Utilities|Struct|MakeST_QuestDataEvent (Variables|Default|GetCurrentIndex) 0.0 (.Counter (Utilities|Struct|BreakST_CounterOverallStruct (Utilities|Array|Get(acopy) (Variables|Default|GetCounterData) (Variables|Default|GetCurrentIndex))))) true)
            (else
              (CallFunction|ObjectiveUpdate false (Utilities|Struct|MakeST_QuestDataEvent (Variables|Default|GetCurrentIndex) 0.0 (.Counter (Utilities|Struct|BreakST_CounterOverallStruct (Utilities|Array|Get(acopy) (Variables|Default|GetCounterData) (Variables|Default|GetCurrentIndex))))) false))))))))

(fn Init
  (params (GameManager :type BP%20Game%20Manager%20Object%20Reference))
  (|CallParentFunction GameManager)
  (for _array_element (Variables|Default|GetQuestObjectives)
    (Utilities|Array|AddUnique (Variables|Default|GetCounterData) (Utilities|Struct|MakeST_CounterOverallStruct (.Key (Utilities|Map|GetKeyValueByIndex (.Counter (Utilities|Struct|BreakST_QuestObjectiveData _array_element)) 0)) (.EventTagTriggered (Utilities|Struct|BreakST_QuestObjectiveData _array_element)) (Utilities|Struct|MakeST_CounterQuestStruct (.Value (Utilities|Map|GetKeyValueByIndex (.Counter (Utilities|Struct|BreakST_QuestObjectiveData _array_element)) 0)))))))

(fn GetDatas
  (params (ObjectiveIndex :type Integer) (DataGivenByObjective :type ST%20Quest%20Data%20Event%20Structure))
  (|CallParentFunction ObjectiveIndex (Utilities|Struct|MakeST_QuestDataEvent ObjectiveIndex 0.0 (.Counter (Utilities|Struct|BreakST_CounterOverallStruct (Utilities|Array|Get(acopy) (Variables|Default|GetCounterData) ObjectiveIndex))))))