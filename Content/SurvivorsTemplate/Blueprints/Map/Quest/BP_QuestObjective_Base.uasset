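; Base quest objective Blueprint that tracks a set of sub-objectives and resolves as succeeded or failed.
; Init gathers each objective's event tags, falling back to defaults, and registers as a GameManager listener, optionally filtered to a target actor.
; Updates broadcast through dispatchers: any failure fails the quest, while finishing every objective completes it, unregistering the listener and messaging the target actor.
; OnEventReceived is empty here.
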(event Custom|StartQuest
  (Variables|Default|SetIsActive true)
  (Class|IQuest|StartQuest(Message) (Variables|Default|GetTargetActor)))

(event Custom|EndObjective
  (params (ObjectiveIndex :type Integer) (IsSuccess :type Boolean))
  ;[0.15 0.1369 0.0299 0.5] End an objective
  (Math|Integer|DecrementInt (Variables|Default|GetObjectivesCount)
    (:%20%20
      (Default|CallObjectiveEnd IsSuccess ObjectiveIndex))))

(event Custom|CompleteObjectiveType
  ;[0.05188 0.06534 0.15 0.5] Quest achievement or failure managment
  (Variables|Default|SetIsComplete true)
  (Default|UnregisterListener (Variables|Default|GetGameManager) self)
  (Default|CallObjectiveClassEnd true self)
  (bind _targetactor (Variables|Default|GetTargetActor)
    (:then
      (Class|IQuest|EndQuest(Message) _targetactor true))
    (:else)))

(event Custom|FailQuest
  ;[0.05188 0.06534 0.15 0.5] Quest achievement or failure managment
  (Variables|Default|SetIsFailed true)
  (Default|UnregisterListener (Variables|Default|GetGameManager) self)
  (Default|CallObjectiveClassEnd false self)
  (bind _targetactor (Variables|Default|GetTargetActor)
    (:then
      (Class|IQuest|EndQuest(Message) _targetactor false))
    (:else)))

(event Custom|ObjectiveUpdate
  (params (IsOver :type Boolean) (ObjectiveData :type ST%20Quest%20Data%20Event%20Structure) (IsSuccess :type Boolean))
  ;[0.15 0.0388 0.0388 0.5] Updates the objectives, mostly for widget update. If not done, will only update, if done will end objective
  (if IsOver
    (Default|CallOnObjectiveUpdate ObjectiveData)
    (CallFunction|EndObjective (.ObjectiveIndex (Utilities|Struct|BreakST_QuestDataEvent ObjectiveData)) IsSuccess)
    (if IsSuccess
      (if (<= (Variables|Default|GetObjectivesCount) 0)
        (CallFunction|CompleteObjectiveType))
      (else
        (CallFunction|FailQuest)))
    (else
      (Default|CallOnObjectiveUpdate ObjectiveData))))

(event EventOnEventReceived
  (params (EventTag :type Gameplay%20Tag%20Structure) (Instigator :type Actor%20Object%20Reference) (Payload :type ST%20Event%20Payload%20Structure)))

(fn Init
  (params (GameManager :type BP%20Game%20Manager%20Object%20Reference))
  (bind _default_tags_triggered_for_quest_update (Variables|Default|GetDefault%20Tags%20triggered%20for%20quest%20update))
  ;[0.05182 0.15 0.139 0.5] Starts quest and subscribe the quest to the game manager events to update quest
  (Variables|Default|SetGameManager GameManager)
  (Variables|Default|SetObjectivesCount (Utilities|Array|Length (Variables|Default|GetQuestObjectives)))
  (for (_array_element _array_index) (Variables|Default|GetQuestObjectives)
    (LocalVariables|SetObjectiveIndex _array_index)
    (LocalVariables|SetCurrentObjective _array_element)
    (if (> (GameplayTags|GetNumGameplayTagsinContainer (Utilities|Struct|BreakST_QuestObjectiveData (LocalVariables|GetCurrentObjective))) 0)
      (GameplayTags|AppendGameplayTagContainers (LocalVariables|GetTags) (Utilities|Struct|BreakST_QuestObjectiveData (LocalVariables|GetCurrentObjective)))
      (else
        (GameplayTags|AppendGameplayTagContainers (LocalVariables|GetTags) _default_tags_triggered_for_quest_update)
        (bind _structout (Utilities|Struct|SetmembersinST_QuestObjectiveData (LocalVariables|GetCurrentObjective) _default_tags_triggered_for_quest_update))
        (Utilities|Array|SetArrayElem (Variables|Default|GetQuestObjectives) (LocalVariables|GetObjectiveIndex) _structout))))
  (if (Variables|Default|GetUseTargetActor)
    _
    (else
      (Variables|Default|SetTargetActor 0)))
  (Default|RegisterListeners (Variables|Default|GetGameManager) (LocalVariables|GetTags) (Variables|Default|GetTargetActor) self))

(fn GetDatas
  (params (ObjectiveIndex :type Integer) (DataGivenByObjective :type ST%20Quest%20Data%20Event%20Structure))
  (CallFunction|ObjectiveUpdate false DataGivenByObjective false))