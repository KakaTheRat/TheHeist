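; BP_Cheer is a skeletal mesh actor, apparently a cheering spectator, that switches looping animations with the arena's idle state.
; On BeginPlay, after a random delay, it plays a random key from the Animations map and stores a randomly picked key/value pair in Current.
; It binds to BP_ArenaZone's idle event, playing Current's value when idle and its key otherwise, each after a random delay that staggers reactions.
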(event Custom|CustomEvent
  (params (IsIdle :type Boolean))
  (if IsIdle
    (Utilities|FlowControl|Delay (Math|Random|RandomFloatinRange 0.0 3.0))
    (Components|Animation|PlayAnimation (Variables|Default|GetSkeletalMesh) (.Value (Utilities|Map|GetKeyValueByIndex (Variables|Default|GetCurrent) 0)) true)
    (else
      (Utilities|FlowControl|Delay (Math|Random|RandomFloatinRange 0.0 3.0))
      (Components|Animation|PlayAnimation (Variables|Default|GetSkeletalMesh) (.Key (Utilities|Map|GetKeyValueByIndex (Variables|Default|GetCurrent) 0)) true))))

(event EventBeginPlay
  (bind _animations (Variables|Default|GetAnimations))
  (bind _returnvalue (Utilities|Map|Length _animations))
  (bind _returnvalue_2 (- _returnvalue 1))
  (bind _returnvalue_3 (Math|Random|RandomIntegerinRange 0 _returnvalue_2))
  (bind (_key _value) (Utilities|Map|GetKeyValueByIndex _animations _returnvalue_3))
  (Utilities|FlowControl|Delay (Math|Random|RandomFloatinRange 0.0 3.0))
  (Components|Animation|SetAnimation (Variables|Default|GetSkeletalMesh) _key)
  (Components|Animation|PlayAnimation (Variables|Default|GetSkeletalMesh) _key true)
  (Variables|Default|SetCurrent (Utilities|Map|MakeMap _key _value))
  (bind _returnvalue_4 (Actor|GetActorOfClass "/Game/SurvivorsTemplate/Blueprints/Map/Arena/BP_ArenaZone.BP_ArenaZone_C"))
  (EventDispatchers|BindEventtoArenaIdle _returnvalue_4 (delegate Custom|CustomEvent)))

(event Collision|EventActorBeginOverlap
  (params (OtherActor :type Actor%20Object%20Reference)))

(fn ConstructionScript)