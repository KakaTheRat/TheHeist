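; BP_SequenceRunner runs the actions of a sequence one after another.
; Start calls ExecuteNextAction, which constructs the current entry's action class and finds any attached struct by name in the sequence's struct list.
; It passes that struct to ExecuteAction, advances the index, then binds to the action's over event to chain the sequence.
; Execution stops at the end of the data or at an invalid action class.
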(event Custom|Start
  (CallFunction|ExecuteNextAction))

(fn ExecuteNextAction
  (bind _sequenceglobal (Variables|Default|GetSequenceGlobal))
  (bind _currentindex (Variables|Default|GetCurrentIndex))
  (bind (_sequencetype _sequencestruct) (Utilities|Struct|BreakST_SequenceGroup _sequenceglobal))
  (bind _data (Variables|/Game/SurvivorsTemplate/PDA_SequenceData.PDA_SequenceData_C|GetData _sequencetype))
  (bind _output (Utilities|Array|Get(acopy) _data _currentindex))
  (bind (_action _attachedstructname) (Utilities|Struct|BreakST_DASequence _output))
  ;[1 0.4767 0.9318 0.2058] Runs several action one after another
  (LocalVariables|SetCurrentFoundStruct "")
  (if (> (Utilities|Array|Length _data) (Variables|Default|GetCurrentIndex))
    (if (Utilities|IsValidClass _action)
      (if (== _attachedstructname "")
        (bind _returnvalue (Game|ConstructObjectfromClass _action (Variables|Default|GetOwner) :!label _label))
        (Default|ExecuteAction _returnvalue (LocalVariables|GetCurrentFoundStruct))
        (Math|Integer|IncrementInt (Variables|Default|GetCurrentIndex)
          (:%20%20
            (EventDispatchers|BindEventtoActionOver _returnvalue (EventDispatchers|CreateEvent :!event ExecuteNextAction))))
        (else
          (bind _array_element (Utilities|Array|ForEachLoopwithBreak _sequencestruct :!label _label_2)
            (:LoopBody
              (if (== _attachedstructname (Utilities|Struct|BreakST_SequenceInfos _array_element))
                (LocalVariables|SetCurrentFoundStruct _array_element)
                (goto _label_2 Break)))
            (:Completed
              (goto _label))))))))