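; Lockpickable door that opens and closes on interaction once its lock has been picked.
; While locked, interacting registers it with the player's BPC_LockPick component, disables movement and streams in LockPickingLevel as a level instance to run the lockpicking, exposing Difficulty via a getter.
; OnPicked unlocks it, prints success, opens it after a short delay and later auto-closes it.
; Separate timelines drive the door's yaw for opening and closing.
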(event Custom|Close%20Door
  ;[1 0.7187 0.6486] Handles Closing Of Door After Opened
  (Variables|Default|SetisAnimating true)
  (bind _dooryaw (Timeline|Timeline_0 PlayFromStart)
    (:Update
      (Transformation|SetRelativeRotation (Variables|Default|GetDoor) (Math|Rotator|MakeRotator 0.0 0.0 _dooryaw) false true)
      (Variables|Default|SetIsOpened false)
      (Variables|Default|SetisAnimating false))))

(event Custom|OpenDoor
  (Variables|Default|SetisAnimating true)
  (bind _dooryaw (Timeline|Timeline ReverseFromEnd)
    (:Update
      (Transformation|SetRelativeRotation (Variables|Default|GetDoor) (Math|Rotator|MakeRotator 0.0 0.0 _dooryaw) false true)
      (Variables|Default|SetIsOpened true)
      (Variables|Default|SetisAnimating false))))

(event EventInteract
  (params (HitComponent :type Scene%20Component%20Object%20Reference) (InteractingActor :type Actor%20Object%20Reference) (Context :type EInteractionContext%20Enum :default "Default") (Data :type Interaction%20Data%20Object%20Reference))
  (bind _returnvalue (Actor|GetComponentbyClass InteractingActor "/Game/01_Blueprints/Components/Player/BPC_LockPick.BPC_LockPick_C"))
  (if (Variables|Default|GetIsLockpicked)
    (if (Variables|Default|GetIsOpened)
      (CallFunction|CloseDoor)
      (else
        (CallFunction|OpenDoor)))
    (else
      (Utilities|IsValid _returnvalue
        (:Is%20Valid
          (bind _asbpi_lock_picking (Utilities|Casting|CastToBPI_LockPicking self))
          (Variables|/Game/01_Blueprints/Components/Player/BPC_LockPick.BPC_LockPick_C|SetObjectBeingPicked _returnvalue _asbpi_lock_picking)
          ;[1 0.376 0.7236] Stops Player Moving When Interacting With Door
          (Pawn|Components|CharacterMovement|DisableMovement (Variables|/Script/Engine.Character|GetCharacterMovement (Variables|/Game/01_Blueprints/Components/Player/BPC_LockPick.BPC_LockPick_C|GetOwner _returnvalue)))
          ;[1 0.1667 0.00675] Streams In Level That Will Be Handling The Code For Lock Picking
          (bind _returnvalue_2 (Class|LevelStreamingDynamic|LoadLevelInstance "LockPickingLevel" "0.000000,1000.000000,0.000000" "0, 0, 0" "" 0 false))
          (Variables|Default|SetOpenedLevel _returnvalue_2)
          (Class|InteractionData|EndOfInteraction Data))))))

(event EventOnPicked
  (Variables|Default|SetIsLockpicked true)
  (Variables|/Script/Engine.LevelStreaming|SetbShouldBeLoaded (Variables|Default|GetOpenedLevel) true)
  ;[0.28 1 0.6233] Easy Debut To Notify Player Of Success
  (Development|PrintString "You Successfully Picked The Door Lock")
  (Utilities|FlowControl|Delay 1.5)
  ;[0.97 0.6319 1] Opens Door
  (CallFunction|OpenDoor)
  ;[0.06198 1 0.9702] Auto Close Door After 6.5 Seconds
  (Utilities|FlowControl|Delay 6.5)
  (if (and (not (Variables|Default|GetisAnimating)) (Variables|Default|GetIsOpened))
    (CallFunction|CloseDoor)))

(fn ConstructionScript)

(fn GetDifficulty
  (return (Variables|Default|GetDifficulty)))